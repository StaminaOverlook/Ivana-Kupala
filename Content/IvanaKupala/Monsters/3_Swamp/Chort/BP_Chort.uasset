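; Chort swamp monster that attacks the player by summoning and firing a ChortFlare projectile.
; AttackPlayer passes a DoOnce gate, turns the mesh toward the player, plays the attack montage and shows a summon effect.
; A montage notify spawns the flare, then after a delay sends AttackOver to the StateTree queue and reopens the gate.
; CancelAttack stops the montage and resets the gate, while death disables capsule collision.
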(event EventCancelAttack
  (bind _returnvalue (Transformation|GetActorRotation))
  (bind _projectilefire (Variables|Default|GetProjectileFire))
  (bind (_roll _pitch) (Math|Rotator|BreakRotator _returnvalue))
  (bind _returnvalue_2 (Transformation|GetWorldTransform _projectilefire))
  (Animation|Montage|MontageStop (Components|SkeletalMesh|GetAnimInstance (Variables|Character|GetMesh)) 0.0 (Variables|Default|GetAttack%20Anim))
  ;[1 1 1] Attack!
  (Utilities|FlowControl|DoOnce false) ; enters at Reset
)

(event EventOnDead
  (|CallParentFunction)
  (Collision|SetCollisionEnabled (Variables|Default|GetCapsule) "NoCollision"))

(event EventAttackPlayer
  (bind _returnvalue (Transformation|GetActorRotation))
  (bind _projectilefire (Variables|Default|GetProjectileFire))
  (bind (_roll _pitch) (Math|Rotator|BreakRotator _returnvalue))
  (bind _returnvalue_2 (Transformation|GetWorldTransform _projectilefire))
  ;[1 1 1] Attack!
  (Utilities|FlowControl|DoOnce false :!label _label
    (:Completed
      (Transformation|SetWorldRotation (Variables|Character|GetMesh) (Math|Rotator|MakeRotator _roll _pitch (- (.Yaw (Math|Rotator|BreakRotator (Math|Rotator|FindLookatRotation (Transformation|GetActorLocation) (Transformation|GetActorLocation (Game|GetPlayerCharacter 0))))) 9e+01)) false false)
      (bind _notifyname (Animation|Montage|PlayMontage (Variables|Character|GetMesh) (Variables|Default|GetAttack%20Anim))
        (:then
          (Utilities|FlowControl|Delay 0.5)
          (Niagara|SpawnSystematLocation "/Game/IvanaKupala/Monsters/3_Swamp/Chort/AttackFlare/Flare_Summon.Flare_Summon" (.location _returnvalue_2) (.rotation _returnvalue_2)))
        (:OnNotifyBegin
          (if (== _notifyname "ChortSendProjectile")
            (Game|SpawnActorfromClass "/Game/IvanaKupala/Monsters/3_Swamp/Chort/AttackFlare/ChortFlare.ChortFlare_C" (Math|Transform|MakeTransform (.location _returnvalue_2) (.rotation _returnvalue_2) "0.500000,0.500000,0.500000") "AlwaysSpawn" "MultiplyWithRoot" 0 0)
            (Utilities|FlowControl|Delay 2.0)
            (Default|AddEvent (Variables|Default|GetStateTreeQueue) "(TagName=\"AttackOver\")")
            (goto _label Reset)))))))

(fn ConstructionScript
  (|CallParentFunction))