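; Kikimora swamp monster Blueprint with a melee attack that damages the player through a box overlap.
; AttackPlayer re-arms a DoOnce hit gate and plays the attack montage, later sending AttackOver to the StateTree.
; Overlaps while CanDealDamage is set either apply damage or trigger blocked reactions if the player's location check and Blocking pass.
; CancelAttack stops the montage, and death disables the box's collision.
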(event OnComponentBeginOverlap(Box)
  (params (OverlappedComponent :type Primitive%20Component%20Object%20Reference) (OtherActor :type Actor%20Object%20Reference) (OtherComp :type Primitive%20Component%20Object%20Reference) (OtherBodyIndex :type Integer) (bFromSweep :type Boolean) (SweepResult :type Hit%20Result%20Structure%20%28by%20ref%29))
  ;[1 1 1] On Hitting Something
  (if (Variables|Default|GetCan%20Deal%20Damage?)
    (bind _output_get (Variables|Default|SetOther%20Actor OtherActor))
    (bind _asbp_oka_character (Utilities|Casting|CastToBP_OkaCharacter _output_get))
    (Utilities|FlowControl|DoOnce false :!label _label
      (:Completed
        (bind _returnvalue (Default|CheckActorLoc _asbp_oka_character self))
        (if (and _returnvalue (Variables|/Game/IvanaKupala/Oka/BP_OkaCharacter.BP_OkaCharacter_C|GetBlocking _asbp_oka_character))
          (Default|BlockedDamage _asbp_oka_character)
          (CallFunction|BlockedDamage)
          (else
            (Development|PrintString "Player attacked!")
            (Game|Damage|ApplyDamage (Variables|Default|GetOther%20Actor) (Variables|Default|GetDamage) 0 self)))
        (Utilities|FlowControl|Delay 1.0)
        (goto _label Reset)))))

(event EventCancelAttack
  (Animation|StopAnimMontage (Variables|Default|GetAttack%20Anim))
  ;[1 1 1] On Hitting Something
  (Utilities|FlowControl|DoOnce false) ; enters at Reset
)

(event EventOnDead
  (|CallParentFunction)
  (Collision|SetCollisionEnabled (Variables|Default|GetBox) "NoCollision"))

(event EventAttackPlayer
  ;[1 1 1] Attack!
  (Utilities|FlowControl|Sequence
    (:then_0
      ;[1 1 1] On Hitting Something
      (Utilities|FlowControl|DoOnce false) ; enters at Reset
    )
    (:then_1
      (Utilities|FlowControl|DoOnce false :!label _label
        (:Completed
          (Animation|Montage|PlayMontage (Variables|Character|GetMesh) (Variables|Default|GetAttack%20Anim) ; Attack animation here
            (:OnCompleted
              (Utilities|FlowControl|Delay 1.0)
              (Default|AddEvent (Variables|Default|GetStateTreeQueue) "(TagName=\"AttackOver\")")
              (goto _label Reset))
            (:OnInterrupted
              (goto _label Reset))))))))

(fn ConstructionScript
  (|CallParentFunction))