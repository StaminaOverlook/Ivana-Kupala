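; BP_Zver is the swamp boss Zver, which opens a boss health bar when battle starts.
; It reports start, injury, recovery, death and attack completion to a StateTree through StateTreeQueue, playing injury and death montages.
; AttackPlayer randomly picks a delayed three-flare spread or an arced leap to the player's predicted position, ending in a landing burst.
; Hoof overlaps deal damage when enabled, unless Oka is blocking.
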(event OnComponentBeginOverlap(HoofWeapon)
  (params (OverlappedComponent :type Primitive%20Component%20Object%20Reference) (OtherActor :type Actor%20Object%20Reference) (OtherComp :type Primitive%20Component%20Object%20Reference) (OtherBodyIndex :type Integer) (bFromSweep :type Boolean) (SweepResult :type Hit%20Result%20Structure%20%28by%20ref%29))
  ;[1 1 1] On Box Hit
  (if (Variables|Default|GetCan%20Deal%20Damage?)
    (Variables|Default|SetOther%20Actor OtherActor)
    (Utilities|FlowControl|DoOnce false :!label _label
      (:Completed
        (bind _asbp_oka_character (Utilities|Casting|CastToBP_OkaCharacter (Variables|Default|GetOther%20Actor)))
        (if (Variables|/Game/IvanaKupala/Oka/BP_OkaCharacter.BP_OkaCharacter_C|GetBlocking _asbp_oka_character)
          (Default|BlockedDamage _asbp_oka_character)
          (CallFunction|BlockedDamage)
          (else
            (Development|PrintString "Oka is damaged!")
            (Game|Damage|ApplyDamage (Variables|Default|GetOther%20Actor) (Variables|Default|GetDamage) 0 self)))
        (Utilities|FlowControl|Delay 1.0)
        (goto _label Reset)))))

(event Custom|Jump%20To
  (params (Position :type Vector))
  (bind (_x _y _z) (Math|Vector|BreakVector Position))
  ;[1 1 1] Jump To
  (Utilities|FlowControl|DoOnce false
    (:Completed
      (Animation|Montage|PlayMontage (Variables|Character|GetMesh) (Variables|Default|GetAttack%202%20Anim)
        (:then
          (bind _outlaunchvelocity (Game|SuggestProjectileVelocityCustomArc (Transformation|GetActorLocation) (Math|Vector|MakeVector _x _y (+ _z 1e+02)) 0.0 0.5))
          (Character|LaunchCharacter _outlaunchvelocity true true)
          (EventDispatchers|AssignLandedDelegate (delegate Custom|OnLand)))))))

(event Custom|Attack%20Jump
  ;[1 1 1] Attack Jump
  (Utilities|FlowControl|Sequence
    (:then_0
      ;[1 1 1] Jump To
      (Utilities|FlowControl|DoOnce false) ; enters at Reset
    )
    (:then_1
      ;[1 1 1] On Box Hit
      (Utilities|FlowControl|DoOnce false) ; enters at Reset
    )
    (:then_2
      (if (not (Variables|Default|GetAttacking))
        (Variables|Default|SetAttacking true)
        (bind _location (CallFunction|CalculateFutureActorLoc (Game|GetPlayerCharacter 0) 1.0))
        (CallFunction|Jumpto _location)))))

(event Custom|Attack%20Flare
  (bind _projectilefire (Variables|Default|GetProjectileFire))
  (bind _returnvalue (Transformation|GetWorldTransform _projectilefire))
  (bind (_roll _pitch _yaw) (Math|Rotator|BreakRotator (.rotation _returnvalue)))
  ;[1 1 1] Attack!
  (if (not (Variables|Default|GetAttacking))
    (Variables|Default|SetAttacking true)
    (Utilities|FlowControl|DoOnce false :!label _label
      (:Completed
        (Animation|Montage|PlayMontage (Variables|Character|GetMesh) (Variables|Default|GetAttack%20Anim)
          (:then
            (Utilities|FlowControl|Delay 0.5)
            (Niagara|SpawnSystemAttached "/Game/IvanaKupala/Monsters/3_Swamp/Chort/AttackFlare/Flare_Summon.Flare_Summon" _projectilefire "None" "0, 0, 0" "0, 0, 0" "KeepRelativeOffset" false)
            (Utilities|FlowControl|Delay 1.5)
            (Game|SpawnActorfromClass "/Game/IvanaKupala/Monsters/3_Swamp/Chort/AttackFlare/ChortFlare.ChortFlare_C" (Math|Transform|MakeTransform (.location _returnvalue) (Math|Rotator|MakeRotator _roll _pitch (- _yaw 5.0)) "0.500000,0.500000,0.500000") "AlwaysSpawn" "MultiplyWithRoot" 0 0)
            (Utilities|FlowControl|Delay 0.2)
            (Game|SpawnActorfromClass "/Game/IvanaKupala/Monsters/3_Swamp/Chort/AttackFlare/ChortFlare.ChortFlare_C" (Math|Transform|MakeTransform (.location _returnvalue) (Math|Rotator|MakeRotator _roll _pitch _yaw) "0.500000,0.500000,0.500000") "AlwaysSpawn" "MultiplyWithRoot" 0 0)
            (Utilities|FlowControl|Delay 0.2)
            (Game|SpawnActorfromClass "/Game/IvanaKupala/Monsters/3_Swamp/Chort/AttackFlare/ChortFlare.ChortFlare_C" (Math|Transform|MakeTransform (.location _returnvalue) (Math|Rotator|MakeRotator _roll _pitch (+ _yaw 5.0)) "0.500000,0.500000,0.500000") "AlwaysSpawn" "MultiplyWithRoot" 0 0)
            (Utilities|FlowControl|Delay 2.0)
            (Variables|Default|SetAttacking false)
            (Default|AddEvent (Variables|Default|GetStateTreeQueue) "(TagName=\"AttackOver\")")
            (goto _label Reset)))))))

(event Custom|OnLand
  (params (Hit :type Hit%20Result%20Structure%20%28by%20ref%29))
  ;[1 1 1] Jump To
  (EventDispatchers|UnbindEventfromLandedDelegate (delegate Custom|OnLand))
  (Variables|Default|SetAttacking false)
  (Default|AddEvent (Variables|Default|GetStateTreeQueue) "(TagName=\"Boss.Init\")")
  (Components|Movement|StopMovementImmediately (Variables|Character|GetCharacterMovement))
  (Niagara|SpawnSystematLocation "/Game/IvanaKupala/Monsters/3_Swamp/Zver/LandingBurst.LandingBurst" (Transformation|GetActorLocation)))

(event Custom|Initialize%20Battle
  (bind _healthcomponent (Variables|Default|GetHealthComponent))
  ;[1 1 1] Comment
  (bind _returnvalue (UserInterface|CreateWidget "/Game/IvanaKupala/Interface/WB_BossHealth.WB_BossHealth_C"))
  (bind _output_get (Variables|Default|SetBossHealthWidget _returnvalue))
  (Default|InitWidget _output_get _healthcomponent "Зверь, Коллекционер Редких Вещей")
  (EventDispatchers|BindEventtoDamaged _healthcomponent (delegate EventOnDamaged))
  (EventDispatchers|BindEventtoDead _healthcomponent (delegate EventOnDead))
  (Default|AddEvent (Variables|Default|GetStateTreeQueue) "(TagName=\"Boss.Start\")"))

(event EventAttackPlayer
  ;[1 1 1] Comment
  (switch int (Math|Random|RandomIntegerinRange 0 1)
    (:Default
      (CallFunction|AttackFlare :!label _label))
    (:0
      (goto _label))
    (:1
      (CallFunction|AttackJump))))

(event EventBeginPlay)

(event EventOnDamaged
  (params (NewHealth :type Float%20%28double-precision%29) (Amount :type Float%20%28double-precision%29))
  (bind _charactermovement (Variables|Character|GetCharacterMovement))
  (bind _injured_anim (Variables|Default|GetInjured%20Anim))
  ;[1 1 1] Taking Damage
  (Default|AddEvent (Variables|Default|GetStateTreeQueue) "(TagName=\"Injured\")")
  (Pawn|Components|CharacterMovement|SetMovementMode _charactermovement "MOVE_None" 0)
  (bind _returnvalue (CallFunction|IsMontagePlaying _injured_anim))
  (if (not _returnvalue)
    (Animation|Montage|PlayMontage (Variables|Character|GetMesh) _injured_anim ; Injured Animation here
      (:OnCompleted
        (Pawn|Components|CharacterMovement|SetMovementMode _charactermovement "MOVE_Walking" 0)
        (Default|AddEvent (Variables|Default|GetStateTreeQueue) "(TagName=\"Recover\")")))))

(event EventOnDead
  ;[1 1 1] Taking Damage
  (Default|AddEvent (Variables|Default|GetStateTreeQueue) "(TagName=\"Dead\")")
  (Utilities|FlowControl|DoOnce false
    (:Completed
      (Animation|Montage|PlayMontage (Variables|Character|GetMesh) (Variables|Default|GetDeath%20Anim) 1.0 0.0 "Dying" ; Death Animation here
        (:then
          (Utilities|FlowControl|DoOnce false
            (:Completed
              (Default|CallOnDeath))))))))

(fn ConstructionScript
  (bind _statetreequeue (Variables|Default|GetStateTreeQueue))
  (Components|DestroyComponent (Variables|Default|GetWidgetHealth))
  (Default|ConnectStateTree _statetreequeue (Variables|Default|GetMonsterStateTree))
  (Default|AddEvent _statetreequeue "(TagName=\"Boss.Init\")"))

(fn CalculateFutureActorLoc
  (params (Actor :type Actor%20Object%20Reference) (Time :type Float%20%28double-precision%29))
  (return (+ (Transformation|GetActorLocation Actor) (* (+ (Transformation|GetVelocity Actor) "1.000000,0.000000,0.000000") Time))))