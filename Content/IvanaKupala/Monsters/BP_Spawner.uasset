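; BP_Spawner is a monster spawn point that creates an enemy of a configurable class just above itself when activated.
; Activation can first play a summon sound and circle effect with a short delay before spawning.
; The spawned BP_MonsterAI receives the see-player flag, triggering a Noticed StateTree event when true.
; Its death event is bound so the spawner reports itself to BP_TopDownGameMode through EnemyDied.
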(event Custom|Activate_Spawner
  (params (See%20Player? :type Boolean) (Spawn%20Circle? :type Boolean))
  (bind _returnvalue (Transformation|GetActorLocation))
  (bind _returnvalue_2 (Transformation|GetActorLocation))
  (bind (_x _y _z) (Math|Vector|BreakVector _returnvalue_2))
  (bind (_x_2 _y_2 _z_2) (Math|Vector|BreakVector _returnvalue))
  (bind _returnvalue_3 (+ _z_2 5e+01))
  (bind _returnvalue_4 (Math|Vector|MakeVector _x_2 _y_2 _returnvalue_3))
  ;[0 0 0] Activate Spawner
  (if Spawn%20Circle?
    (Audio|SpawnSoundatLocation "/Game/IvanaKupala/Monsters/_WAVES/SUMMON_CIRCLE_MAT/Monster_summon.Monster_summon" _returnvalue_4 "0, 0, 0" 1.0 1.0 0.0 0 0)
    (Niagara|SpawnSystematLocation "/Game/IvanaKupala/Monsters/_WAVES/SUMMON_CIRCLE_MAT/SummonCircle.SummonCircle" _returnvalue_4)
    (Utilities|FlowControl|Delay 2.0))
  (bind _returnvalue_5 (Game|SpawnActorfromClass (Variables|Default|GetClass) (Math|Transform|MakeTransform (Math|Vector|MakeVector _x _y (+ _z 1.5e+02)) "0, 0, 0" "1.000000,1.000000,1.000000") "AdjustIfPossibleButAlwaysSpawn" "MultiplyWithRoot" 0 0))
  (Utilities|IsValid _returnvalue_5
    (:Is%20Valid
      (bind _asbp_monster_ai (Utilities|Casting|CastToBP_MonsterAI _returnvalue_5))
      (bind _output_get (Variables|/Game/IvanaKupala/Monsters/BP_MonsterAI.BP_MonsterAI_C|SetCan%20See%20Player? _asbp_monster_ai See%20Player?))
      (EventDispatchers|BindEventtoOnDeath _asbp_monster_ai (delegate Custom|On%20Monster%20Dead))
      (if _output_get
        (Default|AddEvent (Variables|/Game/IvanaKupala/Monsters/BP_MonsterAI.BP_MonsterAI_C|GetStateTreeQueue _asbp_monster_ai) "(TagName=\"Noticed\")")))))

(event Custom|On%20Monster%20Dead
  ;[0 0 0] Send to Game Mode - Monster Died
  (bind _asbp_top_down_game_mode (Utilities|Casting|CastToBP_TopDownGameMode (Game|GetGameMode)))
  (Default|EnemyDied _asbp_top_down_game_mode self))

(fn ConstructionScript)