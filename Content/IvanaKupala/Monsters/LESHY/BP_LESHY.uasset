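; BP_LESHY is the Leshy monster NPC, which moves into place when it appears and only then becomes interactable.
; It starts non-interactable on BeginPlay, and AppearNPC activates its InterpToMovement component, then binds that component's stop event to set Interactable to true.
; DisappearNPC is left empty, and the construction script only calls the parent.
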(event Custom|Event%20Disappear%20NPC)

(event Custom|Activate%20Interactable
  (params (ImpactResult :type Hit%20Result%20Structure%20%28by%20ref%29) (Time :type Float%20%28single-precision%29))
  ;[1 1 1] On Movement Stop
  (Variables|Default|SetInteractable true))

(event Collision|EventActorBeginOverlap
  (params (OtherActor :type Actor%20Object%20Reference))
  (|CallParentFunction OtherActor) ; This node is disabled and will not be called.\nDrag off pins to build functionality.
)

(event EventTick
  (params (DeltaSeconds :type Float%20%28single-precision%29))
  (|CallParentFunction DeltaSeconds) ; This node is disabled and will not be called.\nDrag off pins to build functionality.
)

(event EventAppearNPC
  (params (Location :type Vector :default "0, 0, 0"))
  (bind _interptomovement (Variables|Default|GetInterpToMovement))
  ;[1 1 1] On Appear NPC
  (Components|Activation|Activate _interptomovement true)
  (EventDispatchers|BindEventtoOnInterptoStop _interptomovement (delegate Custom|Activate%20Interactable)))

(event EventBeginPlay
  ;[1 1 1] Begin Play
  (Variables|Default|SetInteractable false))

(fn ConstructionScript
  (|CallParentFunction))