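; Boss enemy Zver ("Beast, Collector of Rare Things") that chases the player and shows a boss health bar during battle.
; On reaching the player, it randomly fires a three-flare fan or leaps along a computed arc toward the player's velocity-predicted position.
; Tick resumes pursuit and turns the mesh toward the player mid-attack.
; Hoof overlaps deal blockable damage; incoming hits play an injury montage or trigger death.
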(event OnComponentBeginOverlap(HoofWeapon)
  (params (OverlappedComponent :type Primitive%20Component%20Object%20Reference) (OtherActor :type Actor%20Object%20Reference) (OtherComp :type Primitive%20Component%20Object%20Reference) (OtherBodyIndex :type Integer) (bFromSweep :type Boolean) (SweepResult :type Hit%20Result%20Structure%20%28by%20ref%29))
  ;[1 1 1] On Box Hit
  (if (Variables|Default|GetCan%20Deal%20Damage?)
    (Variables|Default|SetOther%20Actor OtherActor)
    (Utilities|FlowControl|DoOnce false :!label _label
      (:Completed
        (bind _asbp_top_down_character (Utilities|Casting|CastToBP_TopDownCharacter (Variables|Default|GetOther%20Actor)))
        (if (Variables|/Game/IvanaKupala/Oka/BP_TopDownCharacter.BP_TopDownCharacter_C|GetBlocking _asbp_top_down_character)
          (Default|BlockedDamage _asbp_top_down_character)
          (CallFunction|BlockedDamage)
          (else
            (Development|PrintString "Oka is damaged!")
            (Game|Damage|ApplyDamage (Variables|Default|GetOther%20Actor) (Variables|Default|GetDamage) 0 self)))
        (Utilities|FlowControl|Delay 1.0)
        (goto _label Reset)))))

(event Custom|Jump%20To
  (params (Position :type Vector))
  (bind (_x _y _z) (Class|KismetMathLibrary|BreakVector3f Position))
  ;[1 1 1] Jump To
  (Utilities|FlowControl|DoOnce false
    (:Completed
      (Animation|Montage|PlayMontage (Variables|Character|GetMesh) (Variables|Default|GetAttack%202%20Anim)
        (:then
          (bind _outlaunchvelocity (Game|SuggestProjectileVelocityCustomArc (Transformation|GetActorLocation) (Math|Vector|MakeVector _x _y (+ _z 1e+02)) 0.0 0.5))
          (Character|LaunchCharacter _outlaunchvelocity true true)
          (EventDispatchers|AssignLandedDelegate (delegate Custom|OnLand)))))))

(event Custom|Attack%20Jump
  ;[1 1 1] Attack Jump
  (Utilities|FlowControl|Sequence
    (:then_0
      ;[1 1 1] Jump To
      (Utilities|FlowControl|DoOnce false) ; enters at Reset
    )
    (:then_1
      ;[1 1 1] On Box Hit
      (Utilities|FlowControl|DoOnce false) ; enters at Reset
    )
    (:then_2
      (if (not (Variables|Default|GetAttacking))
        (Variables|Default|SetAttacking true)
        (bind _location (CallFunction|CalculateFutureActorLoc (Game|GetPlayerCharacter 0) 1.0))
        (CallFunction|Jumpto _location)))))

(event Custom|Attack%20Flare
  (bind _projectilefire (Variables|Default|GetProjectileFire))
  (bind _returnvalue (Transformation|GetWorldTransform _projectilefire))
  (bind (_roll _pitch _yaw) (Math|Rotator|BreakRotator (.rotation _returnvalue)))
  ;[1 1 1] Attack!
  (if (not (Variables|Default|GetAttacking))
    (Variables|Default|SetAttacking true)
    (Utilities|FlowControl|DoOnce false :!label _label
      (:Completed
        (Animation|Montage|PlayMontage (Variables|Character|GetMesh) (Variables|Default|GetAttack%20Anim)
          (:then
            (Utilities|FlowControl|Delay 0.5)
            (Niagara|SpawnSystemAttached "/Game/IvanaKupala/Monsters/Chort/AttackFlare/Flare_Summon.Flare_Summon" _projectilefire "None" "0, 0, 0" "0, 0, 0" "KeepRelativeOffset" false)
            (Utilities|FlowControl|Delay 1.5)
            (Game|SpawnActorfromClass "/Game/IvanaKupala/Monsters/Chort/AttackFlare/ChortFlare.ChortFlare_C" (Math|Transform|MakeTransform (.location _returnvalue) (Math|Rotator|MakeRotator _roll _pitch (+ _yaw -5.0)) "0.500000,0.500000,0.500000") "AlwaysSpawn" "MultiplyWithRoot" 0 0)
            (Utilities|FlowControl|Delay 0.2)
            (Game|SpawnActorfromClass "/Game/IvanaKupala/Monsters/Chort/AttackFlare/ChortFlare.ChortFlare_C" (Math|Transform|MakeTransform (.location _returnvalue) (Math|Rotator|MakeRotator _roll _pitch _yaw) "0.500000,0.500000,0.500000") "AlwaysSpawn" "MultiplyWithRoot" 0 0)
            (Utilities|FlowControl|Delay 0.2)
            (Game|SpawnActorfromClass "/Game/IvanaKupala/Monsters/Chort/AttackFlare/ChortFlare.ChortFlare_C" (Math|Transform|MakeTransform (.location _returnvalue) (Math|Rotator|MakeRotator _roll _pitch (+ _yaw 5.0)) "0.500000,0.500000,0.500000") "AlwaysSpawn" "MultiplyWithRoot" 0 0)
            (Utilities|FlowControl|Delay 2.0)
            (Variables|Default|SetAttacking false)
            (goto _label Reset)))))))

(event Custom|OnLand
  (params (Hit :type Hit%20Result%20Structure%20%28by%20ref%29))
  ;[1 1 1] Jump To
  (EventDispatchers|UnbindEventfromLandedDelegate (delegate Custom|OnLand))
  (Variables|Default|SetAttacking false)
  (Components|Movement|StopMovementImmediately (Variables|Character|GetCharacterMovement))
  (Niagara|SpawnSystematLocation "/Game/IvanaKupala/Monsters/Zver/LandingBurst.LandingBurst" (Transformation|GetActorLocation)))

(event Custom|Initialize%20Battle
  (bind _maxhealth (Variables|Default|GetMaxHealth))
  ;[1 1 1] Comment
  (bind _returnvalue (UserInterface|CreateWidget "/Game/IvanaKupala/Interface/WidgetBossHealth.WidgetBossHealth_C"))
  (UserInterface|Viewport|AddtoViewport _returnvalue 0)
  (UserInterface|Animation|PlayAnimation _returnvalue (Variables|/Game/IvanaKupala/Interface/WidgetBossHealth.WidgetBossHealth_C|GetAppear _returnvalue) 0.0 1 "Forward" 1.0 false)
  (bind _output_get (Variables|Default|SetNewVar _returnvalue))
  (Default|UpdateHealthBar _output_get _maxhealth _maxhealth)
  (Default|SetName _output_get "Зверь, Коллекционер Редких Вещей"))

(event EventFollowPlayer
  ;[1 1 1] Follow Player
  (if (not (Variables|Default|GetAttacking))
    (AI|AIMoveTo self "0, 0, 0" (Game|GetPlayerCharacter 0) (Variables|Default|GetAcceptance%20Radius) true
      (:OnSuccess
        (Variables|Default|SetFollowing%20Player? false)
        (CallFunction|AttackPlayer))
      (:OnFail
        (Variables|Default|SetFollowing%20Player? false)))))

(event EventAttackPlayer
  ;[1 1 1] Comment
  (switch int (Math|Random|RandomIntegerinRange 0 1)
    (:Default
      (CallFunction|AttackFlare :!label _label))
    (:0
      (goto _label))
    (:1
      (CallFunction|AttackJump))))

(event EventBeginPlay
  (Components|DestroyComponent (Variables|Default|GetWidgetHealth)))

(event Game|Damage|EventAnyDamage
  (params (Damage :type Float%20%28single-precision%29) (DamageType :type Damage%20Type%20Object%20Reference) (InstigatedBy :type Controller%20Object%20Reference) (DamageCauser :type Actor%20Object%20Reference))
  (bind _mesh (Variables|Character|GetMesh))
  ;[1 1 1] Taking Damage
  (if (Variables|Default|GetbCanBeDamaged)
    (Variables|Default|SetbCanBeDamaged false)
    (Variables|Default|SetCan%20See%20Player? true)
    (Pawn|Components|CharacterMovement|SetMovementMode (Variables|Character|GetCharacterMovement) "MOVE_None" 0)
    (Animation|StopAnimMontage 0)
    (bind _output_get (Variables|Default|SetHealth (- (Variables|Default|GetHealth) Damage)))
    (Default|UpdateHealthBar (Variables|Default|GetNewVar) _output_get (Variables|Default|GetMaxHealth))
    (if (<= (Variables|Default|GetHealth) 0.0)
      (Utilities|FlowControl|DoOnce false :!label _label
        (:Completed
          (Animation|Montage|PlayMontage _mesh (Variables|Default|GetDeath%20Anim) 1.0 0.0 "Dying" :!pinned true ; Death Animation here
            (:then
              (Utilities|FlowControl|DoOnce false
                (:Completed
                  (Default|CallOnDeath))))
            (:OnInterrupted
              (goto _label Reset)))))
      (else
        (Animation|Montage|PlayMontage _mesh (Variables|Default|GetInjured%20Anim) :!pinned true ; Injured Animation here
          (:OnCompleted
            _)
          (:OnInterrupted
            _))
        (Pawn|Components|CharacterMovement|SetMovementMode (Variables|Character|GetCharacterMovement) "MOVE_Walking" 0)
        (Variables|Default|SetbCanBeDamaged true)
        (CallFunction|FollowPlayer)))))

(event EventTick
  (params (DeltaSeconds :type Float%20%28single-precision%29))
  (bind _returnvalue (Transformation|GetActorRotation))
  (bind (_roll _pitch) (Math|Rotator|BreakRotator _returnvalue))
  ;[1 1 1] Event Tick
  (if (<= (Variables|Default|GetHealth) 0.0)
    (if (not (== (Animation|GetCurrentMontage :!class /Script/Engine.Character) (Variables|Default|GetDeath%20Anim)))
      (Class|PawnSensingComponent|SetSensingUpdatesEnabled (Variables|Default|GetPawnSensing) false)
      (Variables|Default|SetCan%20See%20Player? false)
      (Variables|Default|SetAttacking true)
      (Components|Movement|StopMovementImmediately (Variables|Character|GetCharacterMovement))
      (Utilities|FlowControl|DoOnce false :!label _label
        (:Completed
          (Animation|Montage|PlayMontage 0 (Variables|Default|GetDeath%20Anim) 1.0 0.0 "Dying" :!pinned true ; Death Animation here
            (:then
              (Utilities|FlowControl|DoOnce false
                (:Completed
                  (Default|CallOnDeath))))
            (:OnInterrupted
              (goto _label Reset))))))
    (elif (Variables|Default|GetAttacking)
      (Transformation|SetWorldRotation (Variables|Character|GetMesh) (Math|Rotator|MakeRotator _roll _pitch (- (.Yaw (Math|Rotator|BreakRotator (Math|Rotator|FindLookatRotation (Transformation|GetActorLocation) (Transformation|GetActorLocation (Game|GetPlayerCharacter 0))))) 9e+01)) false false)
      (elif (Math|Boolean|ANDBoolean (Variables|Default|GetCan%20See%20Player?) (not (Variables|Default|GetFollowing%20Player?)) (not (Variables|Default|GetCan%20Deal%20Damage?)))
        (Variables|Default|SetFollowing%20Player? true)
        (CallFunction|FollowPlayer)))))

(fn ConstructionScript
  (|CallParentFunction))

(fn CalculateFutureActorLoc
  (params (Actor :type Actor%20Object%20Reference) (Time :type Float%20%28double-precision%29))
  (return (+ (Transformation|GetActorLocation Actor) (* (+ (Transformation|GetVelocity Actor) "1.000000,0.000000,0.000000") Time))))