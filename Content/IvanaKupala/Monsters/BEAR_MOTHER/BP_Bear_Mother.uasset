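; Bear Mother monster Blueprint that handles spawn animation and picks between charge, one-time low-health roar and montage melee attacks, signalling AttackOver to its StateTree queue.
; The charge tracks the player through a looping timer during windup, then speeds AIMoveTo past them, with a Timeline cooldown.
; Overlaps drive damage: melee checks blocking, while charge hits add damage and knockback.
; Death disables hit collisions.
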(event OnComponentBeginOverlap(Box)
  (params (OverlappedComponent :type Primitive%20Component%20Object%20Reference) (OtherActor :type Actor%20Object%20Reference) (OtherComp :type Primitive%20Component%20Object%20Reference) (OtherBodyIndex :type Integer) (bFromSweep :type Boolean) (SweepResult :type Hit%20Result%20Structure%20%28by%20ref%29))
  ;[1 1 1] On Hitting Something
  (if (Variables|Default|GetCan%20Deal%20Damage?)
    (bind _output_get (Variables|Default|SetOther%20Actor OtherActor))
    (bind _asbp_oka_character (Utilities|Casting|CastToBP_OkaCharacter _output_get))
    (Utilities|FlowControl|DoOnce false :!label _label
      (:Completed
        (bind _returnvalue (Default|CheckActorLoc _asbp_oka_character self))
        (if (and _returnvalue (Variables|/Game/IvanaKupala/Oka/BP_OkaCharacter.BP_OkaCharacter_C|GetBlocking _asbp_oka_character))
          (Default|BlockedDamage _asbp_oka_character)
          (CallFunction|BlockedDamage)
          (else
            (Development|PrintString "Player attacked!")
            (Game|Damage|ApplyDamage (Variables|Default|GetOther%20Actor) (Variables|Default|GetDamage) 0 self)))
        (Utilities|FlowControl|Delay 1.0)
        (goto _label Reset)))))

(event OnComponentBeginOverlap(ChargeCollision)
  (params (OverlappedComponent :type Primitive%20Component%20Object%20Reference) (OtherActor :type Actor%20Object%20Reference) (OtherComp :type Primitive%20Component%20Object%20Reference) (OtherBodyIndex :type Integer) (bFromSweep :type Boolean) (SweepResult :type Hit%20Result%20Structure%20%28by%20ref%29))
  ;[1 1 1] Charge
  (if (Variables|Default|GetCharge)
    (bind _output_get (Variables|Default|SetOther%20Actor OtherActor))
    (bind _asbp_oka_character (Utilities|Casting|CastToBP_OkaCharacter _output_get))
    (Utilities|FlowControl|DoOnce false :!label _label
      (:Completed
        (Variables|Default|SetOka%20locaton (Transformation|GetActorLocation _asbp_oka_character))
        (Game|Damage|ApplyDamage (Variables|Default|GetOther%20Actor) (+ (Variables|Default|GetDamage) 1e+01) 0 self)
        (Character|LaunchCharacter _asbp_oka_character (+ (* (Math|Vector|GetForwardVector (Transformation|GetActorRotation)) 1e+03) "0.000000,0.000000,200.000000") false false)
        (Utilities|FlowControl|Delay 2.0)
        (goto _label Reset)))))

(event Custom|Event%20Charge
  ;[1 1 1] Charge
  (Development|PrintString "charge" true true "(R=1.000000,G=0.067083,B=0.166763,A=1.000000)")
  (Variables|Default|SetCharge%20ready false)
  (Utilities|Time|SetTimerbyFunctionName 0 "LookForPlayer" 0.0001 true true)
  (Animation|Montage|PlayMontage (Variables|Character|GetMesh) "/Game/IvanaKupala/Monsters/BEAR_MOTHER/Animations/Bear_Mother_Attack_Prepare_Montage.Bear_Mother_Attack_Prepare_Montage" ; Attack animation here
    (:then
      (Utilities|FlowControl|Delay 1.25)
      (Class|KismetSystemLibrary|PauseTimer 0 "LookForPlayer"))
    (:OnCompleted
      (Variables|Default|SetCharge true)
      (Variables|/Script/Engine.CharacterMovementComponent|SetMaxWalkSpeed (Variables|Character|GetCharacterMovement) 1.6e+03)
      (Variables|Default|SetCharge%20Location (+ (Transformation|GetActorLocation (Game|GetPlayerCharacter 0)) (* (Math|Vector|GetForwardVector (Transformation|GetActorRotation)) 6e+02)))
      (AI|AIMoveTo self (Variables|Default|GetCharge%20Location) 0 5e+01 false
        (:OnSuccess
          _)
        (:OnFail
          (Development|PrintString "fail" true true "(R=1.000000,G=0.250773,B=0.000000,A=1.000000)")))
      (Variables|/Script/Engine.CharacterMovementComponent|SetMaxWalkSpeed (Variables|Character|GetCharacterMovement) 6e+02)
      (Variables|Default|SetCharge false)
      (CallFunction|ReloadCharge)
      (Default|AddEvent (Variables|Default|GetStateTreeQueue) "(TagName=\"AttackOver\")"))
    (:OnInterrupted
      (Default|AddEvent (Variables|Default|GetStateTreeQueue) "(TagName=\"AttackOver\")")
      (CallFunction|ReloadCharge))))

(event Custom|Spawn%20amination
  (Animation|Montage|PlayMontage (Variables|Character|GetMesh) "/Game/IvanaKupala/Monsters/BEAR_MOTHER/Animations/Bear_Mother_Appearance_Montage.Bear_Mother_Appearance_Montage" ; Attack animation here
    (:then
      (Utilities|FlowControl|Delay 4.2))))

(event Custom|Reload%20charge
  (Timeline|Timeline PlayFromStart
    (:Finished
      (Variables|Default|SetCharge%20ready true))))

(event Custom|Event%20Roar
  (Variables|Default|SetRoarSkill false)
  (Variables|Default|SetDamage 3e+01)
  (Animation|Montage|PlayMontage 0 "/Game/IvanaKupala/Monsters/BEAR_MOTHER/Animations/Bear_Mother_Roar_Montage.Bear_Mother_Roar_Montage"
    (:then
      (Utilities|FlowControl|Delay 1.7)
      (Default|AddEvent (Variables|Default|GetStateTreeQueue) "(TagName=\"AttackOver\")"))))

(event EventCancelAttack
  ;[1 1 1] On Hitting Something
  (Animation|StopAnimMontage (Variables|Default|GetAttack%20Anim))
  (Utilities|FlowControl|DoOnce false) ; enters at Reset
)

(event EventOnDead
  (|CallParentFunction)
  (for _array_element (Utilities|Array|MakeArray (Variables|Default|GetBox) (Variables|Default|GetBox1) (Variables|Default|GetChargeCollision))
    (Collision|SetCollisionEnabled _array_element "NoCollision")))

(event EventAttackPlayer
  ;[1 1 1] Attack!
  (Utilities|FlowControl|Sequence
    (:then_0
      ;[1 1 1] On Hitting Something
      (Utilities|FlowControl|DoOnce false) ; enters at Reset
    )
    (:then_1
      (if (Variables|Default|GetCharge%20ready)
        (CallFunction|EventCharge)
        (elif (and (< (Variables|/Game/IvanaKupala/Interface/HealthComponent.HealthComponent_C|GetHealth (Variables|Default|GetHealthComponent)) 5e+01) (Variables|Default|GetRoarSkill))
          (CallFunction|EventRoar)
          (else
            (Utilities|FlowControl|DoOnce false :!label _label
              (:Completed
                (Animation|Montage|PlayMontage (Variables|Character|GetMesh) (Variables|Default|GetAttack%20Anim) ; Attack animation here
                  (:OnCompleted
                    (Utilities|FlowControl|Delay 1.0))
                  (:OnInterrupted
                    _))
                (Default|AddEvent (Variables|Default|GetStateTreeQueue) "(TagName=\"AttackOver\")")
                (goto _label Reset)))))))))

(fn ConstructionScript
  (|CallParentFunction))

(fn LookforPlayer
  (bind _returnvalue (Transformation|GetActorRotation))
  (Transformation|SetActorRotation (Math|Rotator|MakeRotator (.roll _returnvalue) (.pitch _returnvalue) (.yaw (Class|KismetMathLibrary|RInterptoConstant (Transformation|GetActorRotation) (Math|Rotator|FindLookatRotation (Transformation|GetActorLocation) (Transformation|GetActorLocation (Game|GetPlayerCharacter 0))) (Utilities|Time|GetWorldDeltaSeconds) 3.5e+02)))))