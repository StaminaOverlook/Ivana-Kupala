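; BP_StartFly is the Red Raven's flying attack actor, which swoops at the player's position five seconds after BeginPlay.
; One timeline lerps it to that position, then a second starts pushing it forward, whose update immediately spawns a reversed-facing BP_RedRaven and destroys this actor.
; Its sphere overlap hits BP_OkaCharacter once, calling BlockedDamage for a block that passes the location check, otherwise applying pushed-type damage.
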(event OnComponentBeginOverlap(Sphere)
  (params (OverlappedComponent :type Primitive%20Component%20Object%20Reference) (OtherActor :type Actor%20Object%20Reference) (OtherComp :type Primitive%20Component%20Object%20Reference) (OtherBodyIndex :type Integer) (bFromSweep :type Boolean) (SweepResult :type Hit%20Result%20Structure%20%28by%20ref%29))
  (bind _output_get (Variables|Default|SetOther%20Actor OtherActor))
  (bind _asbp_oka_character (Utilities|Casting|CastToBP_OkaCharacter _output_get))
  (Utilities|FlowControl|DoOnce false
    (:Completed
      (bind _returnvalue (Default|CheckActorLoc _asbp_oka_character self))
      (if (and _returnvalue (Variables|/Game/IvanaKupala/Oka/BP_OkaCharacter.BP_OkaCharacter_C|GetBlocking _asbp_oka_character))
        (Default|BlockedDamage _asbp_oka_character)
        (else
          (Development|PrintString "Player attacked!")
          (Game|Damage|ApplyDamage (Variables|Default|GetOther%20Actor) (Variables|Default|GetDamage) 0 self "/Game/IvanaKupala/Monsters/Pushed_DamageType.Pushed_DamageType_C"))))))

(event Custom|StartFly
  (bind _returnvalue (Transformation|GetActorRotation))
  (Variables|Default|SetEndLocation (Transformation|GetActorLocation (Game|GetPlayerCharacter 0)))
  (bind _newtrack_0 (Timeline|Timeline PlayFromStart)
    (:Update
      (Transformation|SetActorLocation (Math|Vector|Lerp(Vector) (Variables|Default|GetStartLocation) (Variables|Default|GetEndLocation) _newtrack_0) false false))
    (:Finished
      (bind _output_get (Variables|Default|SetStartLocation (Transformation|GetActorLocation)))
      (Variables|Default|SetEndLocation (+ _output_get (* (Math|Vector|GetForwardVector (Transformation|GetActorRotation)) 1e+03)))
      (bind _newtrack_0_2 (Timeline|Timeline_0 PlayFromStart)
        (:Update
          (Transformation|SetActorLocation (Math|Vector|Lerp(Vector) (Variables|Default|GetStartLocation) (Variables|Default|GetEndLocation) _newtrack_0_2) false false)
          (Game|SpawnActorfromClass "/Game/IvanaKupala/Monsters/2_Deepwood/RedRaven/BP_RedRaven.BP_RedRaven_C" (Math|Transform|MakeTransform (Transformation|GetActorLocation) (Math|Rotator|MakeRotator (.roll _returnvalue) (.pitch _returnvalue) (- (.yaw _returnvalue) 1.8e+02)) "1.000000,1.000000,1.000000") "Undefined" "MultiplyWithRoot" 0 0)
          (Actor|DestroyActor))))))

(event EventBeginPlay
  (Variables|Default|SetStartLocation (Transformation|GetActorLocation))
  (Utilities|FlowControl|Delay 5.0)
  (CallFunction|StartFly))

(fn ConstructionScript)