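; Red Raven enemy, a child monster Blueprint that walks, caws at random intervals while it cannot see the player, and attacks on contact.
; AttackPlayer re-arms a DoOnce gate so a capsule overlap deals one hit, unless the player's directional block turns it into blocked damage.
; FollowPlayer and AttackPlayer send attack ready and over events to StateTreeQueue.
; Damage briefly flashes the mesh white, and death disables capsule collision.
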(event OnComponentBeginOverlap(CapsuleComponent)
  (params (OverlappedComponent :type Primitive%20Component%20Object%20Reference) (OtherActor :type Actor%20Object%20Reference) (OtherComp :type Primitive%20Component%20Object%20Reference) (OtherBodyIndex :type Integer) (bFromSweep :type Boolean) (SweepResult :type Hit%20Result%20Structure%20%28by%20ref%29))
  ;[1 1 1] On Hitting Something
  (Variables|Default|SetOther%20Actor OtherActor)
  (if (Variables|Default|GetCan%20Deal%20Damage?)
    (bind _asbp_oka_character (Utilities|Casting|CastToBP_OkaCharacter (Variables|Default|GetOther%20Actor)))
    (Utilities|FlowControl|DoOnce false :!label _label
      (:Completed
        (bind _returnvalue (Default|CheckActorLoc _asbp_oka_character self))
        (if (and _returnvalue (Variables|/Game/IvanaKupala/Oka/BP_OkaCharacter.BP_OkaCharacter_C|GetBlocking _asbp_oka_character))
          (Default|BlockedDamage _asbp_oka_character)
          (CallFunction|BlockedDamage)
          (else
            (Development|PrintString "Player attacked!")
            (Game|Damage|ApplyDamage (Variables|Default|GetOther%20Actor) (Variables|Default|GetDamage) 0 self)))
        (Utilities|FlowControl|Delay 1.0)
        (goto _label Reset)))))

(event EventCancelAttack
  (Animation|StopAnimMontage (Variables|Default|GetAttack%20Anim))
  ;[1 1 1] On Hitting Something
  (Utilities|FlowControl|DoOnce false) ; enters at Reset
)

(event EventOnDead
  (|CallParentFunction)
  (Collision|SetCollisionEnabled (Variables|Default|GetCapsuleComponent) "NoCollision"))

(event EventBeginPlay
  (|CallParentFunction)
  (Pawn|Components|CharacterMovement|SetMovementMode (Variables|Character|GetCharacterMovement) "MOVE_Walking" 0)
  (Variables|Default|SetStartLocation (Variables|/Script/Engine.SceneComponent|GetRelativeLocation (Variables|Character|GetMesh)))
  (Variables|Default|SetStartRotation (Transformation|GetActorRotation)))

(event EventAttackPlayer
  ;[1 1 1] Attack!
  (Utilities|FlowControl|Sequence
    (:then_0
      ;[1 1 1] On Hitting Something
      (Utilities|FlowControl|DoOnce false) ; enters at Reset
    )
    (:then_1
      (Utilities|FlowControl|DoOnce false :!label _label
        (:Completed
          (Utilities|FlowControl|Delay 1.0)
          (Default|AddEvent (Variables|Default|GetStateTreeQueue) "(TagName=\"AttackOver\")")
          (goto _label Reset))))))

(event EventDamageChageColor
  (Rendering|Material|SetMaterial (Variables|Character|GetMesh) 0 "/Game/IvanaKupala/Monsters/M_White.M_White")
  (Utilities|FlowControl|Delay 0.3)
  (Rendering|Material|SetMaterial (Variables|Character|GetMesh) 0 "/Game/IvanaKupala/Monsters/2_Deepwood/RedRaven/Textures/M_RedRaven.M_RedRaven"))

(event EventIdleWalk
  (if (not (Variables|Default|GetCan%20See%20Player?))
    (Utilities|FlowControl|DoOnce false :!label _label
      (:Completed
        (Animation|Montage|PlayMontage (Variables|Character|GetMesh) "/Game/IvanaKupala/Monsters/2_Deepwood/RedRaven/Animation/Red_Raven_Anim_root_Caw_Montage.Red_Raven_Anim_root_Caw_Montage"
          (:OnCompleted
            _)
          (:OnInterrupted
            _))
        (Utilities|FlowControl|Delay (Math|Random|RandomFloatinRange 5.0 3e+01))
        (goto _label Reset)))))

(event EventFollowPlayer
  (Default|AddEvent (Variables|Default|GetStateTreeQueue) "(TagName=\"AttackReady\")"))

(fn ConstructionScript
  (|CallParentFunction))