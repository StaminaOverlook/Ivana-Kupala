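; Red raven enemy that caws at random intervals until it spots the player (Oka), then makes a single dive attack if allowed.
; After a lift montage, timelines lerp it to the player's captured position without sweeping or homing.
; Sphere overlap either triggers the player's directional block or applies damage.
; After damage it drops and is destroyed on a delay; otherwise it flies up and away, then destroys itself.
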(event OnComponentBeginOverlap(Sphere)
  (params (OverlappedComponent :type Primitive%20Component%20Object%20Reference) (OtherActor :type Actor%20Object%20Reference) (OtherComp :type Primitive%20Component%20Object%20Reference) (OtherBodyIndex :type Integer) (bFromSweep :type Boolean) (SweepResult :type Hit%20Result%20Structure%20%28by%20ref%29))
  (bind _output_get (Variables|Default|SetOther%20Actor OtherActor))
  (bind _asbp_oka_character (Utilities|Casting|CastToBP_OkaCharacter _output_get))
  (Utilities|FlowControl|DoOnce false
    (:Completed
      (bind _returnvalue (Default|CheckActorLoc _asbp_oka_character self))
      (if (and _returnvalue (Variables|/Game/IvanaKupala/Oka/BP_OkaCharacter.BP_OkaCharacter_C|GetBlocking _asbp_oka_character))
        (Default|BlockedDamage _asbp_oka_character)
        (else
          (Development|PrintString "Player attacked!")
          (Game|Damage|ApplyDamage (Variables|Default|GetOther%20Actor) (Variables|Default|GetDamage) 0 self)
          (Variables|Default|Setdeal%20damage true)
          (Collision|SetCollisionEnabled (Variables|Default|GetSphere) "NoCollision")
          (Utilities|FlowControl|Delay 2.5)
          (Actor|DestroyActor))))))

(event OnSeePawn(PawnSensing)
  (params (Pawn :type Pawn%20Object%20Reference))
  (Utilities|FlowControl|DoOnce false
    (:Completed
      (if (Variables|Default|GetCanAttack)
        (bind _asbp_oka_character (Utilities|Casting|CastToBP_OkaCharacter Pawn))
        (Variables|Default|SetCaw false)
        (Animation|Montage|PlayMontage (Variables|Default|GetSkeletalMesh) "/Game/IvanaKupala/Monsters/2_Deepwood/RedRaven/Animation/Red_Raven_Anim_root_Lift_Montage.Red_Raven_Anim_root_Lift_Montage"
          (:OnCompleted
            (Variables|Default|SetStartFly_bool true)
            (Variables|Default|SetEndLocation (Transformation|GetActorLocation _asbp_oka_character))
            (bind _newtrack_0 (Timeline|Timeline PlayFromStart)
              (:Update
                (Transformation|SetActorLocation (Math|Vector|Lerp(Vector) (Variables|Default|GetStartLocation) (Variables|Default|GetEndLocation) _newtrack_0) false false))
              (:Finished
                (if (Variables|Default|Getdeal%20damage)
                  (bind _output_get (Variables|Default|SetStartLocation (Transformation|GetActorLocation)))
                  (Variables|Default|SetEndLocation (+ _output_get "0.000000,0.000000,-150.000000"))
                  (bind _newtrack_0_2 (Timeline|Timeline_1 PlayFromStart)
                    (:Update
                      (Transformation|SetActorLocation (Math|Vector|Lerp(Vector) (Variables|Default|GetStartLocation) (Variables|Default|GetEndLocation) _newtrack_0_2) false false)))
                  (else
                    (bind _output_get_2 (Variables|Default|SetStartLocation (Transformation|GetActorLocation)))
                    (Variables|Default|SetEndLocation (+ _output_get_2 "0.000000,-2000.000000,3000.000000"))
                    (bind _newtrack_0_3 (Timeline|Timeline_0 PlayFromStart)
                      (:Update
                        (Transformation|SetActorLocation (Math|Vector|Lerp(Vector) (Variables|Default|GetStartLocation) (Variables|Default|GetEndLocation) _newtrack_0_3) false false))
                      (:Finished
                        (Actor|DestroyActor)))))))))))))

(event Custom|IdleCaw
  (Variables|Default|SetCaw true)
  (Utilities|FlowControl|Delay 1.6)
  (Variables|Default|SetCaw false)
  (Utilities|FlowControl|Delay (Math|Random|RandomFloatinRange 5.0 3e+01))
  (CallFunction|IdleCaw))

(event EventBeginPlay
  (Variables|Default|SetStartLocation (Transformation|GetActorLocation))
  (Utilities|FlowControl|Delay 2.0)
  (CallFunction|IdleCaw))

(fn ConstructionScript)