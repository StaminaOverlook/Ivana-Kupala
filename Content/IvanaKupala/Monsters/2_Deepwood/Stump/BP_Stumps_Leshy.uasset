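; Stump variant for the Leshy boss, a child Blueprint that reports its death to the boss.
; On BeginPlay it runs the parent logic, then sets Alive to false.
; On death it calls the parent handler, then decrements NumStumps on the first BP_Leshy_Boss found through GetAllActorsOfClass, with no validity check.
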(event EventBeginPlay
  (|CallParentFunction)
  (Variables|Default|SetAlive false))

(event Collision|EventActorBeginOverlap
  (params (OtherActor :type Actor%20Object%20Reference)))

(event EventTick
  (params (DeltaSeconds :type Float%20%28single-precision%29)))

(event EventOnDead
  (|CallParentFunction)
  (bind _outactors (Actor|GetAllActorsOfClass "/Game/IvanaKupala/Monsters/2_Deepwood/LESHY/BP_Leshy_Boss.BP_Leshy_Boss_C"))
  (Variables|/Game/IvanaKupala/Monsters/2_Deepwood/LESHY/BP_Leshy_Boss.BP_Leshy_Boss_C|SetNumStumps (Utilities|Array|Get(acopy) _outactors) (- (Variables|/Game/IvanaKupala/Monsters/2_Deepwood/LESHY/BP_Leshy_Boss.BP_Leshy_Boss_C|GetNumStumps (Utilities|Array|Get(acopy) _outactors)) 1)))

(fn ConstructionScript
  (|CallParentFunction))