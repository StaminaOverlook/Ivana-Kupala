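; Rotating four-piece wood shield for the Leshy boss, attached as a child actor of BP_Leshy_Boss.
; It starts hidden and non-colliding, then shows its shields and enables their overlap boxes when the boss fires its StartWoodShield event.
; A coal or fire coal hitting a box destroys the coal and disables that piece.
; When the remaining count reaches zero, it calls its ShieldOff dispatcher.
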(event OnComponentBeginOverlap(Box)
  (params (OverlappedComponent :type Primitive%20Component%20Object%20Reference) (OtherActor :type Actor%20Object%20Reference) (OtherComp :type Primitive%20Component%20Object%20Reference) (OtherBodyIndex :type Integer) (bFromSweep :type Boolean) (SweepResult :type Hit%20Result%20Structure%20%28by%20ref%29))
  (bind _returnvalue (Utilities|GetClass OtherActor))
  ;[1 1 1] WoodShield Destroy
  (if (or (== _returnvalue "/Game/IvanaKupala/Oka/Skills/CauldronSkills/BP_Coal.BP_Coal_C") (== _returnvalue "/Game/IvanaKupala/Oka/Skills/CauldronSkills/BP_FireCoal.BP_FireCoal_C"))
    (Variables|/Script/Engine.PrimitiveComponent|SetbGenerateOverlapEvents OverlappedComponent false)
    (Rendering|SetVisibility OverlappedComponent false false)
    (Collision|SetCollisionEnabled (Variables|Default|Getshield) "NoCollision")
    (Actor|DestroyActor OtherActor)
    (Variables|Default|SetShieldRemaining (- (Variables|Default|GetShieldRemaining) 1))
    (CallFunction|CheckShield)))

(event OnComponentBeginOverlap(Box1)
  (params (OverlappedComponent :type Primitive%20Component%20Object%20Reference) (OtherActor :type Actor%20Object%20Reference) (OtherComp :type Primitive%20Component%20Object%20Reference) (OtherBodyIndex :type Integer) (bFromSweep :type Boolean) (SweepResult :type Hit%20Result%20Structure%20%28by%20ref%29))
  (bind _returnvalue (Utilities|GetClass OtherActor))
  ;[1 1 1] WoodShield Destroy
  (if (or (== _returnvalue "/Game/IvanaKupala/Oka/Skills/CauldronSkills/BP_Coal.BP_Coal_C") (== _returnvalue "/Game/IvanaKupala/Oka/Skills/CauldronSkills/BP_FireCoal.BP_FireCoal_C"))
    (Variables|/Script/Engine.PrimitiveComponent|SetbGenerateOverlapEvents OverlappedComponent false)
    (Rendering|SetVisibility OverlappedComponent false false)
    (Collision|SetCollisionEnabled (Variables|Default|Getshield1) "NoCollision")
    (Actor|DestroyActor OtherActor)
    (Variables|Default|SetShieldRemaining (- (Variables|Default|GetShieldRemaining) 1))
    (CallFunction|CheckShield)))

(event OnComponentBeginOverlap(Box2)
  (params (OverlappedComponent :type Primitive%20Component%20Object%20Reference) (OtherActor :type Actor%20Object%20Reference) (OtherComp :type Primitive%20Component%20Object%20Reference) (OtherBodyIndex :type Integer) (bFromSweep :type Boolean) (SweepResult :type Hit%20Result%20Structure%20%28by%20ref%29))
  (bind _returnvalue (Utilities|GetClass OtherActor))
  ;[1 1 1] WoodShield Destroy
  (if (or (== _returnvalue "/Game/IvanaKupala/Oka/Skills/CauldronSkills/BP_Coal.BP_Coal_C") (== _returnvalue "/Game/IvanaKupala/Oka/Skills/CauldronSkills/BP_FireCoal.BP_FireCoal_C"))
    (Variables|/Script/Engine.PrimitiveComponent|SetbGenerateOverlapEvents OverlappedComponent false)
    (Rendering|SetVisibility OverlappedComponent false false)
    (Collision|SetCollisionEnabled (Variables|Default|Getshield2) "NoCollision")
    (Actor|DestroyActor OtherActor)
    (Variables|Default|SetShieldRemaining (- (Variables|Default|GetShieldRemaining) 1))
    (CallFunction|CheckShield)))

(event OnComponentBeginOverlap(Box3)
  (params (OverlappedComponent :type Primitive%20Component%20Object%20Reference) (OtherActor :type Actor%20Object%20Reference) (OtherComp :type Primitive%20Component%20Object%20Reference) (OtherBodyIndex :type Integer) (bFromSweep :type Boolean) (SweepResult :type Hit%20Result%20Structure%20%28by%20ref%29))
  (bind _returnvalue (Utilities|GetClass OtherActor))
  ;[1 1 1] WoodShield Destroy
  (if (or (== _returnvalue "/Game/IvanaKupala/Oka/Skills/CauldronSkills/BP_Coal.BP_Coal_C") (== _returnvalue "/Game/IvanaKupala/Oka/Skills/CauldronSkills/BP_FireCoal.BP_FireCoal_C"))
    (Variables|/Script/Engine.PrimitiveComponent|SetbGenerateOverlapEvents OverlappedComponent false)
    (Rendering|SetVisibility OverlappedComponent false false)
    (Collision|SetCollisionEnabled (Variables|Default|Getshield3) "NoCollision")
    (Actor|DestroyActor OtherActor)
    (Variables|Default|SetShieldRemaining (- (Variables|Default|GetShieldRemaining) 1))
    (CallFunction|CheckShield)))

(event Custom|CheckShield
  (if (== (Variables|Default|GetShieldRemaining) 0)
    (Default|CallShieldOff)))

(event Custom|StartWoodShield_Event
  (Variables|Default|SetShieldRemaining 4)
  (for _array_element (Variables|Default|GetShildArray)
    (Collision|SetCollisionEnabled _array_element "QueryAndPhysics")
    (Rendering|SetVisibility _array_element true false))
  (for _array_element_2 (Variables|Default|GetShieldBoxArray)
    (Variables|/Script/Engine.PrimitiveComponent|SetbGenerateOverlapEvents _array_element_2 true)))

(event EventBeginPlay
  (bind _asbp_leshy_boss (Utilities|Casting|CastToBP_Leshy_Boss (Actor|GetParentActor self)))
  (bind _output_get (Variables|Default|SetAs%20BP%20Leshy%20Boss _asbp_leshy_boss))
  (EventDispatchers|AssignStartWoodShield _output_get (delegate Custom|StartWoodShield_Event))
  (Variables|Default|SetShieldBoxArray (Utilities|Array|MakeArray (Variables|Default|GetBox) (Variables|Default|GetBox1) (Variables|Default|GetBox2) (Variables|Default|GetBox3)))
  (bind _output_get_2 (Variables|Default|SetShildArray (Utilities|Array|MakeArray (Variables|Default|Getshield) (Variables|Default|Getshield1) (Variables|Default|Getshield2) (Variables|Default|Getshield3))))
  (for _array_element _output_get_2
    (Rendering|SetVisibility _array_element false false)
    (Collision|SetCollisionEnabled _array_element "NoCollision"))
  (for _array_element_2 (Variables|Default|GetShieldBoxArray)
    (Rendering|SetVisibility _array_element_2 false false)))

(event EventTick
  (params (DeltaSeconds :type Float%20%28single-precision%29))
  (Transformation|AddRelativeRotation (Variables|Default|GetDefaultSceneRoot) "0.000000,0.500000,0.000000" false false))

(fn ConstructionScript)