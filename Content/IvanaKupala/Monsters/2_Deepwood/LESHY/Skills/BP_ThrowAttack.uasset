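; BP_ThrowAttack is a thrown projectile for the Leshy monster that spawns a BP_Stumps_Leshy where it comes to rest.
; BeginPlay applies the stored Vilocity to ProjectileMovement and starts a lifetime timer that destroys the actor.
; Tick polls for near-zero velocity, then once spawns the stump slightly raised, copies its Alive value, hides the mesh, disables its collision and destroys itself after a delay.
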(event EventBeginPlay
  (Variables|/Script/Engine.MovementComponent|SetVelocity (Variables|Default|GetProjectileMovement) (Variables|Default|GetVilocity))
  (Utilities|FlowControl|Delay 5.0)
  (Actor|DestroyActor))

(event EventTick
  (params (DeltaSeconds :type Float%20%28single-precision%29))
  (bind _returnvalue (Transformation|GetActorLocation))
  (bind _staticmesh (Variables|Default|GetStaticMesh))
  (if (Utilities|Operators|EqualEqual :A (Variables|/Script/Engine.MovementComponent|GetVelocity (Variables|Default|GetProjectileMovement)) :ErrorTolerance 0.01)
    (Utilities|FlowControl|DoOnce false
      (:Completed
        (bind _returnvalue_2 (Game|SpawnActorfromClass "/Game/IvanaKupala/Monsters/2_Deepwood/Stump/BP_Stumps_Leshy.BP_Stumps_Leshy_C" (Math|Transform|MakeTransform (Math|Vector|MakeVector (.x _returnvalue) (.y _returnvalue) (+ (.z _returnvalue) 5e+01)) "0, 0, 0" "1.000000,1.000000,1.000000") "Undefined" "MultiplyWithRoot" 0 0))
        (Variables|Default|SetAlive (Variables|/Game/IvanaKupala/Monsters/2_Deepwood/Stump/BP_Stumps_Leshy.BP_Stumps_Leshy_C|GetAlive _returnvalue_2))
        (Collision|SetCollisionEnabled _staticmesh "NoCollision")
        (Development|SetHiddeninGame _staticmesh true false)
        (Utilities|FlowControl|Delay 3.0)
        (Actor|DestroyActor)))))

(event Collision|EventActorBeginOverlap
  (params (OtherActor :type Actor%20Object%20Reference)))

(fn ConstructionScript)