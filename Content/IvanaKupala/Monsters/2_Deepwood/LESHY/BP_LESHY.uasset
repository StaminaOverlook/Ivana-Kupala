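; BP_LESHY is the Leshy character in Deepwood, set up as an interactable NPC with dialogue-driven appearance and exit.
; It becomes interactable on BeginPlay and when the movement-stop event fires.
; AppearNPC plays the appear montage, then re-enables interaction and calls VisibalityOn.
; EndDialogue plays the disappear montage and destroys the actor once it completes.
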(event Custom|Activate%20Interactable
  (params (ImpactResult :type Hit%20Result%20Structure%20%28by%20ref%29) (Time :type Float%20%28single-precision%29))
  ;[1 1 1] On Movement Stop
  (Variables|Default|SetInteractable true))

(event EventEndDialogue
  ;[1 1 1] Disappear
  (Animation|Montage|PlayMontage (Variables|Default|GetLeshy) "/Game/IvanaKupala/Monsters/2_Deepwood/LESHY/Animations/Leshy_Disappear_for_NPC_Montage.Leshy_Disappear_for_NPC_Montage"
    (:OnCompleted
      (Actor|DestroyActor))))

(event Collision|EventActorBeginOverlap
  (params (OtherActor :type Actor%20Object%20Reference))
  (|CallParentFunction OtherActor) ; This node is disabled and will not be called.\nDrag off pins to build functionality.
)

(event EventTick
  (params (DeltaSeconds :type Float%20%28single-precision%29))
  (|CallParentFunction DeltaSeconds) ; This node is disabled and will not be called.\nDrag off pins to build functionality.
)

(event EventAppearNPC
  (params (Location :type Vector :default "0, 0, 0"))
  ;[1 1 1] On Appear NPC
  (Animation|Montage|PlayMontage (Variables|Default|GetLeshy) "/Game/IvanaKupala/Monsters/2_Deepwood/LESHY/Animations/Leshy_Appear_for_NPC_Montage_For_NPC.Leshy_Appear_for_NPC_Montage_For_NPC"
    (:OnCompleted
      (Variables|Default|SetInteractable true)
      (CallFunction|Visibalityon))))

(event EventBeginPlay
  ;[1 1 1] Begin Play
  (Variables|Default|SetInteractable true))

(fn ConstructionScript
  (|CallParentFunction))