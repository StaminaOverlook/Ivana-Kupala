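; Leshy boss of the Deepwood monsters, driven by a state tree through queued events.
; It waits frozen, sensing off and invulnerable, until the reveal montage starts the fight and boss health widget.
; Its attack spawns a cone of roots aimed at the player; ThrowAttack is an empty stub.
; Health thresholds each trigger once an invulnerable injured-then-wood-shield montage sequence; death fades music and plays a dying montage.
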(event Custom|WoodShield
  ;[1 1 1] Wood Shield
  (Animation|Montage|PlayMontage (Variables|Character|GetMesh) "/Game/IvanaKupala/Monsters/2_Deepwood/LESHY/Animations/Leshy_Summon_Defense_Montage.Leshy_Summon_Defense_Montage"))

(event Custom|Spawn%20amination
  ;[1 1 1] BEGIN BATTLE
  (Variables|/Script/Engine.SkeletalMeshComponent|SetbPauseAnims (Variables|Character|GetMesh) false)
  (Animation|Montage|PlayMontage (Variables|Character|GetMesh) "/Game/IvanaKupala/Monsters/2_Deepwood/LESHY/Animations/New_leshy/Leshy_2_Reveal_Montage.Leshy_2_Reveal_Montage"
    (:OnCompleted
      _)
    (:OnInterrupted
      _))
  (CallFunction|SendMonsterStateEvent "(TagName=\"Boss.Start\")")
  (Class|PawnSensingComponent|SetSensingUpdatesEnabled (Variables|Default|GetPawnSensing) true)
  (CallFunction|InitHealthWidget))

(event Custom|RootAttack
  (bind _returnvalue (Transformation|GetActorLocation))
  (bind _returnvalue_2 (Transformation|GetActorLocation))
  (bind _returnvalue_3 (Game|GetPlayerCharacter 0))
  (bind _returnvalue_4 (Transformation|GetActorLocation _returnvalue_3))
  (bind _returnvalue_5 (Math|Rotator|FindLookatRotation _returnvalue_2 _returnvalue_4))
  ;[1 1 1] Root Attack
  (Animation|Montage|PlayMontage (Variables|Character|GetMesh) "/Game/IvanaKupala/Monsters/2_Deepwood/LESHY/Animations/New_leshy/Leshy_2_Root_Attack_Montage.Leshy_2_Root_Attack_Montage"
    (:then
      (Utilities|FlowControl|Delay 1.0)
      (for _array_element (Variables|Default|GetRootCone)
        (Game|SpawnActorfromClass "/Game/IvanaKupala/Monsters/2_Deepwood/EvilTree/Skills/BP_RootAttack.BP_RootAttack_C" (Math|Transform|MakeTransform (Math|Vector|MakeVector (.x _returnvalue) (.y _returnvalue) 5e+01) (Math|Rotator|MakeRotator (.roll _returnvalue_5) (.pitch _returnvalue_5) (+ (.yaw _returnvalue_5) _array_element)) "1.000000,1.000000,1.000000") "Undefined" "MultiplyWithRoot" 0 0))
      (CallFunction|SendMonsterStateEvent "(TagName=\"AttackOver\")"))))

(event Custom|ThrowAttack
  ;[1 1 1] Throw Attack
)

(event Custom|Stop%20anim
  (Animation|Montage|PlayMontage (Variables|Character|GetMesh) "/Game/IvanaKupala/Monsters/2_Deepwood/LESHY/Animations/Leshy_Reveal_Montage.Leshy_Reveal_Montage"
    (:then
      (Utilities|FlowControl|Delay 0.2)
      (Variables|/Script/Engine.SkeletalMeshComponent|SetbPauseAnims (Variables|Character|GetMesh) true)
      (Development|PrintString "Hello" true true "(R=1.000000,G=0.027105,B=0.000000,A=1.000000)"))))

(event Custom|On%20Damaged
  (params (NewHealth :type Float%20%28double-precision%29) (Amount :type Float%20%28double-precision%29))
  ;[1 1 1] BEGIN PLAY
  (CallFunction|OnDamaged 0.0 0.0)
  (Utilities|FlowControl|Sequence
    (:then_0
      (if (<= (Variables|/Game/IvanaKupala/Interface/HealthComponent.HealthComponent_C|GetHealth (Variables|Default|GetHealthComponent)) 75.0)
        (Utilities|FlowControl|DoOnce false
          (:Completed
            (Variables|Default|SetbCanBeDamaged false :!label _label)
            (Animation|Montage|PlayMontage (Variables|Character|GetMesh) "/Game/IvanaKupala/Monsters/2_Deepwood/LESHY/Animations/Leshy_Injured_Montage.Leshy_Injured_Montage"
              (:OnCompleted
                (CallFunction|WoodShield)))))))
    (:then_1
      (if (<= (Variables|/Game/IvanaKupala/Interface/HealthComponent.HealthComponent_C|GetHealth (Variables|Default|GetHealthComponent)) 5e+01)
        (Utilities|FlowControl|DoOnce false
          (:Completed
            (goto _label)))))
    (:then_2
      (if (<= (Variables|/Game/IvanaKupala/Interface/HealthComponent.HealthComponent_C|GetHealth (Variables|Default|GetHealthComponent)) 25.0)
        (Utilities|FlowControl|DoOnce false
          (:Completed
            (goto _label)))))))

(event EventBeginPlay
  (bind _healthcomponent (Variables|Default|GetHealthComponent))
  ;[1 1 1] BEGIN PLAY
  (Variables|Default|SetbCanBeDamaged false)
  (Components|DestroyComponent (Variables|Default|GetWidgetHealth))
  (EventDispatchers|BindEventtoDamaged _healthcomponent (delegate Custom|On%20Damaged))
  (EventDispatchers|BindEventtoDead _healthcomponent (delegate EventOnDead))
  (CallFunction|StopAnim))

(event EventOnDead
  ;[1 1 1] On Dead
  (Class|PawnSensingComponent|SetSensingUpdatesEnabled (Variables|Default|GetPawnSensing) false)
  (bind _asbp_top_down_game_mode (Utilities|Casting|CastToBP_TopDownGameMode (Game|GetGameMode)))
  (Default|FadeBGM _asbp_top_down_game_mode)
  (Default|AddEvent (Variables|Default|GetStateTreeQueue) "(TagName=\"Dead\")"))

(event EventFollowPlayer
  ;[1 1 1] Follow Player
  (Utilities|FlowControl|Delay 1.0)
  (CallFunction|SendMonsterStateEvent "(TagName=\"AttackReady\")"))

(event EventAttackPlayer
  ;[1 1 1] Follow Player
  (CallFunction|RootAttack))

(event EventStartDeadState
  (bind _capsulecomponent (Variables|Default|GetCapsuleComponent))
  ;[1 1 1] On Dead
  (Collision|SetCollisionEnabled _capsulecomponent "NoCollision")
  (Variables|/Script/Engine.PrimitiveComponent|SetbGenerateOverlapEvents _capsulecomponent false)
  (bind _returnvalue (CallFunction|IsMontagePlaying (Variables|Default|GetDeath%20Anim)))
  (if (not _returnvalue)
    (Animation|Montage|PlayMontage (Variables|Character|GetMesh) "/Game/IvanaKupala/Monsters/2_Deepwood/LESHY/Animations/Leshy_Dying_Montage.Leshy_Dying_Montage"
      (:then
        (Utilities|FlowControl|Delay 5.0)
        (Default|CallOnDeath)))))

(event EventInitHealthWidget
  ;[1 1 1] Init Health Widget
  (bind _returnvalue (UserInterface|CreateWidget "/Game/IvanaKupala/Interface/WB_BossHealth.WB_BossHealth_C"))
  (UserInterface|SetWidget (Variables|Default|GetWidgetHealth) _returnvalue)
  (Default|InitWidget _returnvalue (Variables|Default|GetHealthComponent) "ЛЕШИЙ")
  (Variables|Default|SetbCanBeDamaged true))

(event EventDamageChageColor
  (Rendering|Material|SetMaterial (Variables|Character|GetMesh) 0 "/Game/IvanaKupala/Monsters/M_White.M_White")
  (Utilities|FlowControl|Delay 0.3)
  (Rendering|Material|SetMaterial (Variables|Character|GetMesh) 0 "/Game/IvanaKupala/Monsters/1_Dubrava/BEAR_MOTHER/Textures/Bear_Material.Bear_Material"))

(fn ConstructionScript
  (bind _statetreequeue (Variables|Default|GetStateTreeQueue))
  (Default|ConnectStateTree _statetreequeue (Variables|Default|GetMonsterStateTree))
  (Default|AddEvent _statetreequeue "(TagName=\"Boss.Init\")")
  (Class|PawnSensingComponent|SetSensingUpdatesEnabled (Variables|Default|GetPawnSensing) false))