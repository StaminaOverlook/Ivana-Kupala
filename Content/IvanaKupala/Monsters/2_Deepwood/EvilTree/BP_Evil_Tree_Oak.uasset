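; Evil oak tree monster that senses the player, reveals its health bar and reports to its StateTree through queued events.
; Attacks spawn a cooldown-limited root attack at long range, or pick a directional montage from facing dot products up close.
; Box overlaps deal damage once per swing unless blocked.
; Death bakes each material to a render target for a burn transition, plays the death montage, then destroys the actor.
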(event OnSeePawn(PawnSensing)
  (params (Pawn :type Pawn%20Object%20Reference))
  (Utilities|FlowControl|Sequence
    (:then_0
      (if (not (Variables|Default|GetCan%20See%20Player?))
        (bind _returnvalue (CallFunction|IsMontagePlaying (Variables|Default|GetInjured%20Anim)))
        (if (not _returnvalue)
          (Default|AddEvent (Variables|Default|GetStateTreeQueue) "(TagName=\"Noticed\")"))))
    (:then_1
      (Utilities|FlowControl|DoOnce false
        (:Completed
          (bind _aswb_monster_health (Utilities|Casting|CastToWB_MonsterHealth (UserInterface|GetWidget (Variables|Default|GetWidgetHealth))))
          (Default|InitWidget _aswb_monster_health (Variables|Default|GetHealthComponent))
          (Development|SetHiddeninGame (Variables|Default|GetWidgetHealth) false false))))))

(event OnComponentBeginOverlap(Box)
  (params (OverlappedComponent :type Primitive%20Component%20Object%20Reference) (OtherActor :type Actor%20Object%20Reference) (OtherComp :type Primitive%20Component%20Object%20Reference) (OtherBodyIndex :type Integer) (bFromSweep :type Boolean) (SweepResult :type Hit%20Result%20Structure%20%28by%20ref%29))
  ;[1 1 1] Cancel Attak
  (if (Variables|Default|GetCan%20Deal%20Damage?)
    (bind _output_get (Variables|Default|SetOther%20Actor OtherActor))
    (bind _asbp_oka_character (Utilities|Casting|CastToBP_OkaCharacter _output_get))
    (Utilities|FlowControl|DoOnce false :!label _label
      (:Completed
        (bind _returnvalue (Default|CheckActorLoc _asbp_oka_character self))
        (if (and _returnvalue (Variables|/Game/IvanaKupala/Oka/BP_OkaCharacter.BP_OkaCharacter_C|GetBlocking _asbp_oka_character))
          (Default|BlockedDamage _asbp_oka_character)
          (CallFunction|BlockedDamage)
          (else
            (Development|PrintString "Player attacked!")
            (Game|Damage|ApplyDamage (Variables|Default|GetOther%20Actor) (Variables|Default|GetDamage) 0 self)))
        (Utilities|FlowControl|Delay 1.0)
        (goto _label Reset)))))

(event Custom|ReloadRootAttack
  ;[1 1 1] Attack!
  (Utilities|FlowControl|Delay 1e+01)
  (Variables|Default|SetRootAttack true))

(event EventCancelAttack
  ;[1 1 1] Cancel Attak
  (Animation|StopAnimMontage (Variables|Default|GetAttack%20Anim))
  (Utilities|FlowControl|DoOnce false) ; enters at Reset
)

(event EventOnDead
  (|CallParentFunction)
  (Collision|SetCollisionEnabled (Variables|Default|GetCapsuleComponent) "NoCollision"))

(event EventFollowPlayer
  (Utilities|FlowControl|DoOnce false :!label _label
    (:Completed
      (Utilities|FlowControl|Delay 1.0)
      (Default|AddEvent (Variables|Default|GetStateTreeQueue) "(TagName=\"AttackReady\")")
      (goto _label Reset))))

(event EventAttackPlayer
  (bind _returnvalue (Transformation|GetActorRotation))
  (bind _returnvalue_2 (Transformation|GetActorLocation))
  (bind _returnvalue_3 (Game|GetPlayerCharacter 0))
  (bind _returnvalue_4 (Transformation|GetActorLocation))
  (bind _returnvalue_5 (Math|Vector|GetForwardVector _returnvalue))
  (bind _returnvalue_6 (Transformation|GetActorLocation _returnvalue_3))
  (bind _returnvalue_7 (Math|Vector|GetRightVector _returnvalue))
  (bind _returnvalue_8 (- _returnvalue_6 _returnvalue_4))
  (bind _returnvalue_9 (Class|KismetMathLibrary|VectorCosineAngle2D _returnvalue_8 _returnvalue_7))
  (bind _returnvalue_10 (Class|KismetMathLibrary|VectorCosineAngle2D _returnvalue_8 _returnvalue_5))
  (bind _returnvalue_11 (Math|Float|Absolute(Float) _returnvalue_10))
  (bind _returnvalue_12 (> _returnvalue_9 0.0))
  (bind _returnvalue_13 (> _returnvalue_11 0.45))
  ;[1 1 1] Attack!
  (Utilities|FlowControl|DoOnce false :!label _label
    (:Completed
      (Utilities|FlowControl|Sequence
        (:then_0
          ;[1 1 1] Cancel Attak
          (Utilities|FlowControl|DoOnce false) ; enters at Reset
        )
        (:then_1
          (if (> (Math|Vector|Distance(Vector) _returnvalue_6 _returnvalue_4) 6e+02)
            (if (Variables|Default|GetRootAttack)
              (Variables|Default|SetRootAttack false)
              (Game|SpawnActorfromClass "/Game/IvanaKupala/Monsters/2_Deepwood/EvilTree/Skills/BP_RootAttack.BP_RootAttack_C" (Math|Transform|MakeTransform (Math|Vector|MakeVector (.x _returnvalue_2) (.y _returnvalue_2) (- (.z _returnvalue_2) 3e+02)) (Math|Rotator|FindLookatRotation (Transformation|GetActorLocation) (Transformation|GetActorLocation (Game|GetPlayerCharacter 0))) "1.000000,1.000000,1.000000") "Undefined" "MultiplyWithRoot" 0 0)
              (CallFunction|ReloadRootAttack))
            (else
              (if (> _returnvalue_10 0.0)
                (if _returnvalue_13
                  (Animation|Montage|PlayMontage (Variables|Character|GetMesh) "/Game/IvanaKupala/Monsters/2_Deepwood/EvilTree/Animations/Evil_Tree_oak__1__Anim_Attack_Montage.Evil_Tree_oak__1__Anim_Attack_Montage"
                    (:OnCompleted
                      _)
                    (:OnInterrupted
                      (Utilities|FlowControl|Delay 3.0 :!label _label_2)))
                  (elif _returnvalue_12
                    (Animation|Montage|PlayMontage (Variables|Character|GetMesh) "/Game/IvanaKupala/Monsters/2_Deepwood/EvilTree/Animations/Evil_Tree_oak__1__Anim_Attack_Right_Montage.Evil_Tree_oak__1__Anim_Attack_Right_Montage" :!label _label_3
                      (:OnCompleted
                        _)
                      (:OnInterrupted
                        (goto _label_2)))
                    (else
                      (Animation|Montage|PlayMontage (Variables|Character|GetMesh) "/Game/IvanaKupala/Monsters/2_Deepwood/EvilTree/Animations/Evil_Tree_oak__1__Anim_Attack_Left_Montage.Evil_Tree_oak__1__Anim_Attack_Left_Montage" :!label _label_4
                        (:OnCompleted
                          _)
                        (:OnInterrupted
                          (goto _label_2))))))
                (elif _returnvalue_13
                  (Animation|Montage|PlayMontage (Variables|Character|GetMesh) "/Game/IvanaKupala/Monsters/2_Deepwood/EvilTree/Animations/Evil_Tree_oak__1__Anim_root_Attack_Behind_Montage.Evil_Tree_oak__1__Anim_root_Attack_Behind_Montage"
                    (:OnCompleted
                      _)
                    (:OnInterrupted
                      (goto _label_2)))
                  (elif _returnvalue_12
                    (goto _label_3)
                    (else
                      (goto _label_4)))))
              (Utilities|FlowControl|Delay 0.2)))
          (Default|AddEvent (Variables|Default|GetStateTreeQueue) "(TagName=\"AttackOver\")")
          (goto _label Reset))))))

(event EventDamageChageColor
  (Rendering|Material|SetMaterial (Variables|Character|GetMesh) 0 "/Game/IvanaKupala/Monsters/M_White.M_White")
  (Utilities|FlowControl|Delay 0.3)
  (Rendering|Material|SetMaterial (Variables|Character|GetMesh) 0 "/Game/IvanaKupala/Monsters/2_Deepwood/EvilTree/Textures/OakMaterial.OakMaterial"))

(event EventInitHealthWidget
  (Development|SetHiddeninGame (Variables|Default|GetWidgetHealth) true false))

(event EventIdleWalk)

(event EventHearNoise
  (Utilities|FlowControl|Sequence
    (:then_0
      (if (not (Variables|Default|GetCan%20See%20Player?))
        (bind _returnvalue (CallFunction|IsMontagePlaying (Variables|Default|GetInjured%20Anim)))
        (if (not _returnvalue)
          (Default|AddEvent (Variables|Default|GetStateTreeQueue) "(TagName=\"Noticed\")"))))
    (:then_1
      (Utilities|FlowControl|DoOnce false
        (:Completed
          (bind _aswb_monster_health (Utilities|Casting|CastToWB_MonsterHealth (UserInterface|GetWidget (Variables|Default|GetWidgetHealth))))
          (Default|InitWidget _aswb_monster_health (Variables|Default|GetHealthComponent))
          (Development|SetHiddeninGame (Variables|Default|GetWidgetHealth) false false))))))

(event EventStartDeadState
  (bind _death_anim (Variables|Default|GetDeath%20Anim))
  (bind _capsulecomponent (Variables|Default|GetCapsuleComponent))
  (bind _mesh (Variables|Character|GetMesh))
  (Components|DestroyComponent (Variables|Default|GetPawnSensing))
  (Collision|SetCollisionEnabled _capsulecomponent "NoCollision")
  (Variables|/Script/Engine.PrimitiveComponent|SetbGenerateOverlapEvents _capsulecomponent false)
  (bind _returnvalue (CallFunction|IsMontagePlaying _death_anim))
  (if (not _returnvalue)
    (for (_array_element _array_index) (Rendering|Material|GetMaterials _mesh)
      (bind _returnvalue_2 (CanvasRenderTarget2D|CreateCanvasRenderTarget2D 0 1024 1024))
      (Rendering|DrawMaterialtoRenderTarget _returnvalue_2 _array_element)
      (bind _returnvalue_3 (Rendering|Material|CreateDynamicMaterialInstance _mesh _array_index "/Game/IvanaKupala/Maps/Transitions/Transition_Mat.Transition_Mat" "Burn" :!class /Script/Engine.PrimitiveComponent))
      (Rendering|Material|SetTextureParameterValue _returnvalue_3 "BurnTexture" _returnvalue_2)
      (Rendering|Material|SetScalarParameterValueonMaterials _mesh "BurnStart" (Utilities|Time|GetRealTimeSeconds))
      (Animation|Montage|PlayMontage (Variables|Character|GetMesh) _death_anim 1.0 0.0 "Dying" ; Death Animation here
        (:then
          (Default|CallOnDeath)
          (Utilities|FlowControl|Delay 4.0)
          (Actor|DestroyActor))))))

(fn ConstructionScript
  (|CallParentFunction))