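; Root attack skill actor for the EvilTree monster that travels in a straight horizontal line toward the player and damages them.
; After a brief delay on spawn, it locks a flattened direction to the player's current position without homing.
; A timeline lerps it along that fixed path without sweeping, then destroys it.
; Its sphere overlap applies RootDamage only to BP_OkaCharacter.
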(event OnComponentBeginOverlap(Sphere)
  (params (OverlappedComponent :type Primitive%20Component%20Object%20Reference) (OtherActor :type Actor%20Object%20Reference) (OtherComp :type Primitive%20Component%20Object%20Reference) (OtherBodyIndex :type Integer) (bFromSweep :type Boolean) (SweepResult :type Hit%20Result%20Structure%20%28by%20ref%29))
  (bind _asbp_oka_character (Utilities|Casting|CastToBP_OkaCharacter OtherActor))
  (Game|Damage|ApplyDamage _asbp_oka_character (Variables|Default|GetRootDamage) 0 self))

(event EventBeginPlay
  (bind _returnvalue (Transformation|GetActorLocation))
  (Utilities|FlowControl|Delay 0.2)
  (Variables|Default|SetEndPoint (+ _returnvalue (* (Class|KismetMathLibrary|VectorNormal2D (- (Transformation|GetActorLocation (Game|GetPlayerCharacter 0)) _returnvalue) 0.0001) 5e+03)))
  (Variables|Default|SetStartPoint (Transformation|GetActorLocation))
  (bind _newtrack_0 (Timeline|Timeline PlayFromStart)
    (:Update
      (Transformation|SetActorLocation (Math|Vector|Lerp(Vector) (Variables|Default|GetStartPoint) (Variables|Default|GetEndPoint) _newtrack_0) false false))
    (:Finished
      (Actor|DestroyActor))))

(fn ConstructionScript)