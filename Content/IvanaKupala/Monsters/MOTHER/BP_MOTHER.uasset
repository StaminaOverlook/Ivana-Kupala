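; Boss monster Alkonost, Gleb's Mother, with a boss health bar and death that kills all Kikimora minions.
; Events queued to a State Tree drive its states as it turns toward the player and attacks.
; It picks beak or wing montages, or summons spawner waves at one-shot health thresholds, attacking faster as health drops.
; Head and wing overlaps deal damage, unless the player's block passes a location check and staggers the boss.
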(event OnComponentBeginOverlap(WingWeaponR)
  (params (OverlappedComponent :type Primitive%20Component%20Object%20Reference) (OtherActor :type Actor%20Object%20Reference) (OtherComp :type Primitive%20Component%20Object%20Reference) (OtherBodyIndex :type Integer) (bFromSweep :type Boolean) (SweepResult :type Hit%20Result%20Structure%20%28by%20ref%29))
  ;[1 1 1] On Hitting Something
  (if (Variables|Default|GetCan%20Deal%20Damage?)
    (Variables|Default|SetOther%20Actor OtherActor)
    (Utilities|FlowControl|DoOnce false :!label _label
      (:Completed
        (bind _asbp_top_down_character (Utilities|Casting|CastToBP_TopDownCharacter (Variables|Default|GetOther%20Actor)))
        (bind _returnvalue (Default|CheckActorLoc _asbp_top_down_character self))
        (if (and _returnvalue (Variables|/Game/IvanaKupala/Oka/BP_TopDownCharacter.BP_TopDownCharacter_C|GetBlocking _asbp_top_down_character))
          (Default|BlockedDamage _asbp_top_down_character)
          (CallFunction|BlockedDamage)
          (else
            (Development|PrintString "Player attacked!")
            (Game|Damage|ApplyDamage (Variables|Default|GetOther%20Actor) (Variables|Default|GetDamage) 0 self)))
        (Utilities|FlowControl|Delay 1.0)
        (goto _label Reset)))))

(event OnComponentBeginOverlap(HeadWeapon)
  (params (OverlappedComponent :type Primitive%20Component%20Object%20Reference) (OtherActor :type Actor%20Object%20Reference) (OtherComp :type Primitive%20Component%20Object%20Reference) (OtherBodyIndex :type Integer) (bFromSweep :type Boolean) (SweepResult :type Hit%20Result%20Structure%20%28by%20ref%29))
  ;[1 1 1] On Hitting Something
  (if (Variables|Default|GetCan%20Deal%20Damage?)
    (Variables|Default|SetOther%20Actor OtherActor)
    (Utilities|FlowControl|DoOnce false :!label _label
      (:Completed
        (bind _asbp_top_down_character (Utilities|Casting|CastToBP_TopDownCharacter (Variables|Default|GetOther%20Actor)))
        (bind _returnvalue (Default|CheckActorLoc _asbp_top_down_character self))
        (if (and _returnvalue (Variables|/Game/IvanaKupala/Oka/BP_TopDownCharacter.BP_TopDownCharacter_C|GetBlocking _asbp_top_down_character))
          (Default|BlockedDamage _asbp_top_down_character)
          (CallFunction|BlockedDamage)
          (else
            (Development|PrintString "Player attacked!")
            (Game|Damage|ApplyDamage (Variables|Default|GetOther%20Actor) (Variables|Default|GetDamage) 0 self)))
        (Utilities|FlowControl|Delay 1.0)
        (goto _label Reset)))))

(event OnComponentBeginOverlap(WingWeaponL)
  (params (OverlappedComponent :type Primitive%20Component%20Object%20Reference) (OtherActor :type Actor%20Object%20Reference) (OtherComp :type Primitive%20Component%20Object%20Reference) (OtherBodyIndex :type Integer) (bFromSweep :type Boolean) (SweepResult :type Hit%20Result%20Structure%20%28by%20ref%29))
  ;[1 1 1] On Hitting Something
  (if (Variables|Default|GetCan%20Deal%20Damage?)
    (Variables|Default|SetOther%20Actor OtherActor)
    (Utilities|FlowControl|DoOnce false :!label _label
      (:Completed
        (bind _asbp_top_down_character (Utilities|Casting|CastToBP_TopDownCharacter (Variables|Default|GetOther%20Actor)))
        (bind _returnvalue (Default|CheckActorLoc _asbp_top_down_character self))
        (if (and _returnvalue (Variables|/Game/IvanaKupala/Oka/BP_TopDownCharacter.BP_TopDownCharacter_C|GetBlocking _asbp_top_down_character))
          (Default|BlockedDamage _asbp_top_down_character)
          (CallFunction|BlockedDamage)
          (else
            (Development|PrintString "Player attacked!")
            (Game|Damage|ApplyDamage (Variables|Default|GetOther%20Actor) (Variables|Default|GetDamage) 0 self)))
        (Utilities|FlowControl|Delay 1.0)
        (goto _label Reset)))))

(event Custom|Spawn%20Wave
  (params (index :type Integer))
  ;[1 1 1] Spawn Wave
  (for _array_element (Utilities|Select :Index index :Option%200 (Variables|Default|GetStage1) :Option%201 (Variables|Default|GetStage2) :Option%202 (Variables|Default|GetStage3))
    (Default|ActivateSpawner _array_element true true)))

(event Custom|Attack%20Player
  (bind _stages (Variables|Default|GetStages))
  ;[1 1 1] Attack!
  (Variables|Default|SetAttacking true)
  (Utilities|FlowControl|Sequence
    (:then_0
      ;[1 1 1] On Hitting Something
      (Utilities|FlowControl|DoOnce false) ; enters at Reset
    )
    (:then_1
      (bind _output_get (Variables|Default|SetAttackOption (Math|Random|RandomIntegerinRange 0 1)))
      (bind _ratio (Default|GetHealthRatio (Variables|Default|GetHealthComponent)))
      (bind (_array_element _array_index) (Utilities|Array|ForEachLoopwithBreak _stages :!label _label)
        (:LoopBody
          (if (<= _ratio _array_element)
            (Development|PrintString "Spawning Wave!")
            (CallFunction|SpawnWave _array_index)
            (Utilities|Array|SetArrayElem _stages _array_index -5e+01)
            (Variables|Default|SetAttackOption 2)
            (goto _label Break)))
        (:Completed
          (Animation|Montage|PlayMontage (Variables|Character|GetMesh) (Utilities|Select :Index _output_get :Option%200 "/Game/IvanaKupala/Monsters/MOTHER/Animations/MOTHER_Beak_Attack_Montage.MOTHER_Beak_Attack_Montage" :Option%201 "/Game/IvanaKupala/Monsters/MOTHER/Animations/MOTHER_Wing_Attack_Montage.MOTHER_Wing_Attack_Montage" :Option%202 "/Game/IvanaKupala/Monsters/MOTHER/Animations/MOTHER_Summon_Minions_Montage.MOTHER_Summon_Minions_Montage") (+ 1.0 (- 0.5 (* _ratio 0.5))) ; Attack animation here
            (:OnCompleted
              (Utilities|FlowControl|Delay 1.0))
            (:OnInterrupted
              _))
          (Variables|Default|SetAttacking false)
          (Default|AddEvent (Variables|Default|GetStateTreeQueue) "(TagName=\"AttackOver\")"))))))

(event Custom|Initialize%20Battle
  (bind _healthcomponent (Variables|Default|GetHealthComponent))
  ;[1 1 1] The Beginning
  (bind _returnvalue (UserInterface|CreateWidget "/Game/IvanaKupala/Interface/WidgetBossHealth.WidgetBossHealth_C"))
  (bind _output_get (Variables|Default|SetBossWidget _returnvalue))
  (Default|InitWidget _output_get (Variables|Default|GetHealthComponent) "Великая Птица Алконост, Мать Глеба")
  (EventDispatchers|BindEventtoDamaged _healthcomponent (delegate EventOnDamaged))
  (EventDispatchers|BindEventtoDead _healthcomponent (delegate EventOnDead))
  (CallFunction|SendMonsterStateEvent "(TagName=\"Boss.Start\")"))

(event EventBeginPlay
  ;[1 1 1] The Beginning
  (Components|DestroyComponent (Variables|Default|GetWidgetHealth))
  (CallFunction|SendMonsterStateEvent "(TagName=\"Boss.Init\")"))

(event EventOnDead
  ;[1 1 1] Taking Damage
  (CallFunction|SendMonsterStateEvent "(TagName=\"Dead\")")
  (Utilities|FlowControl|DoOnce false
    (:Completed
      (Animation|Montage|PlayMontage (Variables|Character|GetMesh) (Variables|Default|GetDeath%20Anim) 1.0 0.0 "" ; Death Animation here
        (:then
          (Default|CallOnDeath)
          (Components|Movement|StopMovementImmediately (Variables|Character|GetCharacterMovement))
          (Widget|RemovefromParent (Variables|Default|GetBossWidget))
          (Utilities|KillAllMinions))))))

(event EventOnDamaged
  (params (NewHealth :type Float%20%28double-precision%29) (Amount :type Float%20%28double-precision%29))
  ;[1 1 1] Taking Damage
  (CallFunction|SendMonsterStateEvent "(TagName=\"Injured\")")
  (Animation|Montage|PlayMontage (Variables|Character|GetMesh) (Variables|Default|GetInjured%20Anim) ; Injured Animation here
    (:then
      (Default|AddEvent (Variables|Default|GetStateTreeQueue) "(TagName=\"Recover\")"))))

(event EventFollowPlayer
  (bind _returnvalue (Transformation|GetActorRotation))
  (bind (_roll _pitch) (Math|Rotator|BreakRotator _returnvalue))
  ;[1 1 1] Event Tick
  (Transformation|SetWorldRotation (Variables|Character|GetMesh) (Math|Rotator|MakeRotator _roll _pitch (- (.Yaw (Math|Rotator|BreakRotator (Math|Rotator|FindLookatRotation (Transformation|GetActorLocation) (Transformation|GetActorLocation (Game|GetPlayerCharacter 0))))) 9e+01)) false false)
  (if (not (Variables|Default|GetAttacking))
    (bind _ratio (Default|GetHealthRatio (Variables|Default|GetHealthComponent)))
    (Utilities|FlowControl|Delay (+ _ratio 2.0))
    (Default|AddEvent (Variables|Default|GetStateTreeQueue) "(TagName=\"AttackReady\")")))

(event EventBlockedDamage
  ;[1 1 1] Player Blocked Attack
  (Utilities|FlowControl|DoOnce false :!label _label
    (:Completed
      (Variables|Default|SetCan%20See%20Player? false)
      (Components|Movement|StopMovementImmediately (Variables|Character|GetCharacterMovement))
      (Animation|StopAnimMontage 0)
      (Animation|Montage|PlayMontage 0 (Variables|Default|GetInjured%20Anim)
        (:OnCompleted
          (Utilities|FlowControl|Delay 2.0)
          (Variables|Default|SetCan%20See%20Player? true)
          (goto _label Reset))))))

(fn ConstructionScript
  (bind _statetreequeue (Variables|Default|GetStateTreeQueue))
  (Components|DestroyComponent (Variables|Default|GetWidgetHealth))
  (Default|ConnectStateTree _statetreequeue (Variables|Default|GetMonsterStateTree))
  (Default|AddEvent _statetreequeue "(TagName=\"Boss.Init\")"))