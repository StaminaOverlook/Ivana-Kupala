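; Short-lived hitbox for the Bear Mother enemy's bash skill, damaging and pushing the Oka player character.
; A timeline scales the sphere from BeginPlay and destroys the actor when finished.
; Overlapping Oka applies BashDamage with a pushed damage type, then calls PushOka on the first Bear Mother found in the level.
; A separate DamageTarget function with interface and already-touched checks is not called in this graph.
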(event OnComponentBeginOverlap(Sphere)
  (params (OverlappedComponent :type Primitive%20Component%20Object%20Reference) (OtherActor :type Actor%20Object%20Reference) (OtherComp :type Primitive%20Component%20Object%20Reference) (OtherBodyIndex :type Integer) (bFromSweep :type Boolean) (SweepResult :type Hit%20Result%20Structure%20%28by%20ref%29))
  ;[1 1 1] Applying Damage
  (bind _asbp_oka_character (Utilities|Casting|CastToBP_OkaCharacter OtherActor))
  (bind _output_get (Variables|Default|SetOtherActor _asbp_oka_character))
  (Game|Damage|ApplyDamage _output_get (Variables|Default|GetBashDamage) 0 self "/Game/IvanaKupala/Monsters/Pushed_DamageType.Pushed_DamageType_C")
  (bind _outactors (Actor|GetAllActorsOfClass "/Game/IvanaKupala/Monsters/1_Dubrava/BEAR_MOTHER/BP_Bear_Mother.BP_Bear_Mother_C"))
  (Default|PushOka (Utilities|Array|Get(acopy) _outactors)))

(event EventBeginPlay
  (bind _newtrack_0 (Timeline|Timeline PlayFromStart)
    (:Update
      (Transformation|SetRelativeScale3D (Variables|Default|GetSphere) (Math|Vector|MakeVector _newtrack_0 _newtrack_0 _newtrack_0)))
    (:Finished
      (Actor|DestroyActor))))

(fn ConstructionScript)

(fn DamageTarget
  (params (Actor :type Actor%20Object%20Reference))
  (if (and (Utilities|DoesObjectImplementInterface Actor "/Game/IvanaKupala/Interface/DamageInterface.DamageInterface_C") (not (Utilities|Set|Contains (Variables|Default|GetTouchedActors) Actor)))
    (Game|Damage|ApplyDamage Actor (Variables|Default|GetBashDamage) 0 self)
    (Utilities|Set|Add (Variables|Default|GetTouchedActors) 0)))