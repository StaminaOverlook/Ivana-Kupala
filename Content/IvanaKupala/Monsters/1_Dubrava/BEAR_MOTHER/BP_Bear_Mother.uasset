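; Bear Mother boss character with an intro, boss health bar, melee and charge attacks, and death sequence.
; Events for following, attacking, roaring and dying report back to MonsterStateTree through StateTreeQueue.
; Hitbox overlaps deal blockable melee damage, while the charge turns toward the player, rushes past their position and knocks them back, then recharges on a Timeline.
; At low health a one-time roar grants temporary invulnerability and sets a new damage value.
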(event OnComponentBeginOverlap(Box1)
  (params (OverlappedComponent :type Primitive%20Component%20Object%20Reference) (OtherActor :type Actor%20Object%20Reference) (OtherComp :type Primitive%20Component%20Object%20Reference) (OtherBodyIndex :type Integer) (bFromSweep :type Boolean) (SweepResult :type Hit%20Result%20Structure%20%28by%20ref%29))
  ;[1 1 1] On Hitting Something
  (Variables|Default|SetOther%20Actor OtherActor)
  (if (Variables|Default|GetCan%20Deal%20Damage?)
    (bind _asbp_oka_character (Utilities|Casting|CastToBP_OkaCharacter (Variables|Default|GetOther%20Actor)))
    (Utilities|FlowControl|DoOnce false :!label _label
      (:Completed
        (bind _returnvalue (Default|CheckActorLoc _asbp_oka_character self))
        (if (and _returnvalue (Variables|/Game/IvanaKupala/Oka/BP_OkaCharacter.BP_OkaCharacter_C|GetBlocking _asbp_oka_character))
          (Default|BlockedDamage _asbp_oka_character)
          (CallFunction|BlockedDamage)
          (else
            (Development|PrintString "Player attacked!")
            (Game|Damage|ApplyDamage (Variables|Default|GetOther%20Actor) (Variables|Default|GetDamage) 0 self)))
        (Utilities|FlowControl|Delay 1.0)
        (goto _label Reset)))))

(event OnComponentBeginOverlap(Box)
  (params (OverlappedComponent :type Primitive%20Component%20Object%20Reference) (OtherActor :type Actor%20Object%20Reference) (OtherComp :type Primitive%20Component%20Object%20Reference) (OtherBodyIndex :type Integer) (bFromSweep :type Boolean) (SweepResult :type Hit%20Result%20Structure%20%28by%20ref%29))
  ;[1 1 1] On Hitting Something
  (Variables|Default|SetOther%20Actor OtherActor)
  (if (Variables|Default|GetCan%20Deal%20Damage?)
    (bind _asbp_oka_character (Utilities|Casting|CastToBP_OkaCharacter (Variables|Default|GetOther%20Actor)))
    (Utilities|FlowControl|DoOnce false :!label _label
      (:Completed
        (bind _returnvalue (Default|CheckActorLoc _asbp_oka_character self))
        (if (and _returnvalue (Variables|/Game/IvanaKupala/Oka/BP_OkaCharacter.BP_OkaCharacter_C|GetBlocking _asbp_oka_character))
          (Default|BlockedDamage _asbp_oka_character)
          (CallFunction|BlockedDamage)
          (else
            (Development|PrintString "Player attacked!")
            (Game|Damage|ApplyDamage (Variables|Default|GetOther%20Actor) (Variables|Default|GetDamage) 0 self)))
        (Utilities|FlowControl|Delay 1.0)
        (goto _label Reset)))))

(event OnComponentBeginOverlap(ChargeCollision)
  (params (OverlappedComponent :type Primitive%20Component%20Object%20Reference) (OtherActor :type Actor%20Object%20Reference) (OtherComp :type Primitive%20Component%20Object%20Reference) (OtherBodyIndex :type Integer) (bFromSweep :type Boolean) (SweepResult :type Hit%20Result%20Structure%20%28by%20ref%29))
  ;[1 1 1] Charge
  (if (Variables|Default|GetCharge)
    (bind _output_get (Variables|Default|SetOther%20Actor OtherActor))
    (bind _asbp_oka_character (Utilities|Casting|CastToBP_OkaCharacter _output_get)
      (:then
        (Utilities|FlowControl|DoOnce false
          (:Completed
            (Variables|Default|SetOka%20locaton (Transformation|GetActorLocation _asbp_oka_character))
            (Game|Damage|ApplyDamage (Variables|Default|GetOther%20Actor) (+ (Variables|Default|GetDamage) 1e+01) 0 self "/Game/IvanaKupala/Monsters/Pushed_DamageType.Pushed_DamageType_C")
            (Character|LaunchCharacter _asbp_oka_character (+ (* (Math|Vector|GetForwardVector (Transformation|GetActorRotation)) 1e+03) "0.000000,0.000000,200.000000") false false))))
      (:CastFailed
        (Development|PrintString "CAST TO OKA FAILED.")))))

(event Custom|Spawn%20amination
  (bind _mesh (Variables|Character|GetMesh))
  ;[1 1 1] BEGIN BATTLE
  (Variables|/Script/Engine.SkeletalMeshComponent|SetbPauseAnims (Variables|Character|GetMesh) false)
  (Animation|Montage|PlayMontage _mesh "/Game/IvanaKupala/Monsters/1_Dubrava/BEAR_MOTHER/Animations/Bear_Mother_Appearance_Montage.Bear_Mother_Appearance_Montage" ; Appearance animation here
    (:OnCompleted
      _)
    (:OnInterrupted
      _))
  (Animation|Montage|PlayMontage _mesh "/Game/IvanaKupala/Monsters/1_Dubrava/BEAR_MOTHER/Animations/Bear_Mother_Roar_Montage.Bear_Mother_Roar_Montage"
    (:OnCompleted
      _)
    (:OnInterrupted
      _))
  (CallFunction|SendMonsterStateEvent "(TagName=\"Boss.Start\")")
  (Class|PawnSensingComponent|SetSensingUpdatesEnabled (Variables|Default|GetPawnSensing) true)
  (CallFunction|InitHealthWidget))

(event Custom|Reload%20charge
  ;[1 1 1] Reload Charge
  (Timeline|Timeline PlayFromStart
    (:Finished
      (Variables|Default|SetCharge%20ready true)
      ;[1 1 1] Charge
      (Utilities|FlowControl|DoOnce false) ; enters at Reset
    )))

(event Custom|Event%20Roar
  ;[1 1 1] Roar
  (Class|PawnSensingComponent|SetSensingUpdatesEnabled (Variables|Default|GetPawnSensing) false)
  (Variables|Default|SetRoarSkill false)
  (Variables|Default|SetDamage 3e+01)
  (Utilities|FlowControl|Delay 0.1)
  (Utilities|FlowControl|Delay (Animation|GetPlayLength (Variables|Default|GetInjured%20Anim)))
  (Variables|Default|SetInjured%20Anim "/Game/IvanaKupala/Monsters/1_Dubrava/BEAR_MOTHER/Animations/Bear_Mother_Injured_Montage.Bear_Mother_Injured_Montage")
  (Pawn|Components|CharacterMovement|SetMovementMode (Variables|Character|GetCharacterMovement) "MOVE_None" 0)
  (Animation|Montage|PlayMontage (Variables|Character|GetMesh) "/Game/IvanaKupala/Monsters/1_Dubrava/BEAR_MOTHER/Animations/Bear_Mother_Roar_Montage.Bear_Mother_Roar_Montage"
    (:OnCompleted
      (Class|PawnSensingComponent|SetSensingUpdatesEnabled (Variables|Default|GetPawnSensing) true)
      (Pawn|Components|CharacterMovement|SetMovementMode (Variables|Character|GetCharacterMovement) "MOVE_Walking" 0)
      (Variables|Default|SetbCanBeDamaged true)
      (Default|AddEvent (Variables|Default|GetStateTreeQueue) "(TagName=\"AttackOver\")"))))

(event Custom|Event%20Charge
  ;[1 1 1] Charge
  (Development|PrintString "Charge begin!" true true "(R=1.000000,G=0.067083,B=0.166763,A=1.000000)")
  (Variables|Default|SetCharge%20ready false)
  (Utilities|Time|SetTimerbyFunctionName 0 "LookForPlayer" 0.0001 true true)
  (Animation|Montage|PlayMontage (Variables|Character|GetMesh) "/Game/IvanaKupala/Monsters/1_Dubrava/BEAR_MOTHER/Animations/Bear_Mother_Attack_Prepare_Montage.Bear_Mother_Attack_Prepare_Montage" ; Attack animation here
    (:OnCompleted
      (Class|KismetSystemLibrary|PauseTimer 0 "LookForPlayer")
      (Variables|Default|SetCharge true)
      (Variables|/Script/Engine.CharacterMovementComponent|SetMaxWalkSpeed (Variables|Character|GetCharacterMovement) (Variables|Default|GetCharge%20Speed))
      (bind _output_get (Variables|Default|SetCharge%20Location (+ (Transformation|GetActorLocation (Game|GetPlayerCharacter 0)) (* (Math|Vector|GetForwardVector (Transformation|GetActorRotation)) (Variables|Default|GetWalk%20Speed)))))
      (bind _movementresult (AI|AIMoveTo self _output_get 0 1e+01 false)
        (:OnSuccess
          _)
        (:OnFail
          (Development|PrintString (Utilities|String|EnumtoString _movementresult) true true "(R=1.000000,G=0.250773,B=0.000000,A=1.000000)")))
      (Variables|/Script/Engine.CharacterMovementComponent|SetMaxWalkSpeed (Variables|Character|GetCharacterMovement) (Variables|Default|GetWalk%20Speed))
      (Variables|Default|SetCharge false)
      (Utilities|FlowControl|Delay 2.0)
      (CallFunction|ReloadCharge)
      (Default|AddEvent (Variables|Default|GetStateTreeQueue) "(TagName=\"AttackOver\")"))
    (:OnInterrupted
      (Development|PrintString "Charge interrupted.")
      (Default|AddEvent (Variables|Default|GetStateTreeQueue) "(TagName=\"AttackOver\")")
      (CallFunction|ReloadCharge))))

(event Custom|On%20Damaged
  (params (NewHealth :type Float%20%28double-precision%29) (Amount :type Float%20%28double-precision%29))
  ;[1 1 1] BEGIN PLAY
  (if (and (<= (Variables|/Game/IvanaKupala/Interface/HealthComponent.HealthComponent_C|GetHealth (Variables|Default|GetHealthComponent)) 5e+01) (Variables|Default|GetRoarSkill))
    (Variables|Default|SetInjured%20Anim "/Game/IvanaKupala/Monsters/1_Dubrava/BEAR_MOTHER/Animations/Bear_Mother_Death_Before_Rotation_Montage.Bear_Mother_Death_Before_Rotation_Montage")
    (Variables|Default|SetbCanBeDamaged false)
    (CallFunction|OnDamaged 0.0 0.0)
    (CallFunction|EventRoar)
    (else
      (CallFunction|OnDamaged 0.0 0.0))))

(event EventBeginPlay
  (bind _healthcomponent (Variables|Default|GetHealthComponent))
  ;[1 1 1] BEGIN PLAY
  (Components|DestroyComponent (Variables|Default|GetWidgetHealth))
  (EventDispatchers|BindEventtoDamaged _healthcomponent (delegate Custom|On%20Damaged))
  (EventDispatchers|BindEventtoDead _healthcomponent (delegate EventOnDead)))

(event EventOnDead
  ;[1 1 1] On Dead
  (for _array_element (Utilities|Array|MakeArray (Variables|Default|GetBox) (Variables|Default|GetBox1) (Variables|Default|GetChargeCollision))
    (Collision|SetCollisionEnabled _array_element "NoCollision"))
  (Class|PawnSensingComponent|SetSensingUpdatesEnabled (Variables|Default|GetPawnSensing) false)
  (bind _asbp_top_down_game_mode (Utilities|Casting|CastToBP_TopDownGameMode (Game|GetGameMode)))
  (Default|FadeBGM _asbp_top_down_game_mode)
  (Default|AddEvent (Variables|Default|GetStateTreeQueue) "(TagName=\"Dead\")"))

(event EventFollowPlayer
  ;[1 1 1] Follow Player
  (if (<= (Variables|Default|GetCharge%20Radius) (Math|Vector|Distance(Vector) (Transformation|GetActorLocation) (Transformation|GetActorLocation (Game|GetPlayerCharacter 0))))
    (AI|AIMoveTo self "0, 0, 0" (Game|GetPlayerCharacter 0) (Variables|Default|GetAcceptance%20Radius) true :!label _label
      (:OnSuccess
        (if (Variables|Default|GetFollowing%20Player?)
          (Default|AddEvent (Variables|Default|GetStateTreeQueue) "(TagName=\"AttackReady\")"))))
    (elif (Variables|Default|GetCharge%20ready)
      (if (Variables|Default|GetFollowing%20Player?)
        (Default|AddEvent (Variables|Default|GetStateTreeQueue) "(TagName=\"AttackReady\")"))
      (else
        (goto _label)))))

(event EventAttackPlayer
  ;[1 1 1] Attack!
  (Utilities|FlowControl|Sequence
    (:then_0
      ;[1 1 1] On Hitting Something
      (Utilities|FlowControl|DoOnce false) ; enters at Reset
    )
    (:then_1
      (if (Variables|Default|GetCharge%20ready)
        (CallFunction|EventCharge)
        (else
          (Utilities|FlowControl|DoOnce false :!label _label
            (:Completed
              (Animation|Montage|PlayMontage (Variables|Character|GetMesh) (Variables|Default|GetAttack%20Anim) ; Attack animation here
                (:OnCompleted
                  (Utilities|FlowControl|Delay 1.0))
                (:OnInterrupted
                  _))
              (Default|AddEvent (Variables|Default|GetStateTreeQueue) "(TagName=\"AttackOver\")")
              (goto _label Reset))))))))

(event EventDamageChageColor
  (Rendering|Material|SetMaterial (Variables|Character|GetMesh) 0 "/Game/IvanaKupala/Monsters/M_White.M_White")
  (Utilities|FlowControl|Delay 0.3)
  (Rendering|Material|SetMaterial (Variables|Character|GetMesh) 0 "/Game/IvanaKupala/Monsters/1_Dubrava/BEAR_MOTHER/Textures/Bear_Material.Bear_Material"))

(event EventCancelAttack
  ;[1 1 1] On Hitting Something
  (Animation|StopAnimMontage (Variables|Default|GetAttack%20Anim))
  (Utilities|FlowControl|DoOnce false) ; enters at Reset
)

(event EventStartDeadState
  (bind _death_anim (Variables|Default|GetDeath%20Anim))
  (bind _capsulecomponent (Variables|Default|GetCapsuleComponent))
  (Collision|SetCollisionEnabled _capsulecomponent "NoCollision")
  (Variables|/Script/Engine.PrimitiveComponent|SetbGenerateOverlapEvents _capsulecomponent false)
  (bind _returnvalue (CallFunction|IsMontagePlaying _death_anim))
  (if (not _returnvalue)
    (Animation|Montage|PlayMontage (Variables|Character|GetMesh) "/Game/IvanaKupala/Monsters/1_Dubrava/BEAR_MOTHER/Animations/Bear_Mother_Death_Before_Rotation_Montage.Bear_Mother_Death_Before_Rotation_Montage"
      (:OnCompleted
        _)
      (:OnInterrupted
        _))
    (Animation|Montage|PlayMontage (Variables|Character|GetMesh) _death_anim 1.0 0.0 "Dying" ; Death Animation here
      (:then
        _)
      (:OnInterrupted
        _))
    (Default|CallOnDeath)))

(event EventInitHealthWidget
  ;[1 1 1] BEGIN PLAY
  ;[1 1 1] Init Health Widget
  (bind _returnvalue (UserInterface|CreateWidget "/Game/IvanaKupala/Interface/WB_BossHealth.WB_BossHealth_C"))
  (UserInterface|SetWidget (Variables|Default|GetWidgetHealth) _returnvalue)
  (Default|InitWidget _returnvalue (Variables|Default|GetHealthComponent) "ВЕДМЕДЪ О ТЫСЯЧЕ ОЧЕЙ"))

(fn ConstructionScript
  (bind _statetreequeue (Variables|Default|GetStateTreeQueue))
  (Default|ConnectStateTree _statetreequeue (Variables|Default|GetMonsterStateTree))
  (Default|AddEvent _statetreequeue "(TagName=\"Boss.Init\")")
  (Class|PawnSensingComponent|SetSensingUpdatesEnabled (Variables|Default|GetPawnSensing) false)
  (Variables|/Script/Engine.SkeletalMeshComponent|SetbPauseAnims (Variables|Character|GetMesh) true))

(fn LookforPlayer
  (bind _returnvalue (Transformation|GetActorRotation))
  (Transformation|SetActorRotation (Math|Rotator|MakeRotator (.roll _returnvalue) (.pitch _returnvalue) (.yaw (Class|KismetMathLibrary|RInterptoConstant (Transformation|GetActorRotation) (Math|Rotator|FindLookatRotation (Transformation|GetActorLocation) (Transformation|GetActorLocation (Game|GetPlayerCharacter 0))) (Utilities|Time|GetWorldDeltaSeconds) 3.5e+02)))))