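; Wolf enemy that guards its spawn point, chasing and biting the player, with normal and long attacks.
; PawnSensing and movement push events to a StateTree queue; attack montages pair with a toggleable hit box that respects player blocking.
; A periodic howl at spawn sphere-traces for nearby wolves, temporarily buffing damage, material, Niagara effect and capsule scale.
; Random delays recharge howl and long attack; idle wolves return home to eat.
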(event OnComponentBeginOverlap(Box)
  (params (OverlappedComponent :type Primitive%20Component%20Object%20Reference) (OtherActor :type Actor%20Object%20Reference) (OtherComp :type Primitive%20Component%20Object%20Reference) (OtherBodyIndex :type Integer) (bFromSweep :type Boolean) (SweepResult :type Hit%20Result%20Structure%20%28by%20ref%29))
  ;[1 1 1] On Hitting Something
  (if (Variables|Default|GetCan%20Deal%20Damage?)
    (bind _output_get (Variables|Default|SetOther%20Actor OtherActor))
    (bind _asbp_oka_character (Utilities|Casting|CastToBP_OkaCharacter _output_get))
    (Utilities|FlowControl|DoOnce false :!label _label
      (:Completed
        (bind _returnvalue (Default|CheckActorLoc _asbp_oka_character self))
        (if (and _returnvalue (Variables|/Game/IvanaKupala/Oka/BP_OkaCharacter.BP_OkaCharacter_C|GetBlocking _asbp_oka_character))
          (Default|BlockedDamage _asbp_oka_character)
          (CallFunction|BlockedDamage)
          (else
            (Development|PrintString "Player attacked!")
            (Game|Damage|ApplyDamage (Variables|Default|GetOther%20Actor) (Variables|Default|GetDamage) 0 self)))
        (Utilities|FlowControl|Delay 1.0)
        (goto _label Reset)))))

(event OnSeePawn(PawnSensing)
  (params (Pawn :type Pawn%20Object%20Reference))
  (if (Variables|Default|GetCan%20See%20Player?)
    (Utilities|FlowControl|DoOnce false) ; enters at Reset
    (else
      (Utilities|FlowControl|DoOnce false :!label _label
        (:Completed
          (Default|AddEvent (Variables|Default|GetStateTreeQueue) "(TagName=\"Noticed\")")
          (goto _label Reset))))))

(event OnHearNoise(PawnSensing)
  (params (Instigator :type Pawn%20Object%20Reference) (Location :type Vector%20%28by%20ref%29 :default "0, 0, 0") (Volume :type Float%20%28single-precision%29))
  (Utilities|FlowControl|DoOnce false
    (:Completed
      (CallFunction|HearNoise))))

(event Custom|LargeAttackReload
  (Utilities|FlowControl|Delay (Math|Random|RandomFloatinRange 4.0 1e+01))
  (Variables|Default|SetLarge%20attack true))

(event Custom|Howl_reload
  (Utilities|FlowControl|Delay (Math|Random|RandomFloatinRange 14.0 2e+01))
  (Variables|Default|SetHowl true))

(event Custom|Howl_Buff
  (Variables|Default|SetHowl_buff_disactivated false)
  (CallFunction|ChangeScale)
  (Components|Activation|Activate (Variables|Default|GetNiagara) false)
  (Variables|Default|SetDamage (* (Variables|Default|GetDamage) 1.2))
  (Utilities|FlowControl|Delay (Math|Random|RandomFloatinRange 8.0 16.0))
  (if (not (<= (Variables|/Game/IvanaKupala/Interface/HealthComponent.HealthComponent_C|GetHealth (Variables|Default|GetHealthComponent)) 0.0))
    (CallFunction|ChangeScale)
    (Components|Activation|Deactivate (Variables|Default|GetNiagara))
    (Variables|Default|SetDamage (/ (Variables|Default|GetDamage) 1.2))
    (Variables|Default|SetHowl_buff_disactivated true)))

(event Custom|Change%20scale
  (bind _mesh (Variables|Character|GetMesh))
  (Utilities|FlowControl|FlipFlop
    (:A
      (Rendering|Material|SetMaterial _mesh 0 "/Game/IvanaKupala/Monsters/1_Dubrava/Wolf/Textures/Material_002.Material_002")
      (bind _newtrack_0 (Timeline|Timeline_0 PlayFromStart)
        (:Update
          (Transformation|SetRelativeScale3D (Variables|Default|GetCapsuleComponent) (Math|Vector|MakeVector _newtrack_0 _newtrack_0 _newtrack_0)))))
    (:B
      (Rendering|Material|SetMaterial _mesh 0 "/Game/IvanaKupala/Monsters/1_Dubrava/Wolf/Textures/Material_001.Material_001")
      (Timeline|Timeline_0 ReverseFromEnd))))

(event Custom|Howl_skill
  (bind _returnvalue (Transformation|GetActorLocation))
  (if (Variables|Default|GetHowl_buff_disactivated)
    (Animation|Montage|PlayMontage (Variables|Character|GetMesh) "/Game/IvanaKupala/Monsters/1_Dubrava/Wolf/Animations/Wolf_Howl_Montage.Wolf_Howl_Montage"
      (:then
        (Utilities|FlowControl|Delay 0.8)
        (bind _outhits (Collision|MultiSphereTraceByChannel _returnvalue _returnvalue 8e+02 "TraceTypeQuery2" false 0 "ForDuration" true "(R=1.000000,G=0.000000,B=0.000000,A=1.000000)" "(R=0.000000,G=1.000000,B=0.000000,A=1.000000)" 2.0))
        (for _array_element _outhits
          (bind _asbp_wolf (Utilities|Casting|CastToBP_Wolf (.HitActor (Collision|BreakHitResult _array_element))))
          (if (Variables|BP_Wolf_C|GetHowl_buff_disactivated _asbp_wolf)
            (CallFunction|HowlBuff _asbp_wolf)))
        (if (Variables|Default|GetHowl_buff_disactivated)
          (CallFunction|HowlBuff))
        (Variables|Default|SetStop_Movenemt false)))))

(event EventCancelAttack
  ;[1 1 1] On Hitting Something
  (Animation|StopAnimMontage (Variables|Default|GetAttack%20Anim))
  (Utilities|FlowControl|DoOnce false) ; enters at Reset
)

(event EventOnDead
  (|CallParentFunction)
  (if (Variables|Default|GetHowl_buff_disactivated)
    _
    (else
      (CallFunction|ChangeScale)
      (Components|Activation|Deactivate (Variables|Default|GetNiagara))))
  (Collision|SetCollisionEnabled (Variables|Default|GetBox) "NoCollision"))

(event EventCanDealDmg
  (Collision|SetCollisionEnabled (Variables|Default|GetBox) "QueryAndPhysics"))

(event EventAttackPlayer
  ;[1 1 1] Attack!
  (Utilities|FlowControl|Sequence
    (:then_0
      ;[1 1 1] On Hitting Something
      (Utilities|FlowControl|DoOnce false) ; enters at Reset
    )
    (:then_1
      (Utilities|FlowControl|DoOnce false :!label _label
        (:Completed
          (if (Variables|Default|GetLarge%20attack)
            (Animation|Montage|PlayMontage (Variables|Character|GetMesh) "/Game/IvanaKupala/Monsters/1_Dubrava/Wolf/Animations/Wolf_AttackLong_Montage.Wolf_AttackLong_Montage" ; Attack animation here
              (:OnCompleted
                _)
              (:OnInterrupted
                (CallFunction|StopDealDmg :!label _label_2)))
            (else
              (Animation|Montage|PlayMontage (Variables|Character|GetMesh) "/Game/IvanaKupala/Monsters/1_Dubrava/Wolf/Animations/Wolf_Attack_Montage.Wolf_Attack_Montage" ; Attack animation here
                (:OnCompleted
                  _)
                (:OnInterrupted
                  (goto _label_2)))))
          (Utilities|FlowControl|Delay 1.0)
          (Default|AddEvent (Variables|Default|GetStateTreeQueue) "(TagName=\"AttackOver\")")
          (goto _label Reset))))))

(event EventStopDealDmg
  (Collision|SetCollisionEnabled (Variables|Default|GetBox) "NoCollision"))

(event EventFollowPlayer
  (Utilities|FlowControl|Sequence
    (:then_0
      (Utilities|FlowControl|DoOnce false
        (:Completed
          (Animation|StopAnimMontage 0))))
    (:then_1
      (if (not (Variables|Default|GetStop_Movenemt))
        (if (and (Variables|Default|GetHowl) (Variables|Default|GetHowl_buff_disactivated))
          (Variables|Default|SetHowl false)
          (Variables|Default|SetStop_Movenemt true)
          (AI|AIMoveTo self (Variables|Default|GetSpawnLocation) 0 1e+02 true
            (:OnSuccess
              (CallFunction|HowlSkill)
              (CallFunction|HowlReload)))
          (elif (< (Math|Vector|Distance(Vector) (Variables|Default|GetSpawnLocation) (Transformation|GetActorLocation (Game|GetPlayerCharacter 0))) 3.5e+03)
            (if (Variables|Default|GetLarge%20attack)
              (AI|AIMoveTo self "0, 0, 0" (Game|GetPlayerCharacter 0) (* (Variables|Default|GetAcceptance%20Radius) 2.0) true
                (:OnSuccess
                  (if (Variables|Default|GetFollowing%20Player?)
                    (Default|AddEvent (Variables|Default|GetStateTreeQueue) "(TagName=\"AttackReady\")"))))
              (else
                (AI|AIMoveTo self "0, 0, 0" (Game|GetPlayerCharacter 0) (Variables|Default|GetAcceptance%20Radius) true
                  (:then
                    (Utilities|FlowControl|DoOnce false
                      (:Completed
                        (Utilities|FlowControl|Delay (Math|Random|RandomFloatinRange 4.0 1e+01))
                        (Variables|Default|SetHowl true)
                        (CallFunction|LargeAttackReload))))
                  (:OnSuccess
                    (if (Variables|Default|GetFollowing%20Player?)
                      (Default|AddEvent (Variables|Default|GetStateTreeQueue) "(TagName=\"AttackReady\")"))))))
            (else
              (Default|AddEvent (Variables|Default|GetStateTreeQueue) "(TagName=\"Missing\")"))))))))

(event EventIdleWalk
  (if (not (Variables|Default|GetCan%20See%20Player?))
    (if (< (Math|Vector|Distance(Vector) (Variables|Default|GetSpawnLocation) (Transformation|GetActorLocation)) 6e+02)
      (Utilities|FlowControl|DoOnce false :!label _label
        (:Completed
          (Animation|Montage|PlayMontage (Variables|Character|GetMesh) "/Game/IvanaKupala/Monsters/1_Dubrava/Wolf/Animations/Wolf_Eating_Montage.Wolf_Eating_Montage"
            (:OnCompleted
              _)
            (:OnInterrupted
              _))
          (Utilities|FlowControl|Delay 0.2)
          (goto _label Reset)))
      (else
        (Utilities|FlowControl|DoOnce false :!label _label_2
          (:Completed
            (AI|AIMoveTo self (Variables|Default|GetSpawnLocation) 0 (Variables|Default|GetAcceptance%20Radius) true
              (:OnSuccess
                (goto _label_2 Reset)))))))))

(fn ConstructionScript
  (|CallParentFunction))