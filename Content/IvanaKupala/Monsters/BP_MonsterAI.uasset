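; Base monster character AI that wanders, notices and chases the player, takes damage and dies, leaving attack and color-change events empty.
; Pawn sensing, movement and health events feed a StateTree through an event queue; state events handle injury recovery and death.
; Pushed damage triggers a timeline knockback, while blocked attacks briefly stun the monster.
; Save data restores transform, health and flags, collapsing Attack and Injured states into Move.
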(event OnSeePawn(PawnSensing)
  (params (Pawn :type Pawn%20Object%20Reference))
  ;[1 1 1] On See Pawn
  (if (Variables|Default|GetCan%20See%20Player?)
    ;[1 1 1] On Hear Noise
    (Utilities|FlowControl|DoOnce false) ; enters at Reset
    (else
      (bind _returnvalue (CallFunction|IsMontagePlaying (Variables|Default|GetInjured%20Anim)))
      (if (not _returnvalue)
        (Default|AddEvent (Variables|Default|GetStateTreeQueue) "(TagName=\"Noticed\")")))))

(event OnHearNoise(PawnSensing)
  (params (Instigator :type Pawn%20Object%20Reference) (Location :type Vector%20%28by%20ref%29 :default "0, 0, 0") (Volume :type Float%20%28single-precision%29))
  ;[1 1 1] On Hear Noise
  (Utilities|FlowControl|DoOnce false
    (:Completed
      (CallFunction|HearNoise))))

(event Custom|Follow%20Player
  ;[1 1 1] Follow Player
  (AI|AIMoveTo self "0, 0, 0" (Game|GetPlayerCharacter 0) (Variables|Default|GetAcceptance%20Radius) true
    (:OnSuccess
      (if (Variables|Default|GetFollowing%20Player?)
        (Default|AddEvent (Variables|Default|GetStateTreeQueue) "(TagName=\"AttackReady\")")))))

(event Custom|Attack%20Player
  ;[1 1 1] Attack Player
)

(event Custom|IdleWalk
  ;[1 1 1] Idle Walking
  (if (not (Variables|Default|GetCan%20See%20Player?))
    (Utilities|FlowControl|DoOnce false :!label _label
      (:Completed
        (AI|AIMoveTo self (.RandomLocation (AI|Navigation|GetRandomReachablePointinRadius (Transformation|GetActorLocation) 4e+02 0 0)) 0 5.0 false
          (:OnSuccess
            (Utilities|FlowControl|Delay (Math|Random|RandomFloatinRange 2.0 5.0))
            (goto _label Reset)))))))

(event Custom|OnDamaged
  (params (NewHealth :type Float%20%28double-precision%29) (Amount :type Float%20%28double-precision%29))
  ;[1 1 1] Init
  (Default|AddEvent (Variables|Default|GetStateTreeQueue) "(TagName=\"Injured\")"))

(event Custom|OnDead
  ;[1 1 1] Init
  (Default|AddEvent (Variables|Default|GetStateTreeQueue) "(TagName=\"Dead\")"))

(event Custom|CancelAttack
  ;[1 1 1] Attack Player
)

(event Custom|DamageChangeColor
  ;[1 1 1] Attack Player
)

(event Custom|InitHealthWidget
  ;[1 1 1] Health Widget
  (bind _aswb_monster_health (Utilities|Casting|CastToWB_MonsterHealth (UserInterface|GetWidget (Variables|Default|GetWidgetHealth))))
  (Default|InitWidget _aswb_monster_health (Variables|Default|GetHealthComponent)))

(event Custom|HearNoise
  (Utilities|Time|SetTimerbyFunctionName 0 "RotationToThePlayer" 0.001 true true)
  (Utilities|FlowControl|Delay 1.0)
  (Utilities|Time|ClearTimerbyFunctionName 0 "RotationToThePlayer")
  (Utilities|FlowControl|Delay 1.0))

(event Custom|Push
  (bind _returnvalue (Transformation|GetActorLocation))
  (Utilities|FlowControl|DoOnce false :!label _label
    (:Completed
      (bind _output_get (Variables|Default|SetPushLerp (Utilities|Struct|MakeRigVMFunction_MathVectorLerp _returnvalue (- _returnvalue (* (Transformation|GetActorForwardVector) (Variables|Default|GetPushDistance))) 0.0)))
      (bind _pushease (Timeline|Timeline PlayFromStart)
        (:Update
          (Transformation|SetActorLocation (Math|Vector|Lerp(Vector) (.A (Utilities|Struct|BreakRigVMFunction_MathVectorLerp _output_get)) (.B (Utilities|Struct|BreakRigVMFunction_MathVectorLerp _output_get)) _pushease) false false))
        (:Finished
          (goto _label Reset))))))

(event EventBeginPlay
  (bind _healthcomponent (Variables|Default|GetHealthComponent))
  ;[1 1 1] Init
  (CallFunction|InitHealthWidget)
  (EventDispatchers|BindEventtoDamaged _healthcomponent (delegate Custom|OnDamaged))
  (EventDispatchers|BindEventtoDead _healthcomponent (delegate Custom|OnDead)))

(event EventLoadfromEnemySaveData
  (params (SaveData :type Enemy%20Save%20Data%20Structure))
  (bind (_isfollowing _canseeoka _candamage _isattacking _state _location _health) (Utilities|Struct|BreakEnemySaveData SaveData))
  (Transformation|SetActorTransform _location false true)
  (Variables|/Game/IvanaKupala/Interface/HealthComponent.HealthComponent_C|SetHealth (Variables|Default|GetHealthComponent) _health)
  (Variables|Default|SetFollowing%20Player? _isfollowing)
  (Variables|Default|SetCan%20See%20Player? _canseeoka)
  (Variables|Default|SetCan%20Deal%20Damage? _candamage)
  (Variables|Default|SetAttacking _isattacking)
  (switch Utilities|FlowControl|Switch|SwitchonEnemyStates (CallFunction|LoadSignalState _state)
    (:NewEnumerator1
      (CallFunction|SendMonsterStateEvent "(TagName=\"Boss.Init\")"))
    (:NewEnumerator2
      (CallFunction|SendMonsterStateEvent "(TagName=\"Init\")"))
    (:NewEnumerator3
      (CallFunction|SendMonsterStateEvent "(TagName=\"Noticed\")"))))

(event Game|Damage|EventAnyDamage
  (params (Damage :type Float%20%28single-precision%29) (DamageType :type Damage%20Type%20Object%20Reference) (InstigatedBy :type Controller%20Object%20Reference) (DamageCauser :type Actor%20Object%20Reference))
  ;[1 1 1] Taking Damage
  (if (Variables|Actor|GetbCanBeDamaged)
    (Pawn|Components|CharacterMovement|SetMovementMode (Variables|Character|GetCharacterMovement) "MOVE_Walking" 0)
    (Animation|StopAnimMontage 0)
    (Default|EventDamage (Variables|Default|GetHealthComponent) Damage)
    (Utilities|Casting|CastToPushed_DamageType DamageType)
    (CallFunction|Push)))

(event EventBlockedDamage
  ;[1 1 1] Player Blocked Attack
  (Utilities|FlowControl|DoOnce false :!label _label
    (:Completed
      (Variables|Default|SetCan%20See%20Player? false)
      (Components|Movement|StopMovementImmediately (Variables|Character|GetCharacterMovement))
      (Animation|StopAnimMontage 0)
      (Animation|Montage|PlayMontage 0 (Variables|Default|GetInjured%20Anim)
        (:OnCompleted
          (Utilities|FlowControl|Delay 2.0)
          (Variables|Default|SetCan%20See%20Player? true)
          (goto _label Reset))))))

(event Custom|StartDeadState
  (bind _death_anim (Variables|Default|GetDeath%20Anim))
  (bind _capsulecomponent (Variables|Collision|GetCapsuleComponent))
  (Components|DestroyComponent (Variables|Default|GetPawnSensing))
  (Collision|SetCollisionEnabled _capsulecomponent "NoCollision")
  (Variables|/Script/Engine.PrimitiveComponent|SetbGenerateOverlapEvents _capsulecomponent false)
  (bind _returnvalue (CallFunction|IsMontagePlaying _death_anim))
  (if (not _returnvalue)
    (CallFunction|DamageChangeColor)
    (Animation|Montage|PlayMontage (Variables|Character|GetMesh) _death_anim 1.0 0.0 "Dying" ; Death Animation here
      (:then
        (Default|CallOnDeath)
        (Utilities|FlowControl|Delay 4.0)
        (Actor|DestroyActor)))))

(event Custom|StartInjuredState
  (bind _returnvalue (CallFunction|IsMontagePlaying (Variables|Default|GetInjured%20Anim)))
  (bind _returnvalue_2 (CallFunction|IsMontagePlaying (Variables|Default|GetDeath%20Anim)))
  (if (Math|Boolean|NORBoolean _returnvalue_2 _returnvalue)
    (CallFunction|DamageChangeColor)
    (Default|AddEvent (Variables|Default|GetStateTreeQueue) "(TagName=\"Recover\")")))

(fn ConstructionScript
  (bind _statetreequeue (Variables|Default|GetStateTreeQueue))
  (Default|ConnectStateTree _statetreequeue (Variables|Default|GetMonsterStateTree))
  (Default|AddEvent _statetreequeue "(TagName=\"Init\")"))

(fn IsMontagePlaying
  (params (Montage :type Anim%20Montage%20Object%20Reference))
  (return (Animation|Montage|MontageIsPlaying (Components|SkeletalMesh|GetAnimInstance (Variables|Character|GetMesh)) Montage)))

(fn SendMonsterStateEvent
  (params (Tag :type Gameplay%20Tag%20Structure))
  (Gameplay|StateTree|SendStateTreeEvent (Variables|Default|GetMonsterStateTree) (Utilities|Struct|MakeStateTreeEvent Tag) :!class /Script/GameplayStateTreeModule.StateTreeComponent)
  (return))

(fn RotationtothePlayer
  (bind _returnvalue (Transformation|GetActorRotation))
  (Transformation|SetActorRotation (Math|Rotator|MakeRotator (.roll _returnvalue) (.pitch _returnvalue) (.yaw (Class|KismetMathLibrary|RInterptoConstant (Transformation|GetActorRotation) (Math|Rotator|FindLookatRotation (Transformation|GetActorLocation) (Transformation|GetActorLocation (Game|GetPlayerCharacter 0))) (Utilities|Time|GetWorldDeltaSeconds) 3.5e+02)))))

(fn LoadSignalState
  (params (State :type EnemyStates%20Enum :default "NewEnumerator0"))
  (switch Utilities|FlowControl|Switch|SwitchonEnemyStates State
    (:NewEnumerator1
      (bind _output_get (LocalVariables|SetFinalState "NewEnumerator1"))
      (return _output_get))
    (:NewEnumerator2
      (bind _output_get_2 (LocalVariables|SetFinalState "NewEnumerator2"))
      (return _output_get_2))
    (:NewEnumerator3
      _)
    (:NewEnumerator4
      _)
    (:NewEnumerator5
      _))
  (bind _output_get_3 (LocalVariables|SetFinalState "NewEnumerator3"))
  (return _output_get_3))

(fn GetEnemySaveData
  (bind _self self)
  (return (Utilities|Struct|MakeEnemySaveData (Variables|Default|GetFollowing%20Player?) (Variables|Default|GetCan%20See%20Player?) (Variables|Default|GetCan%20Deal%20Damage?) (Variables|Default|GetAttacking) (Variables|Default|GetStateEnum) (Transformation|GetActorTransform) (Variables|/Game/IvanaKupala/Interface/HealthComponent.HealthComponent_C|GetHealth (Variables|Default|GetHealthComponent)) (Utilities|GetClass _self)) (Utilities|GetObjectName _self)))