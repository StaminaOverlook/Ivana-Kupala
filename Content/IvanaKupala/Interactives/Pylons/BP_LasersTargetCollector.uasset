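; Interactable laser-puzzle pylon that collects beams on two input mirrors and emits a new laser from a third, output mirror.
; Interacting rotates the mirror assembly 45 degrees on a timeline, while dynamic materials color the mirrors chosen by IndexComponent.
; LaserBounce tracks hit components, tints or clears each input, and clears attached lasers when an input is unmatched.
; When both inputs carry CheckColor, it spawns an attached BP_Laser in NewColor, registered with the source's SpawnReference.
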(event EventBeginPlay
  (|CallParentFunction)
  (Variables|Default|SetRotation (Variables|/Script/Engine.SceneComponent|GetRelativeRotation (Variables|Default|GetMirors)))
  (for _array_element (Variables|Default|GetIndexComponent)
    (Utilities|Array|Insert (Variables|Default|GetActiveMirors) (Utilities|Array|Get(acopy) (Utilities|Array|MakeArray (Variables|Default|GetMiror_0) (Variables|Default|GetMiror_1) (Variables|Default|GetMiror_2) (Variables|Default|GetMiror_3) (Variables|Default|GetMiror_4) (Variables|Default|GetMiror_5) (Variables|Default|GetMiror_6) (Variables|Default|GetMiror_7)) _array_element)))
  (for (_array_element_2 _array_index) (Variables|Default|GetActiveMirors)
    (bind _returnvalue (Rendering|Material|CreateDynamicMaterialInstance _array_element_2 0 "/Game/IvanaKupala/Interactives/Pylons/M_Laser_2.M_Laser_2" "None" :!class /Script/Engine.PrimitiveComponent))
    (if (== _array_index 2)
      (Rendering|Material|SetVectorParameterValue _returnvalue "Color" (Variables|Default|GetColor_output) :!class /Script/Engine.MaterialInstanceDynamic)
      (else
        (Rendering|Material|SetVectorParameterValue _returnvalue "Color" (Variables|Default|GetColor_input) :!class /Script/Engine.MaterialInstanceDynamic)
        (Utilities|Array|Add (Variables|Default|GetActiveMiror) _array_element_2))))
  (Variables|Default|SetCheckMirors (Utilities|Array|MakeArray (Variables|Default|GetCube1) (Variables|Default|GetCube))))

(event EventInteracting
  (Variables|Default|SetInteractable false)
  (bind _asbp_top_down_controller (Utilities|Casting|CastToBP_TopDownController (Game|GetPlayerController 0)))
  (Variables|/Game/IvanaKupala/Oka/Input/BP_TopDownController.BP_TopDownController_C|SetDisabled_Input _asbp_top_down_controller false)
  (Variables|Default|Setcheck true)
  (bind _newtrack_0 (Timeline|Timeline PlayFromStart)
    (:Update
      (Transformation|SetRelativeRotation (Variables|Default|GetMirors) (Math|Rotator|Lerp(Rotator) (Variables|Default|GetRotation) (Math|Rotator|MakeRotator (.Roll (Math|Rotator|BreakRotator (Variables|Default|GetRotation))) (.Pitch (Math|Rotator|BreakRotator (Variables|Default|GetRotation))) (+ (.Yaw (Math|Rotator|BreakRotator (Variables|Default|GetRotation))) 45.0)) _newtrack_0) false false))
    (:Finished
      (Variables|Default|SetRotation (Math|Rotator|Lerp(Rotator) (Variables|Default|GetRotation) (Math|Rotator|MakeRotator (.Roll (Math|Rotator|BreakRotator (Variables|Default|GetRotation))) (.Pitch (Math|Rotator|BreakRotator (Variables|Default|GetRotation))) (+ (.Yaw (Math|Rotator|BreakRotator (Variables|Default|GetRotation))) 45.0)) _newtrack_0))
      (Variables|Default|SetInteractable true)
      (Variables|Default|Setcheck false))))

(fn ConstructionScript
  (|CallParentFunction))

(fn PuzzleCollector
  (params (ColorLaser :type Linear%20Color%20Structure) (Target :type Primitive%20Component%20Object%20Reference))
  (bind _returnvalue (Rendering|Material|CreateDynamicMaterialInstance Target 0 "/Game/IvanaKupala/Interactives/Pylons/M_Laser_2.M_Laser_2" "None" :!class /Script/Engine.PrimitiveComponent))
  (Rendering|Material|SetVectorParameterValue _returnvalue "Color" (Math|Color|SelectColor ColorLaser "(R=0.745098,G=0.070588,B=0.043137,A=1.000000)" (Variables|Default|GetActive)) :!class /Script/Engine.MaterialInstanceDynamic))

(fn ClearColor
  (params (Target :type Primitive%20Component%20Object%20Reference))
  (bind _returnvalue (Rendering|Material|CreateDynamicMaterialInstance Target 0 "/Game/IvanaKupala/Interactives/Pylons/M_Laser_2.M_Laser_2" "None" :!class /Script/Engine.PrimitiveComponent))
  (Rendering|Material|SetVectorParameterValue _returnvalue "Color" "(R=0.745098,G=0.070588,B=0.043137,A=1.000000)" :!class /Script/Engine.MaterialInstanceDynamic))

(fn LaserBounce
  (params (P_LaserHit :type BP%20Laser%20Object%20Reference) (P_HitResponce :type Boolean) (P_HitInformation :type Hit%20Result%20Structure) (P_HitComponent :type Primitive%20Component%20Object%20Reference))
  (bind _checkcolor (Variables|Default|GetCheckColor))
  (bind _activemiror (Variables|Default|GetActiveMiror))
  (bind _activemirors (Variables|Default|GetActiveMirors))
  (bind _activemiror_2 (Variables|Default|GetActiveMiror))
  (bind _output (Utilities|Array|Get(acopy) _activemiror_2 1))
  (bind _output_2 (Utilities|Array|Get(acopy) _activemiror))
  (bind _output_3 (Utilities|Array|Get(acopy) _activemirors 2))
  (bind _returnvalue (Components|GetChildComponent _output_3 0))
  (Variables|Default|SetActive P_HitResponce)
  (Utilities|Array|AddUnique (Variables|Default|GetCheckMirors) P_HitComponent)
  (if (< (Utilities|Array|Length (Variables|Default|GetCheckMirors)) 3)
    (Utilities|FlowControl|Sequence
      (:then_0
        (if (or (== (Utilities|Array|Get(acopy) (Variables|Default|GetActiveMiror)) (Utilities|Array|Get(acopy) (Variables|Default|GetCheckMirors))) (== (Utilities|Array|Get(acopy) (Variables|Default|GetActiveMiror)) (Utilities|Array|Get(acopy) (Variables|Default|GetCheckMirors) 1)))
          (Variables|Default|SetFirst_input true)
          (Variables|Default|SetFirst_laser_color (Variables|/Game/IvanaKupala/Interactives/Pylons/BP_LasersParent.BP_LasersParent_C|GetLaserColor P_LaserHit))
          (CallFunction|PuzzleCollector (Variables|/Game/IvanaKupala/Interactives/Pylons/BP_LasersParent.BP_LasersParent_C|GetLaserColor P_LaserHit) _output_2)
          (else
            (Variables|Default|SetFirst_input false)
            (Variables|Default|SetFirst_laser_color "(R=0.000000,G=0.000000,B=0.000000,A=1.000000)")
            (CallFunction|ClearAllLasersAttached)
            (Variables|Default|SetNeedLaser true)
            (CallFunction|ClearColor _output_2))))
      (:then_1
        (if (or (== (Utilities|Array|Get(acopy) (Variables|Default|GetActiveMiror) 1) (Utilities|Array|Get(acopy) (Variables|Default|GetCheckMirors))) (== (Utilities|Array|Get(acopy) (Variables|Default|GetActiveMiror) 1) (Utilities|Array|Get(acopy) (Variables|Default|GetCheckMirors) 1)))
          (Variables|Default|SetSecond_input true)
          (Variables|Default|SetSecond_laser_color (Variables|/Game/IvanaKupala/Interactives/Pylons/BP_LasersParent.BP_LasersParent_C|GetLaserColor P_LaserHit))
          (CallFunction|PuzzleCollector (Variables|/Game/IvanaKupala/Interactives/Pylons/BP_LasersParent.BP_LasersParent_C|GetLaserColor P_LaserHit) _output)
          (else
            (Variables|Default|SetSecond_input false)
            (Variables|Default|SetSecond_laser_color "")
            (CallFunction|ClearAllLasersAttached)
            (Variables|Default|SetNeedLaser true)
            (CallFunction|ClearColor _output))))
      (:then_2
        (if (Variables|Default|Getcheck)
          (Utilities|Array|RemoveIndex (Variables|Default|GetCheckMirors))
          (else
            (Utilities|IsValid P_LaserHit
              (:Is%20Valid
                (Variables|Default|SetSpawnReference (Variables|/Game/IvanaKupala/Interactives/Pylons/BP_LasersParent.BP_LasersParent_C|GetSpawnReference P_LaserHit))
                (if (Math|Boolean|ANDBoolean (Variables|Default|GetSecond_input) (Variables|Default|GetFirst_input) (== (Variables|Default|GetFirst_laser_color) _checkcolor) (== _checkcolor (Variables|Default|GetSecond_laser_color)))
                  (if (Variables|Default|GetNeedLaser)
                    (bind _returnvalue_2 (Game|SpawnActorfromClass "/Game/IvanaKupala/Interactives/Pylons/BP_Laser.BP_Laser_C" (Math|Transform|MakeTransform (Transformation|GetWorldLocation _returnvalue) "-90.000000,0.000000,0.000000" "1.000000,1.000000,1.000000") "Undefined" "OverrideRootScale" 0 (Default|UpdateID P_LaserHit "C") (Variables|Default|GetNew_color) (Variables|Default|GetSpawnReference) 0))
                    (Transformation|AttachComponentToComponent _returnvalue_2 _returnvalue "None" "SnapToTarget" "KeepRelative" "KeepRelative" true)
                    (Utilities|Array|Add (Variables|Default|GetLasersAttached) _returnvalue_2)
                    (Utilities|Array|Add (Variables|/Game/IvanaKupala/Interactives/Pylons/BP_LasersSpawn.BP_LasersSpawn_C|GetChildLasers (Variables|Default|GetSpawnReference)) _returnvalue_2)
                    (Variables|Default|SetNeedLaser false)
                    (return _returnvalue_2)))))))))
    (else
      (Utilities|Array|RemoveIndex (Variables|Default|GetCheckMirors)))))