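; BP_ReflectLaser is a pylon interactive that bounces lasers by spawning a reflected BP_Laser at the impact point.
; On a hit, LaserBounce orients the new laser from impact normal and trace start, passes on color and spawn reference with an updated ID, and registers it as attached and child.
; Without a hit response, it destroys attached lasers whose IDs contain the incoming laser's ID, matching by substring.
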(fn ConstructionScript
  (|CallParentFunction))

(fn ClearAttachedLasers
  (params (P_ID_Clear :type String))
  (bind _arrayelement (Utilities|Array|ReverseforEachLoop (Variables|Default|GetLasersAttached))
    (:LoopBody
      (Utilities|IsValid _arrayelement
        (:Is%20Valid
          (if (Utilities|String|Contains (Variables|/Game/IvanaKupala/Interactives/Pylons/BP_Laser.BP_Laser_C|GetLaser%20ID _arrayelement) P_ID_Clear)
            (Actor|DestroyActor _arrayelement)
            (Utilities|Array|RemoveItem (Variables|Default|GetLasersAttached) _arrayelement)))))))

(fn LaserBounce
  (params (P_LaserHit :type BP%20Laser%20Object%20Reference) (P_HitResponce :type Boolean) (P_HitInformation :type Hit%20Result%20Structure) (P_HitComponent :type Primitive%20Component%20Object%20Reference))
  (bind (_bblockinghit _binitialoverlap _time _distance _location _impactpoint _normal _impactnormal _physmat _hitactor _hitcomponent _hitbonename _bonename _hititem _elementindex _faceindex _tracestart) (Collision|BreakHitResult P_HitInformation))
  (if P_HitResponce
    (bind _returnvalue (Game|SpawnActorfromClass "/Game/IvanaKupala/Interactives/Pylons/BP_Laser.BP_Laser_C" (Math|Transform|MakeTransform _impactpoint (|CalculateRotation _impactpoint _impactnormal _tracestart) "1.000000,1.000000,1.000000") "Undefined" "MultiplyWithRoot" 0 (Default|UpdateID P_LaserHit) (Variables|/Game/IvanaKupala/Interactives/Pylons/BP_LasersParent.BP_LasersParent_C|GetLaserColor P_LaserHit) (Variables|/Game/IvanaKupala/Interactives/Pylons/BP_LasersParent.BP_LasersParent_C|GetSpawnReference P_LaserHit) 0))
    (Utilities|Array|Add (Variables|Default|GetLasersAttached) _returnvalue)
    (Utilities|Array|Add (Variables|/Game/IvanaKupala/Interactives/Pylons/BP_LasersSpawn.BP_LasersSpawn_C|GetChildLasers (Variables|/Game/IvanaKupala/Interactives/Pylons/BP_LasersParent.BP_LasersParent_C|GetSpawnReference P_LaserHit)) _returnvalue)
    (return _returnvalue)
    (else
      (CallFunction|ClearAttachedLasers (Variables|/Game/IvanaKupala/Interactives/Pylons/BP_Laser.BP_Laser_C|GetLaser%20ID P_LaserHit)))))