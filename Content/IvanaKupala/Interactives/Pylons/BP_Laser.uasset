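; Laser beam segment for the pylon interactives, tinted by a dynamic material and able to link into chains of bounced lasers.
; Each tick it box-traces along its up vector and stretches its mesh to the hit or full range.
; It reports steady hits and lost targets through BPI_Lasers, asking its SpawnReference to remove following lasers when the target changes.
; CancelTargetHit releases the target and destroys the beam unless overridden.
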(event EventBeginPlay
  (CallFunction|ChangeColor))

(event EventTick
  (params (DeltaSeconds :type Float%20%28single-precision%29))
  (CallFunction|SetEndPoint))

(event EventInteract)

(fn ConstructionScript
  (|CallParentFunction))

(fn ChangeColor
  (bind _returnvalue (Rendering|Material|CreateDynamicMaterialInstance (Variables|Default|GetStaticMesh) 0 "/Game/IvanaKupala/Interactives/Pylons/M_Laser.M_Laser" "None" :!class /Script/Engine.PrimitiveComponent))
  (Rendering|Material|SetVectorParameterValue _returnvalue "Color" (Variables|Default|GetLaserColor) :!class /Script/Engine.MaterialInstanceDynamic))

(fn SetEndPoint
  (bind _returnvalue (Transformation|GetActorLocation))
  (bind _returnvalue_2 (Transformation|GetActorUpVector))
  (bind _returnvalue_3 (* _returnvalue_2 2.0))
  (bind _returnvalue_4 (+ _returnvalue _returnvalue_3))
  (bind _outhit (Collision|BoxTraceByChannel _returnvalue_4 (+ _returnvalue_4 (* _returnvalue_2 (LocalVariables|GetL_Range))) "0.500000,0.500000,0.500000" "0, 0, 0" "TraceTypeQuery1" false 0 "None"))
  (bind _output_get (LocalVariables|SetL_HitInfo _outhit))
  (LocalVariables|SetL_HitActor (.HitActor (Collision|BreakHitResult _output_get)))
  (LocalVariables|SetL_HitComponent (.HitComponent (Collision|BreakHitResult _output_get)))
  (Transformation|SetWorldScale3D (Variables|Default|GetSM_Pylon) (Math|Vector|MakeVector 0.05 0.05 (Math|Float|SelectFloat (/ (+ (.Distance (Collision|BreakHitResult _output_get)) 1.0) 1e+02) (/ (LocalVariables|GetL_Range) 1e+02) (.bBlockingHit (Collision|BreakHitResult _output_get)))))
  (LocalVariables|GetL_HitActor
    (:then
      (LocalVariables|GetL_HitComponent
        (:then
          (Utilities|FlowControl|Sequence
            (:then_0
              (if (and (== (Variables|Default|GetLastHitActor) (LocalVariables|GetL_HitActor)) (== (Variables|Default|GetLastHitComponent) (LocalVariables|GetL_HitComponent)))
                (if (Utilities|DoesObjectImplementInterface (LocalVariables|GetL_HitActor) "/Game/IvanaKupala/Interactives/Pylons/BPI_Lasers.BPI_Lasers_C")
                  (Class|BPILasers|LaserBounce(Message) (LocalVariables|GetL_HitActor) self true (LocalVariables|GetL_HitInfo) (LocalVariables|GetL_HitComponent)))
                (elif (Utilities|DoesObjectImplementInterface (Variables|Default|GetLastHitActor) "/Game/IvanaKupala/Interactives/Pylons/BPI_Lasers.BPI_Lasers_C")
                  (Default|RemoveFollowingLasers (Variables|Default|GetSpawnReference) self))))
            (:then_1
              (Variables|Default|SetLastHitComponent (LocalVariables|GetL_HitComponent))
              (Variables|Default|SetLastHitActor (LocalVariables|GetL_HitActor)))))
        (:else
          (Utilities|FlowControl|Sequence :!label _label
            (:then_0
              (bind _lasthitactor (Variables|Default|GetLastHitActor)
                (:then
                  (if (Utilities|DoesObjectImplementInterface _lasthitactor "/Game/IvanaKupala/Interactives/Pylons/BPI_Lasers.BPI_Lasers_C")
                    (Class|BPILasers|LaserBounce(Message) (Variables|Default|GetLastHitActor) self false (LocalVariables|GetL_HitInfo) (Variables|Default|GetLastHitComponent))))
                (:else)))
            (:then_1
              (Variables|Default|SetLastHitActor 0)
              (Variables|Default|SetLastHitComponent 0))))))
    (:else
      (goto _label))))

(fn UpdateID
  (params (P_Append :type String))
  (return (Utilities|String|Append (Variables|Default|GetLaser%20ID) P_Append)))

(fn CancelTargetHit
  (params (overide :type Boolean))
  (Utilities|FlowControl|Sequence
    (:then_0
      (bind _lasthitactor (Variables|Default|GetLastHitActor)
        (:then
          (bind _asbp_lasers_parent (Utilities|Casting|CastToBP_LasersParent _lasthitactor))
          (if (and (Utilities|DoesObjectImplementInterface _asbp_lasers_parent "/Game/IvanaKupala/Interactives/Pylons/BPI_Lasers.BPI_Lasers_C") (Utilities|Array|IsEmpty (Variables|/Game/IvanaKupala/Interactives/Pylons/BP_LasersParent.BP_LasersParent_C|GetLasersAttached _asbp_lasers_parent)))
            (Class|BPILasers|LaserBounce(Message) :self (Variables|Default|GetLastHitActor) :P_LaserHit self :P_HitComponent (Variables|Default|GetLastHitComponent))
            (else
              (Class|BPILasers|LaserBounce(Message) :self (Variables|Default|GetLastHitActor) :P_LaserHit self :P_HitComponent (Variables|Default|GetLastHitComponent))
              (Variables|/Game/IvanaKupala/Interactives/Pylons/BP_LasersParent.BP_LasersParent_C|SetActive _asbp_lasers_parent false))))
        (:else)))
    (:then_1
      (if overide
        (return false)
        (else
          (Actor|DestroyActor)
          (return true))))))