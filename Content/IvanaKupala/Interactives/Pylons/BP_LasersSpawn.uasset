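; Interactable laser emitter pylon that spawns a colored BP_Laser at its Arrow on BeginPlay and tracks the resulting chain in ChildLasers.
; Interacting turns the Sphere another 45 degrees in yaw through a Timeline, blocking re-interaction until finished.
; RemoveFollowingLasers prunes downstream lasers by walking the list backwards and matching LaserID substrings, with IDs rooted in the actor's name.
; A LightOff handler destroys all lasers, but its binding is unconnected.
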(event Custom|LightOff_Event
  (Actor|DestroyActor (Variables|Default|GetLaser))
  (for _array_element (Variables|Default|GetChildLasers)
    (Actor|DestroyActor _array_element)))

(event EventBeginPlay
  (bind _childlasers (Variables|Default|GetChildLasers))
  (|CallParentFunction)
  (Variables|Default|SetRotation (Variables|/Script/Engine.SceneComponent|GetRelativeRotation (Variables|Default|GetSphere)))
  (Variables|Default|SetSpawnReference self)
  (Variables|Default|SetID (Utilities|GetDisplayName self))
  (bind _returnvalue (Game|SpawnActorfromClass "/Game/IvanaKupala/Interactives/Pylons/BP_Laser.BP_Laser_C" (Math|Transform|MakeTransform (Transformation|GetWorldLocation (Variables|Default|GetArrow)) "-90.000000,0.000000,0.000000" "1.000000,1.000000,1.000000") "Undefined" "OverrideRootScale" 0 (Variables|Default|GetID) (Variables|Default|GetLaserColor) (Variables|Default|GetSpawnReference) 0))
  (Variables|Default|SetLaser _returnvalue)
  (Utilities|Array|Add _childlasers _returnvalue)
  (Transformation|AttachComponentToComponent (Utilities|Array|Get(acopy) _childlasers) (Variables|Default|GetArrow) "LeserPoint" "SnapToTarget" "KeepRelative" "KeepRelative" true))

(event Collision|EventActorBeginOverlap
  (params (OtherActor :type Actor%20Object%20Reference))
  (|CallParentFunction 0))

(event EventTick
  (params (DeltaSeconds :type Float%20%28single-precision%29))
  (|CallParentFunction 0.0))

(event EventInteracting
  (Variables|Default|SetInteractable false)
  (bind _asbp_top_down_controller (Utilities|Casting|CastToBP_TopDownController (Game|GetPlayerController 0)))
  (Variables|/Game/IvanaKupala/Oka/Input/BP_TopDownController.BP_TopDownController_C|SetDisabled_Input _asbp_top_down_controller false)
  (bind _newtrack_0 (Timeline|Timeline PlayFromStart)
    (:Update
      (Transformation|SetRelativeRotation (Variables|Default|GetSphere) (Math|Rotator|Lerp(Rotator) (Variables|Default|GetRotation) (Math|Rotator|MakeRotator (.Roll (Math|Rotator|BreakRotator (Variables|Default|GetRotation))) (.Pitch (Math|Rotator|BreakRotator (Variables|Default|GetRotation))) (+ (.Yaw (Math|Rotator|BreakRotator (Variables|Default|GetRotation))) 45.0)) _newtrack_0) false false))
    (:Finished
      (Variables|Default|SetRotation (Math|Rotator|Lerp(Rotator) (Variables|Default|GetRotation) (Math|Rotator|MakeRotator (.Roll (Math|Rotator|BreakRotator (Variables|Default|GetRotation))) (.Pitch (Math|Rotator|BreakRotator (Variables|Default|GetRotation))) (+ (.Yaw (Math|Rotator|BreakRotator (Variables|Default|GetRotation))) 45.0)) _newtrack_0))
      (Variables|Default|SetInteractable true))))

(fn ConstructionScript
  (|CallParentFunction))

(fn RemoveFollowingLasers
  (params (Laser%20Reference :type BP%20Laser%20Object%20Reference))
  (LocalVariables|SetID%20removed (Variables|/Game/IvanaKupala/Interactives/Pylons/BP_Laser.BP_Laser_C|GetLaser%20ID Laser%20Reference))
  (bind _arrayelement (Utilities|Array|ReverseforEachLoop (Variables|Default|GetChildLasers))
    (:LoopBody
      (Utilities|IsValid _arrayelement
        (:Is%20Valid
          (if (Utilities|String|Contains (Variables|/Game/IvanaKupala/Interactives/Pylons/BP_Laser.BP_Laser_C|GetLaser%20ID _arrayelement) (LocalVariables|GetID%20removed))
            (bind _remove_fromarray (Default|CancleTargetHit _arrayelement (Utilities|Enum|Equal(Enum) (Variables|/Game/IvanaKupala/Interactives/Pylons/BP_Laser.BP_Laser_C|GetLaser%20ID _arrayelement) (LocalVariables|GetID%20removed))))
            (if _remove_fromarray
              (Utilities|Array|RemoveItem (Variables|Default|GetChildLasers) _arrayelement))))))))