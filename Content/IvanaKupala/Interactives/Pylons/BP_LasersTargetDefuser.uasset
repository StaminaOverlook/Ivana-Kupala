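; Laser puzzle pylon that splits a laser hitting its input mirror into new lasers from its output mirrors.
; BeginPlay selects mirrors by index and tints them by input or output role, and interacting rotates the mirror assembly 45 degrees over a timeline.
; LaserBounce recolors the input mirror, spawns attached lasers in a new color registered with the source's spawn reference, and clears them when the hit ends.
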(event EventBeginPlay
  (|CallParentFunction)
  (Variables|Default|SetRotation (Variables|/Script/Engine.SceneComponent|GetRelativeRotation (Variables|Default|GetMirors)))
  (for _array_element (Variables|Default|GetIndexComponent)
    (Utilities|Array|Insert (Variables|Default|GetActiveMirors) (Utilities|Array|Get(acopy) (Utilities|Array|MakeArray (Variables|Default|GetMiror_0) (Variables|Default|GetMiror_1) (Variables|Default|GetMiror_2) (Variables|Default|GetMiror_3) (Variables|Default|GetMiror_4) (Variables|Default|GetMiror_5) (Variables|Default|GetMiror_6) (Variables|Default|GetMiror_7)) _array_element)))
  (for (_array_element_2 _array_index) (Variables|Default|GetActiveMirors)
    (bind _returnvalue (Rendering|Material|CreateDynamicMaterialInstance _array_element_2 0 "/Game/IvanaKupala/Interactives/Pylons/M_Laser_2.M_Laser_2" "None" :!class /Script/Engine.PrimitiveComponent))
    (if (== _array_index 2)
      (Rendering|Material|SetVectorParameterValue _returnvalue "Color" (Variables|Default|GetColor_input) :!class /Script/Engine.MaterialInstanceDynamic)
      (else
        (Rendering|Material|SetVectorParameterValue _returnvalue "Color" (Variables|Default|GetColor_output) :!class /Script/Engine.MaterialInstanceDynamic)
        (Utilities|Array|Add (Variables|Default|GetActiveMiror) _array_element_2)))))

(event EventInteracting
  (Variables|Default|SetInteractable false)
  (bind _asbp_top_down_controller (Utilities|Casting|CastToBP_TopDownController (Game|GetPlayerController 0)))
  (Variables|/Game/IvanaKupala/Oka/Input/BP_TopDownController.BP_TopDownController_C|SetDisabled_Input _asbp_top_down_controller false)
  (bind _newtrack_0 (Timeline|Timeline PlayFromStart)
    (:Update
      (Transformation|SetRelativeRotation (Variables|Default|GetMirors) (Math|Rotator|Lerp(Rotator) (Variables|Default|GetRotation) (Math|Rotator|MakeRotator (.Roll (Math|Rotator|BreakRotator (Variables|Default|GetRotation))) (.Pitch (Math|Rotator|BreakRotator (Variables|Default|GetRotation))) (+ (.Yaw (Math|Rotator|BreakRotator (Variables|Default|GetRotation))) 45.0)) _newtrack_0) false false))
    (:Finished
      (Variables|Default|SetRotation (Math|Rotator|Lerp(Rotator) (Variables|Default|GetRotation) (Math|Rotator|MakeRotator (.Roll (Math|Rotator|BreakRotator (Variables|Default|GetRotation))) (.Pitch (Math|Rotator|BreakRotator (Variables|Default|GetRotation))) (+ (.Yaw (Math|Rotator|BreakRotator (Variables|Default|GetRotation))) 45.0)) _newtrack_0))
      (Variables|Default|SetInteractable true))))

(fn ConstructionScript
  (|CallParentFunction))

(fn PuzzleDefuse
  (params (ColorLaser :type Linear%20Color%20Structure) (Target :type Primitive%20Component%20Object%20Reference))
  (bind _returnvalue (Rendering|Material|CreateDynamicMaterialInstance Target 0 "/Game/IvanaKupala/Interactives/Pylons/M_Laser_2.M_Laser_2" "None" :!class /Script/Engine.PrimitiveComponent))
  (Rendering|Material|SetVectorParameterValue _returnvalue "Color" (Math|Color|SelectColor ColorLaser "(R=0.745098,G=0.070588,B=0.043137,A=1.000000)" (Variables|Default|GetActive)) :!class /Script/Engine.MaterialInstanceDynamic))

(fn LaserBounce
  (params (P_LaserHit :type BP%20Laser%20Object%20Reference) (P_HitResponce :type Boolean) (P_HitInformation :type Hit%20Result%20Structure) (P_HitComponent :type Primitive%20Component%20Object%20Reference))
  (bind _activemirors (Variables|Default|GetActiveMirors))
  (bind _output (Utilities|Array|Get(acopy) _activemirors 2))
  (Variables|Default|SetActive P_HitResponce)
  (if (== P_HitComponent _output)
    (CallFunction|PuzzleDefuse (Variables|/Game/IvanaKupala/Interactives/Pylons/BP_LasersParent.BP_LasersParent_C|GetLaserColor P_LaserHit) _output)
    (Utilities|IsValid P_LaserHit
      (:Is%20Valid
        (Variables|Default|SetSpawnReference (Variables|/Game/IvanaKupala/Interactives/Pylons/BP_LasersParent.BP_LasersParent_C|GetSpawnReference P_LaserHit))
        (if (Variables|Default|GetActive)
          (if (Variables|Default|GetNeedLaser)
            (for _array_element (Variables|Default|GetActiveMiror)
              (bind _returnvalue (Game|SpawnActorfromClass "/Game/IvanaKupala/Interactives/Pylons/BP_Laser.BP_Laser_C" (Math|Transform|MakeTransform (Transformation|GetWorldLocation (Components|GetChildComponent _array_element 0)) "-90.000000,0.000000,0.000000" "1.000000,1.000000,1.000000") "Undefined" "OverrideRootScale" 0 (Default|UpdateID P_LaserHit "C") (Variables|Default|GetNew_color) (Variables|Default|GetSpawnReference) 0))
              (Transformation|AttachComponentToComponent _returnvalue (Components|GetChildComponent _array_element 0) "None" "SnapToTarget" "KeepRelative" "KeepRelative" true)
              (Utilities|Array|Add (Variables|Default|GetLasersAttached) _returnvalue)
              (Utilities|Array|Add (Variables|/Game/IvanaKupala/Interactives/Pylons/BP_LasersSpawn.BP_LasersSpawn_C|GetChildLasers (Variables|Default|GetSpawnReference)) _returnvalue))
            (Variables|Default|SetNeedLaser false)
            (return _returnvalue))
          (else
            (CallFunction|ClearAllLasersAttached)
            (Variables|Default|SetNeedLaser true)))))))