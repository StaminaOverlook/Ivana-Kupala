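; BP_Koldun is an interactable NPC that runs a multi-line dialogue with the player.
; Each interaction advances through NPCDialogue, showing name, text and portrait in a WB_Dialogue widget, with a short delay before re-enabling interaction.
; After the last line it removes the widget, restores controller input, fires the end-interaction dispatcher and calls EndDialogue.
; EndDialogue and Appear_NPC are empty events; visibility is switched on at BeginPlay.
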(event Custom|Appear_NPC
  (params (Location :type Vector))
  ;[1 1 1] Appear NPC
)

(event Custom|EndDialogue)

(event EventBeginPlay
  (CallFunction|Visibalityon))

(event Collision|EventActorBeginOverlap
  (params (OtherActor :type Actor%20Object%20Reference))
  (|CallParentFunction OtherActor) ; This node is disabled and will not be called.\nDrag off pins to build functionality.
)

(event EventTick
  (params (DeltaSeconds :type Float%20%28single-precision%29))
  (|CallParentFunction DeltaSeconds) ; This node is disabled and will not be called.\nDrag off pins to build functionality.
)

(event EventInteracting
  (bind _index (Variables|Default|Getindex))
  (bind _npc_dialogue (Variables|Default|GetNPC_Dialogue))
  (bind _output (Utilities|Array|Get(acopy) _npc_dialogue _index))
  (bind (_npc_name _dialogue_text _npc_sprite) (Utilities|Struct|BreakNPC_Chat _output))
  ;[1 1 1] Interacting
  (Utilities|FlowControl|Sequence
    (:then_0
      (Utilities|FlowControl|DoOnce false
        (:Completed
          (bind _newtrack_0 (Timeline|Timeline PlayFromStart)
            (:Update
              (Variables|Default|SetInteractBegin _newtrack_0))))))
    (:then_1
      (Variables|Default|SetInteractable false)
      (Math|Integer|IncrementInt (Variables|Default|Getindex)
        (:%20%20
          (if (< (Variables|Default|Getindex) (Utilities|Array|Length (Variables|Default|GetNPC_Dialogue)))
            (Variables|Default|GetDialogue_Widget
              (:then
                _)
              (:else
                (bind _returnvalue (UserInterface|CreateWidget "/Game/IvanaKupala/Interface/WB_Dialogue.WB_Dialogue_C" (Game|GetPlayerController 0)))
                (bind _output_get (Variables|Default|SetDialogue_Widget _returnvalue))
                (UserInterface|Viewport|AddtoViewport _output_get 0)))
            (Default|SetDialogue (Variables|Default|GetDialogue_Widget) _npc_name _dialogue_text _npc_sprite)
            (Utilities|FlowControl|Sequence
              (:then_0
                (Utilities|FlowControl|DoOnce false
                  (:Completed
                    (UserInterface|Animation|PlayAnimation (Variables|Default|GetDialogue_Widget) (Variables|/Game/IvanaKupala/Interface/WB_Dialogue.WB_Dialogue_C|GetAppear (Variables|Default|GetDialogue_Widget)) 0.0 1 "Forward" 1.0 false))))
              (:then_1
                (Utilities|FlowControl|Delay 0.5)
                (Variables|Default|SetInteractable true)))
            (else
              (Variables|Default|SetInteractable false)
              (bind _asbp_top_down_controller (Utilities|Casting|CastToBP_TopDownController (Game|GetPlayerController 0)))
              (Variables|/Game/IvanaKupala/Oka/Input/BP_TopDownController.BP_TopDownController_C|SetDisabled_Input _asbp_top_down_controller false)
              (Default|CallEndInteractionDispatcher)
              (Widget|RemovefromParent (Variables|Default|GetDialogue_Widget))
              (Variables|Default|SetFinishedSpeach true)
              (CallFunction|EndDialogue))))))))

(fn ConstructionScript
  (|CallParentFunction))