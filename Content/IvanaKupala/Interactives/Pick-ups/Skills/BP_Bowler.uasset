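; BP_Bowler is an interactable pick-up that grants the bowler to the player's Oka character.
; Its Interacting event turns off its own interactability, disables input through the top-down controller and plays the pickup montage on the character's mesh.
; When the montage completes, it calls GiveBowler on the character, restores input and interactability, then destroys itself.
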(event EventBeginPlay
  (|CallParentFunction) ; This node is disabled and will not be called.\nDrag off pins to build functionality.
)

(event Collision|EventActorBeginOverlap
  (params (OtherActor :type Actor%20Object%20Reference)))

(event EventTick
  (params (DeltaSeconds :type Float%20%28single-precision%29)))

(event EventInteracting
  (Variables|Default|SetInteractable false)
  (bind _asbp_top_down_controller (Utilities|Casting|CastToBP_TopDownController (Game|GetPlayerController 0)))
  (Variables|/Game/IvanaKupala/Oka/Input/BP_TopDownController.BP_TopDownController_C|SetDisabled_Input _asbp_top_down_controller true)
  (bind _asbp_oka_character (Utilities|Casting|CastToBP_OkaCharacter (Game|GetPlayerCharacter 0)))
  (Animation|Montage|PlayMontage (Variables|/Script/Engine.Character|GetMesh _asbp_oka_character) "/Game/IvanaKupala/Oka/Animations/Oka_Pick-up_Montage.Oka_Pick-up_Montage"
    (:OnCompleted
      (Default|GiveBowler _asbp_oka_character)
      (Variables|/Game/IvanaKupala/Oka/Input/BP_TopDownController.BP_TopDownController_C|SetDisabled_Input _asbp_top_down_controller false)
      (Variables|Default|SetInteractable true)
      (Actor|DestroyActor))))

(fn ConstructionScript
  (|CallParentFunction))