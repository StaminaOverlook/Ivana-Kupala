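; Skill pick-up that grants the Oka character its dash skills, named for Shield Dash.
; Its GiveSkill event calls GiveDashSkills on the stored character, clears DisabledInput on the top-down controller, sets Interactable to true and destroys the pick-up.
; The BeginPlay, overlap and Tick events are disabled stubs, so nothing in this graph triggers GiveSkill.
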(event EventBeginPlay
  (|CallParentFunction) ; This node is disabled and will not be called.\nDrag off pins to build functionality.
)

(event Collision|EventActorBeginOverlap
  (params (OtherActor :type Actor%20Object%20Reference))
  (|CallParentFunction OtherActor) ; This node is disabled and will not be called.\nDrag off pins to build functionality.
)

(event EventTick
  (params (DeltaSeconds :type Float%20%28single-precision%29))
  (|CallParentFunction DeltaSeconds) ; This node is disabled and will not be called.\nDrag off pins to build functionality.
)

(event EventGiveSkill
  (Default|GiveDashSkills (Variables|Default|GetAs%20BP%20Oka%20Character))
  (Variables|/Game/IvanaKupala/Oka/Input/BP_TopDownController.BP_TopDownController_C|SetDisabled_Input (Variables|Default|GetAs%20BP%20Top%20Down%20Controller) false)
  (Variables|Default|SetInteractable true)
  (Actor|DestroyActor))

(fn ConstructionScript
  (|CallParentFunction))