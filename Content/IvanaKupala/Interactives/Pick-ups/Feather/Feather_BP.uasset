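; Feather pick-up actor for the IvanaKupala interactives that spins in place and can be moved or removed through events.
; Tick rotates the actor around yaw by RotationSpeed scaled by delta time, based on the static mesh's world rotation.
; AppearNPC teleports the feather to a given location, and EndInteraction destroys it.
; The node binding to the EndInteraction dispatcher is unconnected and never runs.
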(event EventBeginPlay
  (|CallParentFunction) ; This node is disabled and will not be called.\nDrag off pins to build functionality.
)

(event Collision|EventActorBeginOverlap
  (params (OtherActor :type Actor%20Object%20Reference))
  (|CallParentFunction OtherActor) ; This node is disabled and will not be called.\nDrag off pins to build functionality.
)

(event EventTick
  (params (DeltaSeconds :type Float%20%28single-precision%29))
  (bind _staticmesh (Variables|Default|GetStaticMesh))
  (bind _returnvalue (Transformation|GetWorldRotation _staticmesh))
  ;[1 1 1] Rotation
  (Transformation|SetActorRotation (Math|Rotator|MakeRotator (.roll _returnvalue) (.pitch _returnvalue) (+ (.yaw _returnvalue) (* DeltaSeconds (Variables|Default|GetRotationSpeed))))))

(event EventAppearNPC
  (params (Location :type Vector :default "0, 0, 0"))
  (Transformation|SetActorLocation Location false true))

(event EventEndInteraction
  (Actor|DestroyActor))

(fn ConstructionScript
  (|CallParentFunction))