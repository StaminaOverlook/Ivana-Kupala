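; Svistulka collectible pickup that the player collects through a two-step interaction.
; The first interaction locks controller input and interactability, ends the interaction, plays Oka's pickup montage, then after its duration shows the WB_SvistulkaPickUp widget and re-enables interaction.
; The second interaction removes the widget, restores input and destroys the actor.
; BeginPlay calls VisibilityOn; the spin logic is disconnected from Tick, so it never runs.
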(event EventBeginPlay
  (CallFunction|Visibilityon))

(event Collision|EventActorBeginOverlap
  (params (OtherActor :type Actor%20Object%20Reference))
  (|CallParentFunction OtherActor) ; This node is disabled and will not be called.\nDrag off pins to build functionality.
)

(event EventTick
  (params (DeltaSeconds :type Float%20%28single-precision%29))
  ;[1 1 1] Rotation
)

(event EventInteracting
  ;[1 1 1] Interacting
  (if (Variables|Default|GetWidgetExists)
    (Widget|RemovefromParent (Variables|Default|GetRuneWidget))
    (bind _top_down_controller (Utilities|GetTopDownController))
    (Variables|/Game/IvanaKupala/Oka/Input/BP_TopDownController.BP_TopDownController_C|SetDisabled_Input _top_down_controller false)
    (Actor|DestroyActor)
    (else
      (Variables|Default|SetInteractable false)
      (bind _top_down_controller_2 (Utilities|GetTopDownController))
      (Variables|/Game/IvanaKupala/Oka/Input/BP_TopDownController.BP_TopDownController_C|SetDisabled_Input _top_down_controller_2 true)
      (Default|CallEndInteractionDispatcher)
      (bind _oka (Utilities|GetOkaCharacter)
        (:Out
          (bind _returnvalue (Animation|PlayAnimMontage _oka "/Game/IvanaKupala/Oka/Animations/Oka_Pick-up_Montage.Oka_Pick-up_Montage" 1.0 "None"))
          (Utilities|FlowControl|Delay _returnvalue)
          (bind _returnvalue_2 (UserInterface|CreateWidget "/Game/IvanaKupala/Interactives/Pick-ups/Collectibles/WB_SvistulkaPickUp.WB_SvistulkaPickUp_C" (Game|GetPlayerController 0)))
          (bind _output_get (Variables|Default|SetRuneWidget _returnvalue_2))
          (UserInterface|Viewport|AddtoViewport _output_get 0)
          (Variables|Default|SetWidgetExists true)
          (Variables|Default|SetInteractable true))))))

(fn ConstructionScript
  (|CallParentFunction))