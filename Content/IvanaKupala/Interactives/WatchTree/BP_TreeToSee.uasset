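; BP_TreeToSee is an interactable tree that plays a two-stage cutscene when the player uses it.
; Each Interacting event clears DisabledInput on the top-down controller.
; Once FinishedView is set, the first interaction creates and plays the CutsceneTreeUse level sequence, then pauses it after a short delay.
; A later interaction resumes the paused sequence, tracked by the InteractGoes and IsPaused flags.
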(event EventBeginPlay
  (|CallParentFunction) ; This node is disabled and will not be called.\nDrag off pins to build functionality.
)

(event Collision|EventActorBeginOverlap
  (params (OtherActor :type Actor%20Object%20Reference))
  (|CallParentFunction OtherActor) ; This node is disabled and will not be called.\nDrag off pins to build functionality.
)

(event EventTick
  (params (DeltaSeconds :type Float%20%28single-precision%29))
  (|CallParentFunction DeltaSeconds) ; This node is disabled and will not be called.\nDrag off pins to build functionality.
)

(event EventInteracting
  (bind _top_down_controller (Utilities|GetTopDownController))
  (Variables|/Game/IvanaKupala/Oka/Input/BP_TopDownController.BP_TopDownController_C|SetDisabled_Input _top_down_controller false)
  (if (Variables|Default|GetInteractGoes)
    (if (Variables|Default|GetisPaused)
      (Sequencer|Player|Play (Variables|/Script/LevelSequence.LevelSequenceActor|GetSequencePlayer (Variables|Default|GetOut%20Actor)) :!class /Script/MovieScene.MovieSceneSequencePlayer))
    (elif (Variables|Default|GetFinishedView)
      (Variables|Default|SetInteractGoes true)
      (bind _outactor (Sequencer|Player|CreateLevelSequencePlayer "/Game/IvanaKupala/Maps/Levels/Cutscenes/CutsceneTreeUse.CutsceneTreeUse"))
      (bind _output_get (Variables|Default|SetOut%20Actor _outactor))
      (Sequencer|Player|Play (Variables|/Script/LevelSequence.LevelSequenceActor|GetSequencePlayer _output_get) :!class /Script/MovieScene.MovieSceneSequencePlayer)
      (Utilities|FlowControl|Delay 1.5)
      (Sequencer|Player|Pause (Variables|/Script/LevelSequence.LevelSequenceActor|GetSequencePlayer _output_get))
      (Variables|Default|SetisPaused true))))

(fn ConstructionScript
  (|CallParentFunction))