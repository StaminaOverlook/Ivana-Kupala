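; Interactable watch tree that gives the player a raised overview by lifting the Oka character's camera.
; On interaction it disables itself and a timeline lerps the camera up by DeltaZ and back along X in proportion, then opens the WatchTree widget in UI-only input.
; Closing watch mode removes the widget and plays a second timeline to lower the camera, restoring game input and interactability during its updates.
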(event Custom|CloseWatchMode_Event
  (Widget|RemovefromParent (Variables|Default|GetWidget_watchtree))
  (bind _newtrack_0 (Timeline|Timeline_0 PlayFromStart)
    (:Update
      (Transformation|SetRelativeLocation (Variables|/Game/IvanaKupala/Oka/BP_OkaCharacter.BP_OkaCharacter_C|GetCamera (stale EventInteracting _oka)) (Math|Vector|Lerp(Vector) (Variables|Default|GetUpPosition) (Variables|Default|GetDownPosition) _newtrack_0) false false)
      (bind _top_down_controller (Utilities|GetTopDownController))
      (Variables|/Game/IvanaKupala/Oka/Input/BP_TopDownController.BP_TopDownController_C|SetDisabled_Input _top_down_controller false)
      (Variables|Default|SetInteractable true)
      (Input|SetInputModeGameOnly (Game|GetPlayerController 0) false))))

(event EventBeginPlay)

(event Collision|EventActorBeginOverlap
  (params (OtherActor :type Actor%20Object%20Reference)))

(event EventTick
  (params (DeltaSeconds :type Float%20%28single-precision%29)))

(event EventInteracting
  (bind _returnvalue (Game|GetPlayerController 0))
  (Variables|Default|SetInteractable false)
  (bind _oka (Utilities|GetOkaCharacter)
    (:Out
      (Variables|Default|SetDownPosition (Variables|/Script/Engine.SceneComponent|GetRelativeLocation (Variables|/Game/IvanaKupala/Oka/BP_OkaCharacter.BP_OkaCharacter_C|GetCamera _oka)))
      (Variables|Default|SetUpPosition (+ (Variables|/Script/Engine.SceneComponent|GetRelativeLocation (Variables|/Game/IvanaKupala/Oka/BP_OkaCharacter.BP_OkaCharacter_C|GetCamera _oka)) (Math|Vector|MakeVector (- 0.0 (/ (Variables|Default|GetDelta_Z) 0.53)) 0.0 (Variables|Default|GetDelta_Z))))
      (bind _newtrack_0 (Timeline|Timeline PlayFromStart)
        (:Update
          (Transformation|SetRelativeLocation (Variables|/Game/IvanaKupala/Oka/BP_OkaCharacter.BP_OkaCharacter_C|GetCamera _oka) (Math|Vector|Lerp(Vector) (Variables|Default|GetDownPosition) (Variables|Default|GetUpPosition) _newtrack_0) false false))
        (:Finished
          (bind _returnvalue_2 (UserInterface|CreateWidget "/Game/IvanaKupala/Interactives/WatchTree/WBP_WatchTreeWidget.WBP_WatchTreeWidget_C" _returnvalue))
          (Variables|Default|SetWidget_watchtree _returnvalue_2)
          (UserInterface|Viewport|AddtoViewport _returnvalue_2 0)
          (Input|SetInputModeUIOnly _returnvalue _returnvalue_2 "LockAlways" false)
          (bind _top_down_controller (Utilities|GetTopDownController))
          (Variables|/Game/IvanaKupala/Oka/Input/BP_TopDownController.BP_TopDownController_C|SetDisabled_Input _top_down_controller false))))))

(fn ConstructionScript
  (|CallParentFunction))