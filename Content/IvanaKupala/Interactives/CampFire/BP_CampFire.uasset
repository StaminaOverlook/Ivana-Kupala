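; BP_CampFire is an interactable campfire that acts as a checkpoint, healing the player and saving the game.
; Each interaction heals by the player's max health, saves the current level through the TopDown game mode, and re-enables controller input.
; The first use runs SkipAction once, swapping the mesh material, showing the Niagara effect and point light, and setting Lit.
; IsActionOver reports Lit.
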(event EventSkipAction
  (Rendering|Material|SetMaterial (Variables|Default|GetStaticMesh) 0 "/Game/IvanaKupala/Interactives/CampFire/M_Campfire.M_Campfire")
  (Rendering|SetVisibility (Variables|Default|GetNiagara) true false)
  (Rendering|SetVisibility (Variables|Default|GetPointLight) true false)
  (Variables|Default|SetLit true))

(event EventInteracting
  (bind _returnvalue (Game|Player|GetPlayerPawn 0))
  (bind _returnvalue_2 (Actor|GetComponentbyClass _returnvalue "/Game/IvanaKupala/Interface/HealthComponent.HealthComponent_C"))
  (Utilities|FlowControl|Sequence
    (:then_0
      (Default|EventHeal _returnvalue_2 (Variables|/Game/IvanaKupala/Interface/HealthComponent.HealthComponent_C|GetMaxHealth _returnvalue_2))
      (bind _bp_top_down_game_mode (Utilities|GetTopDownGameMode)
        (:Out
          (bind _returnvalue_3 (Game|GetCurrentLevelName true))
          (Default|SaveGame _bp_top_down_game_mode _returnvalue_3 true))))
    (:then_1
      (Variables|Default|SetInteractable false))
    (:then_2
      (Utilities|FlowControl|DoOnce false
        (:Completed
          (CallFunction|SkipAction))))
    (:then_3
      (bind _top_down_controller (Utilities|GetTopDownController))
      (Variables|/Game/IvanaKupala/Oka/Input/BP_TopDownController.BP_TopDownController_C|SetDisabled_Input _top_down_controller false)
      (Variables|Default|SetInteractable true))))

(fn ConstructionScript)

(fn IsActionOver
  (return (Variables|Default|GetLit)))