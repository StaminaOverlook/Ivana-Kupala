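; Base interactable actor with a widget prompt, an interaction entry point and save-state support.
; When Interactable, it shows the prompt on BeginPlay; Interact disables top-down controller input, hides the prompt and calls the empty Interacting hook.
; Save data stores the Interactable flag under the object name; loading restores it and calls the empty EndInteraction hook if true.
; Sphere overlap events check for BP_OkaCharacter but take no action.
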(event OnComponentBeginOverlap(SphereCollision)
  (params (OverlappedComponent :type Primitive%20Component%20Object%20Reference) (OtherActor :type Actor%20Object%20Reference) (OtherComp :type Primitive%20Component%20Object%20Reference) (OtherBodyIndex :type Integer) (bFromSweep :type Boolean) (SweepResult :type Hit%20Result%20Structure%20%28by%20ref%29))
  ;[1 1 1] Prompt button
  (if (and (Variables|Default|GetInteractable) (CallFunction|IsChildOf OtherActor "/Game/IvanaKupala/Oka/BP_OkaCharacter.BP_OkaCharacter_C"))
    _))

(event OnComponentEndOverlap(SphereCollision)
  (params (OverlappedComponent :type Primitive%20Component%20Object%20Reference) (OtherActor :type Actor%20Object%20Reference) (OtherComp :type Primitive%20Component%20Object%20Reference) (OtherBodyIndex :type Integer))
  ;[1 1 1] Prompt button
  (if (and (Variables|Default|GetInteractable) (CallFunction|IsChildOf OtherActor "/Game/IvanaKupala/Oka/BP_OkaCharacter.BP_OkaCharacter_C"))
    _))

(event Custom|Interacting)

(event Custom|End%20Interaction)

(event Custom|VisibilityOn
  (Rendering|SetVisibility (Variables|Default|GetWidget) true false))

(event Custom|VisibilityOff
  (Rendering|SetVisibility (Variables|Default|GetWidget) false false))

(event EventBeginPlay
  (if (Variables|Default|GetInteractable)
    ;[1 1 1] Prompt button
    (Rendering|SetVisibility (Variables|Default|GetWidget) true false)))

(event EventLoadInteractionSaveData
  (params (SaveData :type Interaction%20Save%20Data%20Structure))
  (bind _output_get (Variables|Default|SetInteractable (Utilities|Struct|BreakInteractionSaveData SaveData)))
  (if _output_get
    (CallFunction|EndInteraction)))

(event EventInteract
  ;[1 1 1] Interaction Event
  (if (Variables|Default|GetInteractable)
    (bind _top_down_controller (Utilities|GetTopDownController))
    (Variables|/Game/IvanaKupala/Oka/Input/BP_TopDownController.BP_TopDownController_C|SetDisabled_Input _top_down_controller true)
    (Rendering|SetVisibility (Variables|Default|GetWidget) false false)
    (CallFunction|Interacting)))

(fn ConstructionScript)

(fn GetInteractionSaveData
  (return (Utilities|Struct|MakeInteractionSaveData (Variables|Default|GetInteractable) false) (Utilities|GetObjectName self)))