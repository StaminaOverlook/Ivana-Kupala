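; BP_Root_Door is a door that burns away and is destroyed when a BP_Coal or BP_FireCoal overlaps its box.
; It bakes each mesh material into a render target and feeds that as BurnTexture to a dynamic Transition_Mat instance.
; It stamps BurnStart with real time to drive the transition, then destroys the actor after a short delay.
; The separate Burn event is empty.
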(event OnComponentBeginOverlap(Box)
  (params (OverlappedComponent :type Primitive%20Component%20Object%20Reference) (OtherActor :type Actor%20Object%20Reference) (OtherComp :type Primitive%20Component%20Object%20Reference) (OtherBodyIndex :type Integer) (bFromSweep :type Boolean) (SweepResult :type Hit%20Result%20Structure%20%28by%20ref%29))
  (bind _staticmesh (Variables|Default|GetStaticMesh))
  (if (or (== (Utilities|GetClass OtherActor) "/Game/IvanaKupala/Oka/Skills/CauldronSkills/BP_Coal.BP_Coal_C") (== (Utilities|GetClass OtherActor) "/Game/IvanaKupala/Oka/Skills/CauldronSkills/BP_FireCoal.BP_FireCoal_C"))
    (for (_array_element _array_index) (Rendering|Material|GetMaterials _staticmesh)
      (bind _returnvalue (CanvasRenderTarget2D|CreateCanvasRenderTarget2D 0 1024 1024))
      (Rendering|DrawMaterialtoRenderTarget _returnvalue _array_element)
      (bind _returnvalue_2 (Rendering|Material|CreateDynamicMaterialInstance _staticmesh _array_index "/Game/IvanaKupala/Maps/Transitions/Transition_Mat.Transition_Mat" "Burn" :!class /Script/Engine.PrimitiveComponent))
      (Rendering|Material|SetTextureParameterValue _returnvalue_2 "BurnTexture" _returnvalue)
      (Rendering|Material|SetScalarParameterValueonMaterials _staticmesh "BurnStart" (Utilities|Time|GetRealTimeSeconds))
      (Utilities|FlowControl|Delay 5.0)
      (Actor|DestroyActor))))

(event EventBurn)

(fn ConstructionScript)