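; BP_TreeToSee is an interactable tree actor that plays a level sequence when used.
; If TreeUse is set, interacting disables top-down controller input and interactability, then plays the sequence and pauses it after 1.5 seconds; otherwise it re-enables input.
; PlayScene resumes the sequence, and EndInteraction restores interactability and input.
; Appear_NPC is empty, and leftover NPC dialogue widget logic is disconnected.
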(event Custom|Appear_NPC
  (params (Location :type Vector))
  ;[1 1 1] Appear NPC
)

(event Custom|PlayScene
  (Sequencer|Player|Play (Variables|/Script/LevelSequence.LevelSequenceActor|GetSequencePlayer (stale EventInteracting _outactor)) :!class /Script/MovieScene.MovieSceneSequencePlayer))

(event EventBeginPlay
  (|CallParentFunction) ; This node is disabled and will not be called.\nDrag off pins to build functionality.
)

(event Collision|EventActorBeginOverlap
  (params (OtherActor :type Actor%20Object%20Reference))
  (|CallParentFunction OtherActor) ; This node is disabled and will not be called.\nDrag off pins to build functionality.
)

(event EventTick
  (params (DeltaSeconds :type Float%20%28single-precision%29))
  (|CallParentFunction DeltaSeconds) ; This node is disabled and will not be called.\nDrag off pins to build functionality.
)

(event EventInteracting
  (if (Variables|Default|GetTreeUse)
    (bind _asbp_top_down_controller (Utilities|Casting|CastToBP_TopDownController (Game|GetPlayerController 0)))
    (Variables|/Game/IvanaKupala/Oka/Input/BP_TopDownController.BP_TopDownController_C|SetDisabled_Input _asbp_top_down_controller true)
    (bind _outactor (Sequencer|Player|CreateLevelSequencePlayer (Variables|Default|GetLevel%20Sequence)))
    (Sequencer|Player|Play (Variables|/Script/LevelSequence.LevelSequenceActor|GetSequencePlayer _outactor) :!class /Script/MovieScene.MovieSceneSequencePlayer)
    (Variables|Default|SetInteractable false)
    (Utilities|FlowControl|Delay 1.5)
    (Sequencer|Player|Pause (Variables|/Script/LevelSequence.LevelSequenceActor|GetSequencePlayer _outactor))
    (else
      (bind _asbp_top_down_controller_2 (Utilities|Casting|CastToBP_TopDownController (Game|GetPlayerController 0)))
      (Variables|/Game/IvanaKupala/Oka/Input/BP_TopDownController.BP_TopDownController_C|SetDisabled_Input _asbp_top_down_controller_2 false))))

(event EventEndInteraction
  (Variables|Default|SetInteractable true)
  (bind _asbp_top_down_controller (Utilities|Casting|CastToBP_TopDownController (Game|GetPlayerController 0)))
  (Variables|/Game/IvanaKupala/Oka/Input/BP_TopDownController.BP_TopDownController_C|SetDisabled_Input _asbp_top_down_controller false))

(fn ConstructionScript
  (|CallParentFunction))