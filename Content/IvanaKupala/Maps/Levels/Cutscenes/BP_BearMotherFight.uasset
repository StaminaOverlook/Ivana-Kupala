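; Cutscene Blueprint that introduces the Bear Mother boss fight.
; When the cutscene ends, it reveals the BearMotherInstance mesh and disables its trigger.
; Through the top-down game mode it fades the background music, plays the bear's spawn animation, then after a short delay starts the Mother Bear track.
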(event EventAfterCutscene
  (Rendering|SetVisibility (Variables|/Script/Engine.Character|GetMesh (Variables|Default|GetBearMotherInstance)) true false)
  (CallFunction|DisableTrigger)
  (bind _bp_top_down_game_mode (Utilities|GetTopDownGameMode)
    (:Out
      (Default|FadeBGM _bp_top_down_game_mode)
      (Default|SpawnAmination (Variables|Default|GetBearMotherInstance))
      (Utilities|FlowControl|Delay 6.2)
      (Default|SetandPlayBGM _bp_top_down_game_mode "/Game/IvanaKupala/Maps/Music/Mother_Bear.Mother_Bear"))))

(fn ConstructionScript
  (|CallParentFunction))