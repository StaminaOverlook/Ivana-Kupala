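; Cutscene actor that plays a monologue and becomes usable once four wolves are dead.
; BeforeCutscene calls Say on its Monologue.
; SpecialSituation loops over the Wolves array, counting invalid references or wolves with no health left as dead.
; A count of exactly four sets Usable; any other count resets the tally to zero for the next check.
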(event EventSpecialSituation
  (for _array_element (Variables|Default|GetWolves)
    (if (Utilities|IsValid _array_element)
      (if (<= (Variables|/Game/IvanaKupala/Interface/HealthComponent.HealthComponent_C|GetHealth (Variables|/Game/IvanaKupala/Monsters/BP_MonsterAI.BP_MonsterAI_C|GetHealthComponent _array_element)) 0.0)
        (bind _result (Math|Integer|IncrementInt (Variables|Default|GetDeadWolves) :!label _label)
          (:%20%20
            (Variables|Default|SetDeadWolves _result))))
      (else
        (goto _label))))
  (if (== (Variables|Default|GetDeadWolves) 4)
    (Variables|Default|SetUsable true)
    (else
      (Variables|Default|SetDeadWolves 0))))

(event Collision|EventActorBeginOverlap
  (params (OtherActor :type Actor%20Object%20Reference))
  (|CallParentFunction OtherActor) ; This node is disabled and will not be called.\nDrag off pins to build functionality.
)

(event EventTick
  (params (DeltaSeconds :type Float%20%28single-precision%29)))

(event EventBeforeCutscene
  (Default|Say (Variables|Default|GetMonologue)))

(event EventBeginPlay)

(fn ConstructionScript
  (|CallParentFunction))