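; BP_Monologue is an interactive level Blueprint that plays a monologue from its TalkData while locking player input.
; Say disables input on the top-down controller, starts the talk, and binds to the monologue widget's TalkOver event.
; When the talk ends, ReenableMovement restores input and unbinds itself from that event.
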(event Custom|Reenable%20movement
  (bind _top_down_controller (Utilities|GetTopDownController))
  (Variables|/Game/IvanaKupala/Oka/Input/BP_TopDownController.BP_TopDownController_C|SetDisabled_Input _top_down_controller false)
  (EventDispatchers|UnbindEventfromTalkOver (Variables|/Game/IvanaKupala/Oka/Input/BP_TopDownController.BP_TopDownController_C|GetWB_Monologue _top_down_controller) (delegate Custom|Reenable%20movement)))

(event EventSay
  (bind _top_down_controller (Utilities|GetTopDownController))
  (Variables|/Game/IvanaKupala/Oka/Input/BP_TopDownController.BP_TopDownController_C|SetDisabled_Input _top_down_controller true)
  (Default|StartTalk _top_down_controller (Variables|Default|GetTalkData))
  (EventDispatchers|BindEventtoTalkOver (Variables|/Game/IvanaKupala/Oka/Input/BP_TopDownController.BP_TopDownController_C|GetWB_Monologue _top_down_controller) (delegate Custom|Reenable%20movement)))

(fn ConstructionScript)