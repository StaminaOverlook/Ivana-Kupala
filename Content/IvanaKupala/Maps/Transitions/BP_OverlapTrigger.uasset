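; Overlap trigger actor for map transitions that plays an optional level sequence cutscene when an actor enters it.
; Empty BeforeCutscene and AfterCutscene hooks bracket the Play call; AfterCutscene runs immediately, without waiting for playback to finish.
; Each overlap decrements UseCount, destroying the actor at zero.
; SkipAction jumps the sequence to its end and reruns AfterCutscene, while helper functions enable or disable collision.
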(event Custom|Consume
  (bind _result (Math|Integer|DecrementInt (Variables|Default|GetUseCount))
    (:%20%20
      (if (== _result 0)
        (Actor|DestroyActor)))))

(event Custom|BeforeCutscene)

(event Custom|AfterCutscene)

(event EventSkipAction
  (bind _cutscene (Variables|Default|GetCutscene))
  (bind _cutscene_2 (Variables|Default|GetCutscene))
  (bind _sequenceplayer (Variables|/Script/LevelSequence.LevelSequenceActor|GetSequencePlayer _cutscene))
  (bind _returnvalue (Class|MovieSceneSequencePlayer|GetEndTime _sequenceplayer))
  (bind (_frame _framerate _subframe) (Utilities|TimeManagement|BreakQualifiedFrameTime _returnvalue))
  (if (Utilities|IsValid _cutscene_2)
    (Components|Timeline|SetPlaybackPosition (Variables|/Script/LevelSequence.LevelSequenceActor|GetSequencePlayer _cutscene_2) (Utilities|Struct|MakeMovieSceneSequencePlaybackParams (Utilities|Struct|MakeFrameTime _frame _subframe) 0.0 "" "(Hours=0,Minutes=0,Seconds=0,Frames=0,bDropFrameFormat=False)" "Frame" "Play")))
  (CallFunction|AfterCutscene))

(event Collision|EventActorBeginOverlap
  (params (OtherActor :type Actor%20Object%20Reference))
  (bind _cutscene (Variables|Default|GetCutscene))
  (CallFunction|BeforeCutscene)
  (if (Utilities|IsValid _cutscene)
    (Sequencer|Player|Play (Variables|/Script/LevelSequence.LevelSequenceActor|GetSequencePlayer _cutscene) :!class /Script/MovieScene.MovieSceneSequencePlayer))
  (CallFunction|AfterCutscene)
  (CallFunction|Consume))

(fn ConstructionScript)

(fn DisableTrigger
  (Collision|SetCollisionEnabled (Variables|Default|GetCollisionComponent) "NoCollision")
  (Collision|SetActorEnableCollision false))

(fn EnableTrigger
  (Collision|SetCollisionEnabled (Variables|Default|GetCollisionComponent) "QueryOnly")
  (Collision|SetActorEnableCollision true))