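; BP_Coal is a small coal projectile, apparently for Oka's TakeAim skill, that damages what it hits.
; Projectile movement takes its velocity from a variable at BeginPlay, and the actor destroys itself after a fixed delay or once it stops moving.
; Sphere overlaps apply damage and destroy the coal only for actors implementing DamageInterface, excluding the Oka character and shield classes.
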(event OnComponentBeginOverlap(Sphere)
  (params (OverlappedComponent :type Primitive%20Component%20Object%20Reference) (OtherActor :type Actor%20Object%20Reference) (OtherComp :type Primitive%20Component%20Object%20Reference) (OtherBodyIndex :type Integer) (bFromSweep :type Boolean) (SweepResult :type Hit%20Result%20Structure%20%28by%20ref%29))
  (if (Math|Boolean|ANDBoolean (Utilities|DoesObjectImplementInterface OtherActor "/Game/IvanaKupala/Interface/DamageInterface.DamageInterface_C") (!= (Utilities|GetClass OtherActor) "/Game/IvanaKupala/Oka/BP_OkaCharacter.BP_OkaCharacter_C") (!= (Utilities|GetClass OtherActor) "/Game/IvanaKupala/Oka/ShieldClass.ShieldClass_C"))
    (Game|Damage|ApplyDamage OtherActor (Variables|Default|GetCoalDamage) 0 self)
    (Actor|DestroyActor)))

(event EventBeginPlay
  (Variables|/Script/Engine.MovementComponent|SetVelocity (Variables|Default|GetProjectileMovement) (Variables|Default|GetVilocity))
  (Utilities|FlowControl|Delay 5.0)
  (Actor|DestroyActor))

(event EventTick
  (params (DeltaSeconds :type Float%20%28single-precision%29))
  (if (Utilities|Operators|EqualEqual :A (Variables|/Script/Engine.MovementComponent|GetVelocity (Variables|Default|GetProjectileMovement)) :ErrorTolerance 0.01)
    (Actor|DestroyActor)))

(fn ConstructionScript
  (Transformation|SetWorldScale3D (Variables|Default|GetStaticMesh) "0.050000,0.050000,0.050000"))