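; BP_FirePuddle is a short-lived fire area for the cauldron skills that deals periodic damage to actors inside it, then destroys itself after five seconds.
; Its sphere overlaps maintain a list of touched actors that implement DamageInterface.
; Each qualifying entry sets a looping half-second timer, never explicitly cleared, that applies FireDamage to every listed actor.
; The construction script disables shadow casting on the mesh.
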(event OnComponentBeginOverlap(Sphere)
  (params (OverlappedComponent :type Primitive%20Component%20Object%20Reference) (OtherActor :type Actor%20Object%20Reference) (OtherComp :type Primitive%20Component%20Object%20Reference) (OtherBodyIndex :type Integer) (bFromSweep :type Boolean) (SweepResult :type Hit%20Result%20Structure%20%28by%20ref%29))
  (if (Utilities|DoesObjectImplementInterface OtherActor "/Game/IvanaKupala/Interface/DamageInterface.DamageInterface_C")
    (Utilities|Array|AddUnique (Variables|Default|GetTuchedActor) OtherActor)
    (Utilities|Time|SetTimerbyEvent (delegate Custom|DamageFire) 0.5 true)))

(event OnComponentEndOverlap(Sphere)
  (params (OverlappedComponent :type Primitive%20Component%20Object%20Reference) (OtherActor :type Actor%20Object%20Reference) (OtherComp :type Primitive%20Component%20Object%20Reference) (OtherBodyIndex :type Integer))
  (bind _tuchedactor (Variables|Default|GetTuchedActor))
  (bind _returnvalue (Utilities|Array|FindItem _tuchedactor OtherActor))
  (if (not (== _returnvalue -1))
    (Utilities|Array|RemoveIndex (Variables|Default|GetTuchedActor) _returnvalue)))

(event Custom|DamageFire
  (for _array_element (Variables|Default|GetTuchedActor)
    (Game|Damage|ApplyDamage _array_element (Variables|Default|GetFireDamage) 0 self)))

(event EventBeginPlay
  (Utilities|FlowControl|Delay 5.0)
  (Actor|DestroyActor))

(fn ConstructionScript
  (Rendering|SetCastShadow (Variables|Default|GetStaticMesh) false))