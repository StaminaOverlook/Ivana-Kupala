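; Short-lived slash hitbox actor for Oka's skills that damages what it sweeps through, then destroys itself.
; On BeginPlay a Timeline moves two mirrored, angled collision boxes outward and forward along local Y while stretching them.
; Overlaps with either box, except BP_OkaCharacter, call DamageTarget, which applies BashDamage to DamageInterface implementers.
; A shared TouchedActors list limits each target to one hit.
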(event OnComponentBeginOverlap(Box1)
  (params (OverlappedComponent :type Primitive%20Component%20Object%20Reference) (OtherActor :type Actor%20Object%20Reference) (OtherComp :type Primitive%20Component%20Object%20Reference) (OtherBodyIndex :type Integer) (bFromSweep :type Boolean) (SweepResult :type Hit%20Result%20Structure%20%28by%20ref%29))
  ;[1 1 1] Applying Damage
  (bind _output_get (Variables|Default|SetOtherActor OtherActor))
  (Utilities|Casting|CastToBP_OkaCharacter _output_get
    (:CastFailed
      (CallFunction|DamageTarget _output_get))))

(event OnComponentBeginOverlap(Box)
  (params (OverlappedComponent :type Primitive%20Component%20Object%20Reference) (OtherActor :type Actor%20Object%20Reference) (OtherComp :type Primitive%20Component%20Object%20Reference) (OtherBodyIndex :type Integer) (bFromSweep :type Boolean) (SweepResult :type Hit%20Result%20Structure%20%28by%20ref%29))
  ;[1 1 1] Applying Damage
  (bind _output_get (Variables|Default|SetOtherActor OtherActor))
  (Utilities|Casting|CastToBP_OkaCharacter _output_get
    (:CastFailed
      (CallFunction|DamageTarget _output_get))))

(event EventBeginPlay
  (Variables|Default|SetCollisionBoxes (Utilities|Array|MakeArray (Variables|Default|GetBox) (Variables|Default|GetBox1)))
  (for _array_element (Variables|Default|GetCollisionBoxes)
    (Utilities|Array|Add (Variables|Default|GetStartLocation) (Variables|/Script/Engine.SceneComponent|GetRelativeLocation _array_element)))
  (bind _newtrack_0 (Timeline|Timeline PlayFromStart)
    (:Update
      (Transformation|SetRelativeTransform (Variables|Default|GetBox1) (Math|Transform|MakeTransform (Math|Vector|Lerp(Vector) (Utilities|Array|Get(acopy) (Variables|Default|GetStartLocation)) "150.000000,700.000000,1.000000" _newtrack_0) "0.000000,-40.000000,0.000000" (Math|Vector|Lerp(Vector) "0.500000,0.200000,1.000000" "5.500000,0.200000,1.000000" _newtrack_0)) false false)
      (Transformation|SetRelativeTransform (Variables|Default|GetBox) (Math|Transform|MakeTransform (Math|Vector|Lerp(Vector) (Utilities|Array|Get(acopy) (Variables|Default|GetStartLocation) 1) "-150.000000,700.000000,1.000000" _newtrack_0) "0.000000,40.000000,0.000000" (Math|Vector|Lerp(Vector) "0.500000,0.200000,1.000000" "5.500000,0.200000,1.000000" _newtrack_0)) false false))
    (:Finished
      (Actor|DestroyActor))))

(fn ConstructionScript)

(fn DamageTarget
  (params (Actor :type Actor%20Object%20Reference))
  (if (and (Utilities|DoesObjectImplementInterface Actor "/Game/IvanaKupala/Interface/DamageInterface.DamageInterface_C") (not (Utilities|Set|Contains (Variables|Default|GetTouchedActors) Actor)))
    (Game|Damage|ApplyDamage Actor (Variables|Default|GetBashDamage) 0 self)
    (Utilities|Set|Add (Variables|Default|GetTouchedActors) 0)))