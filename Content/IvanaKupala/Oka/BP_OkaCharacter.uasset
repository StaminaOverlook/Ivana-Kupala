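; BP_OkaCharacter is the top-down player character Oka, handling melee combos, blocking, rolling, interaction, damage and death.
; Input and health events send tags to a StateTree, whose state events drive montages, movement locks and invulnerability.
; Event-unlocked skills include Bash, Splash, shield dash and bowler coal throws, with Timeline cooldowns gated by DoOnce.
; Switching equipment toggles shield blocking or cursor-aimed throwing, previewed by a predicted-path spline mesh arc.
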(event Custom|LoadGame
  (params (Health :type Float%20%28double-precision%29))
  ;[1 1 1] Restore Oka's state on game load
  (Default|Override (Variables|Default|GetHealthComponent) Health 1e+02))

(event Custom|CanMove
  ;[1 1 1] Can't or Can Move
  (Input|EnableInput (Variables|Default|GetPlayerController)))

(event Custom|ReloadSplash
  (bind _returnvalue (Transformation|GetActorRotation))
  ;[1 1 1] Skills
  (Timeline|Timeline_3 PlayFromStart
    (:Finished
      (Utilities|FlowControl|DoOnce false) ; enters at Reset
    )))

(event Custom|ReloadBash
  ;[1 1 1] Skills
  (Timeline|Timeline_2 PlayFromStart
    (:Finished
      (Utilities|FlowControl|DoOnce false) ; enters at Reset
    )))

(event Custom|BushSkills_Event
  ;[1 1 1] Skills
  (Variables|Skills|SetBush true))

(event Custom|Can't%20Move
  ;[1 1 1] Can't or Can Move
  (Components|Movement|StopMovementImmediately (Variables|Character|GetCharacterMovement))
  (Input|DisableInput (Variables|Default|GetPlayerController)))

(event Custom|OnDead
  ;[1 1 1] Begin Play
  (CallFunction|SendOkaStateEvent "(TagName=\"Dead\")"))

(event Custom|OnHealthChanged
  (params (NewHealth :type Float%20%28double-precision%29) (Amount :type Float%20%28double-precision%29))
  ;[1 1 1] Begin Play
  (CallFunction|SendOkaStateEvent "(TagName=\"Injured\")"))

(event Custom|SplashSkils_Event
  ;[1 1 1] Skills
  (Variables|Skills|SetSplash true))

(event Custom|Bowler_Event
  ;[1 1 1] Skills
  (Variables|Skills|SetBowler true))

(event Custom|FireBowler_Event
  ;[1 1 1] Skills
  (Variables|Skills|SetFireBowler true))

(event Custom|ShieldDashSkills_Event
  ;[1 1 1] Skills
  (Variables|Skills|SetShieldDash true))

(event Input|EnhancedActionEvents|EnhancedInputActionIA_Attack
  (params (ActionValue :type Boolean) (ElapsedSeconds :type Float%20%28double-precision%29) (TriggeredSeconds :type Float%20%28double-precision%29) (InputAction :type Input%20Action%20Object%20Reference :default "/Game/IvanaKupala/Oka/Input/Actions/IA_Attack.IA_Attack"))
  ;[1 1 1] Attack
  (:Started
    (if (or (Utilities|Enum|Equal(Enum) (Variables|Default|GetState) "NewEnumerator5") (Utilities|Enum|Equal(Enum) (Variables|Default|GetState) "NewEnumerator0"))
      (CallFunction|SendOkaStateEvent "(TagName=\"AttackReady\")"))))

(event Input|EnhancedActionEvents|EnhancedInputActionIA_Block
  (params (ActionValue :type Boolean) (ElapsedSeconds :type Float%20%28double-precision%29) (TriggeredSeconds :type Float%20%28double-precision%29) (InputAction :type Input%20Action%20Object%20Reference :default "/Game/IvanaKupala/Oka/Input/Actions/IA_Block.IA_Block"))
  ;[1 1 1] Blocking Damage
  (:Triggered
    (if (== (Variables|Default|GetEquipment) 0) :!label _label
      (if (Utilities|Enum|Equal(Enum) (Variables|Default|GetState) "NewEnumerator5")
        (CallFunction|SendOkaStateEvent "(TagName=\"Oka.Block\")"))
      (elif (Utilities|Enum|Equal(Enum) (Variables|Default|GetState) "NewEnumerator5")
        (CallFunction|SendOkaStateEvent "(TagName=\"Oka.Aiming\")"))))
  (:Started
    (goto _label))
  (:Canceled
    (if (== (Variables|Default|GetEquipment) 0) :!label _label_2
      (if (Utilities|Enum|Equal(Enum) (Variables|Default|GetState) "NewEnumerator2")
        (CallFunction|SendOkaStateEvent "(TagName=\"Oka.CancelBlock\")"))
      (elif (Utilities|Enum|Equal(Enum) (Variables|Default|GetState) "NewEnumerator6")
        (CallFunction|SendOkaStateEvent "(TagName=\"Oka.CancelAiming\")"))))
  (:Completed
    (goto _label_2)))

(event Input|EnhancedActionEvents|EnhancedInputActionIA_Interact
  (params (ActionValue :type Boolean) (ElapsedSeconds :type Float%20%28double-precision%29) (TriggeredSeconds :type Float%20%28double-precision%29) (InputAction :type Input%20Action%20Object%20Reference :default "/Game/IvanaKupala/Oka/Input/Actions/IA_Interact.IA_Interact"))
  (bind _overlappingactors (Collision|GetOverlappingActors "/Game/IvanaKupala/Interactives/Interactive_BP.Interactive_BP_C" :!class /Script/Engine.Actor))
  ;[1 1 1] Interacting with Objects
  (if (Utilities|Array|IsValidIndex _overlappingactors)
    (Class|InteractiveBPInterface|Interact(Message) (Utilities|Array|Get(acopy) _overlappingactors))))

(event Input|EnhancedActionEvents|EnhancedInputActionIA_Roll
  (params (ActionValue :type Boolean) (ElapsedSeconds :type Float%20%28double-precision%29) (TriggeredSeconds :type Float%20%28double-precision%29) (InputAction :type Input%20Action%20Object%20Reference :default "/Game/IvanaKupala/Oka/Input/Actions/IA_Roll.IA_Roll"))
  ;[1 1 1] Roll to evade damage logic
  (if (Utilities|Enum|Equal(Enum) (Variables|Default|GetState) "NewEnumerator5")
    (CallFunction|SendOkaStateEvent "(TagName=\"Oka.Roll\")")))

(event Input|EnhancedActionEvents|EnhancedInputActionIA_TakeShield
  (params (ActionValue :type Boolean) (ElapsedSeconds :type Float%20%28double-precision%29) (TriggeredSeconds :type Float%20%28double-precision%29) (InputAction :type Input%20Action%20Object%20Reference :default "/Game/IvanaKupala/Oka/Input/Actions/IA_TakeShield.IA_TakeShield"))
  ;[1 1 1] Switch Equipment
  (:Started
    (if (Utilities|Enum|Equal(Enum) (Variables|Default|GetState) "NewEnumerator5")
      (if (!= (Variables|Default|GetEquipment) 0)
        (Utilities|FlowControl|DoOnce false :!label _label
          (:Completed
            (Variables|/Game/IvanaKupala/Oka/Input/BP_TopDownController.BP_TopDownController_C|SetDisabled_Input (Variables|Default|GetPlayerController) true)
            (Pawn|Components|CharacterMovement|DisableMovement (Variables|Character|GetCharacterMovement))
            (Animation|Montage|PlayMontage (Variables|Character|GetMesh) "/Game/IvanaKupala/Oka/Animations/Blocking/Oka_Blocked_Montage.Oka_Blocked_Montage"
              (:OnCompleted
                (Variables|Default|SetEquipment 0))
              (:OnInterrupted
                _))
            (Variables|/Game/IvanaKupala/Oka/Input/BP_TopDownController.BP_TopDownController_C|SetDisabled_Input (Variables|Default|GetPlayerController) false)
            (Pawn|Components|CharacterMovement|SetMovementMode (Variables|Character|GetCharacterMovement) "MOVE_Walking" 0)
            (goto _label Reset)))))))

(event Input|EnhancedActionEvents|EnhancedInputActionIA_TakeBowler
  (params (ActionValue :type Boolean) (ElapsedSeconds :type Float%20%28double-precision%29) (TriggeredSeconds :type Float%20%28double-precision%29) (InputAction :type Input%20Action%20Object%20Reference :default "/Game/IvanaKupala/Oka/Input/Actions/IA_TakeBowler.IA_TakeBowler"))
  ;[1 1 1] Switch Equipment
  (:Started
    (if (Utilities|Enum|Equal(Enum) (Variables|Default|GetState) "NewEnumerator5")
      (if (Variables|Skills|GetBowler)
        (if (!= (Variables|Default|GetEquipment) 1)
          (Utilities|FlowControl|DoOnce false :!label _label
            (:Completed
              (Variables|/Game/IvanaKupala/Oka/Input/BP_TopDownController.BP_TopDownController_C|SetDisabled_Input (Variables|Default|GetPlayerController) true)
              (Pawn|Components|CharacterMovement|DisableMovement (Variables|Character|GetCharacterMovement))
              (Animation|Montage|PlayMontage (Variables|Character|GetMesh) "/Game/IvanaKupala/Oka/Animations/Blocking/Oka_Blocked_Montage.Oka_Blocked_Montage"
                (:OnCompleted
                  (Variables|Default|SetEquipment 1))
                (:OnInterrupted
                  _))
              (Variables|/Game/IvanaKupala/Oka/Input/BP_TopDownController.BP_TopDownController_C|SetDisabled_Input (Variables|Default|GetPlayerController) false)
              (Pawn|Components|CharacterMovement|SetMovementMode (Variables|Character|GetCharacterMovement) "MOVE_Walking" 0)
              (goto _label Reset))))))))

(event Input|EnhancedActionEvents|EnhancedInputActionIA_Bash
  (params (ActionValue :type Boolean) (ElapsedSeconds :type Float%20%28double-precision%29) (TriggeredSeconds :type Float%20%28double-precision%29) (InputAction :type Input%20Action%20Object%20Reference :default "/Game/IvanaKupala/Oka/Input/Actions/IA_Bash.IA_Bash"))
  ;[1 1 1] Skills
  (:Started
    (if (Utilities|Enum|Equal(Enum) (Variables|Default|GetState) "NewEnumerator5")
      (if (Variables|Skills|GetBush)
        (Utilities|FlowControl|DoOnce false
          (:Completed
            (Variables|/Game/IvanaKupala/Oka/Input/BP_TopDownController.BP_TopDownController_C|SetDisabled_Input (Variables|Default|GetPlayerController) true)
            (Pawn|Components|CharacterMovement|DisableMovement (Variables|Character|GetCharacterMovement))
            (Animation|Montage|PlayMontage (Variables|Character|GetMesh) "/Game/IvanaKupala/Oka/Animations/Blocking/Oka_Blocked_Montage.Oka_Blocked_Montage"
              (:then
                (Game|SpawnActorfromClass "/Game/IvanaKupala/Oka/Skills/BP_BashPoint.BP_BashPoint_C" (Math|Transform|MakeTransform (Transformation|GetActorLocation) "0, 0, 0" "1.000000,1.000000,1.000000") "Undefined" "MultiplyWithRoot" 0 0))
              (:OnCompleted
                (Variables|/Game/IvanaKupala/Oka/Input/BP_TopDownController.BP_TopDownController_C|SetDisabled_Input (Variables|Default|GetPlayerController) false :!label _label)
                (Pawn|Components|CharacterMovement|SetMovementMode (Variables|Character|GetCharacterMovement) "MOVE_Walking" 0)
                (CallFunction|ReloadBash))
              (:OnInterrupted
                (goto _label)))))))))

(event Input|EnhancedActionEvents|EnhancedInputActionIA_Splash
  (params (ActionValue :type Boolean) (ElapsedSeconds :type Float%20%28double-precision%29) (TriggeredSeconds :type Float%20%28double-precision%29) (InputAction :type Input%20Action%20Object%20Reference :default "/Game/IvanaKupala/Oka/Input/Actions/IA_Splash.IA_Splash"))
  (bind _returnvalue (Transformation|GetActorRotation))
  ;[1 1 1] Skills
  (:Started
    (if (Utilities|Enum|Equal(Enum) (Variables|Default|GetState) "NewEnumerator5")
      (if (Variables|Skills|GetSplash)
        (Utilities|FlowControl|DoOnce false
          (:Completed
            (Variables|/Game/IvanaKupala/Oka/Input/BP_TopDownController.BP_TopDownController_C|SetDisabled_Input (Variables|Default|GetPlayerController) true)
            (Pawn|Components|CharacterMovement|DisableMovement (Variables|Character|GetCharacterMovement))
            (bind (_x _y _z) (Rotation|RotationbyCursor))
            (Transformation|SetActorRotation (Math|Rotator|MakeRotator _x _y _z))
            (Animation|Montage|PlayMontage (Variables|Character|GetMesh) "/Game/IvanaKupala/Oka/Animations/Attacks/Oka_Second_Slash_Montage.Oka_Second_Slash_Montage"
              (:then
                (Game|SpawnActorfromClass "/Game/IvanaKupala/Oka/Skills/BP_SlashPoint.BP_SlashPoint_C" (Math|Transform|MakeTransform (+ (Transformation|GetActorLocation) "0.000000,0.000000,100.000000") (Math|Rotator|MakeRotator (.roll _returnvalue) (.pitch _returnvalue) (- (.yaw _returnvalue) 9e+01)) "1.000000,1.000000,1.000000") "Undefined" "MultiplyWithRoot" 0 0))
              (:OnCompleted
                (Variables|/Game/IvanaKupala/Oka/Input/BP_TopDownController.BP_TopDownController_C|SetDisabled_Input (Variables|Default|GetPlayerController) false :!label _label)
                (Pawn|Components|CharacterMovement|SetMovementMode (Variables|Character|GetCharacterMovement) "MOVE_Walking" 0)
                (CallFunction|ReloadSplash))
              (:OnInterrupted
                (goto _label)))))))))

(event Collision|EventActorBeginOverlap
  (params (OtherActor :type Actor%20Object%20Reference))
  (bind _asbp_monologue (Utilities|Casting|CastToBP_Monologue OtherActor))
  (if (not (Variables|/Game/IvanaKupala/Maps/Levels/Interactive/BP_Monologue.BP_Monologue_C|GetCutscene _asbp_monologue))
    (for _array_element (Collision|GetOverlappingActors "/Game/IvanaKupala/Maps/Levels/Interactive/BP_Monologue.BP_Monologue_C" :!class /Script/Engine.Actor)
      (if (Utilities|DoesObjectImplementInterface _array_element "/Game/IvanaKupala/Maps/Levels/Interactive/BPI_Talk.BPI_Talk_C")
        (Class|BPITalk|Say(Message) _array_element)))))

(event Game|Damage|EventAnyDamage
  (params (Damage :type Float%20%28single-precision%29) (DamageType :type Damage%20Type%20Object%20Reference) (InstigatedBy :type Controller%20Object%20Reference) (DamageCauser :type Actor%20Object%20Reference))
  (bind _mesh (Variables|Character|GetMesh))
  ;[1 1 1] Taking Damage
  (Audio|PlaySoundatLocation "/Game/IvanaKupala/Interface/GeneralSFX/Enemy_Attacks.Enemy_Attacks" (Transformation|GetActorLocation) "0, 0, 0" 1.0 1.0 0.0 0 0 0 0)
  (Components|Movement|StopMovementImmediately (Variables|Character|GetCharacterMovement))
  (Default|EventDamage (Variables|Default|GetHealthComponent) Damage)
  (Utilities|Casting|CastToPushed_DamageType DamageType
    (:then
      (Animation|Montage|PlayMontage _mesh "/Game/IvanaKupala/Oka/Animations/Oka_Pushed_Montage.Oka_Pushed_Montage"))
    (:CastFailed
      (Animation|Montage|PlayMontage _mesh "/Game/IvanaKupala/Oka/Animations/Oka_Injured_Montage.Oka_Injured_Montage"))))

(event EventBlockedDamage
  ;[1 1 1] Succesfully Blocked Damage
  (if (Variables|/Game/IvanaKupala/Oka/Animations/OkaAnimationBlueprint.OkaAnimationBlueprint_C|GetBlocking (Variables|Default|GetAnimBlueprint))
    (Development|PrintString "Blocked Attack!" true true "(R=0.293285,G=1.000000,B=0.000000,A=1.000000)")
    (Animation|PlayAnimMontage "/Game/IvanaKupala/Oka/Animations/Blocking/Oka_Blocked_Montage.Oka_Blocked_Montage" 1.0 "None")))

(event EventBeginPlay
  ;[1 1 1] Begin Play
  (Utilities|FlowControl|Sequence
    (:then_0
      (bind _asoka_animation_blueprint (Utilities|Casting|CastToOkaAnimationBlueprint (Components|SkeletalMesh|GetAnimInstance (Variables|Character|GetMesh))))
      (Variables|Default|SetAnimBlueprint _asoka_animation_blueprint))
    (:then_1
      (bind _assword_class (Utilities|Casting|CastToSwordClass (Variables|/Script/Engine.ChildActorComponent|GetChildActor (Variables|Default|GetSword))))
      (Variables|Default|SetWeapon _assword_class))
    (:then_2
      (bind _asshield_class (Utilities|Casting|CastToShieldClass (Variables|/Script/Engine.ChildActorComponent|GetChildActor (Variables|Default|GetShield))))
      (Variables|Default|SetShieldRef _asshield_class))
    (:then_3
      (bind _asbp_top_down_controller (Utilities|Casting|CastToBP_TopDownController (Game|GetPlayerController 0)))
      (Variables|Default|SetPlayerController _asbp_top_down_controller))
    (:then_4
      (EventDispatchers|BindEventtoDead (Variables|Default|GetHealthComponent) (delegate Custom|OnDead)))
    (:then_5
      (EventDispatchers|BindEventtoDamaged (Variables|Default|GetHealthComponent) (delegate Custom|OnHealthChanged)))
    (:then_6
      ;[1 1 1] Skills
      (Utilities|FlowControl|Sequence
        (:then_0
          (EventDispatchers|BindEventtoBushSkills (delegate Custom|BushSkills_Event)))
        (:then_1
          (EventDispatchers|BindEventtoSplashSkils (delegate Custom|SplashSkils_Event)))
        (:then_2
          (EventDispatchers|BindEventtoBowlerSkills (delegate Custom|Bowler_Event)))
        (:then_3
          (EventDispatchers|BindEventtoFireBowlerSkills (delegate Custom|FireBowler_Event)))
        (:then_4
          (EventDispatchers|BindEventtoShieldDashSkills (delegate Custom|ShieldDashSkills_Event)))))))

(event Input|KeyboardEvents|E
  (params (Key :type Key%20Structure :default "None"))
  (:Pressed
    (for _array_element (Collision|GetOverlappingActors "/Game/IvanaKupala/Maps/Levels/Interactive/BP_Monologue.BP_Monologue_C" :!class /Script/Engine.Actor)
      (if (Utilities|DoesObjectImplementInterface _array_element "/Game/IvanaKupala/Maps/Levels/Interactive/BPI_Talk.BPI_Talk_C")
        (Class|BPITalk|Say(Message) _array_element)))))

(event Custom|StartInjuredState
  ;[1 1 1] Start Injured State
  (Variables|Actor|SetbCanBeDamaged false)
  (CallFunction|SendOkaStateEvent "(TagName=\"Recover\")")
  (Utilities|FlowControl|Delay 1.0)
  (Variables|Actor|SetbCanBeDamaged true))

(event Custom|StartDeadState
  ;[1 1 1] Start Dead State
  (Input|DisableInput (Variables|Default|GetPlayerController))
  (Pawn|Components|CharacterMovement|DisableMovement (Variables|Character|GetCharacterMovement))
  (Variables|Actor|SetbCanBeDamaged false)
  (Animation|Montage|PlayMontage (Variables|Character|GetMesh) "/Game/IvanaKupala/Oka/Animations/Oka_Death_Montage.Oka_Death_Montage" 1.0 0.0 ""
    (:then
      (Utilities|FlowControl|Delay 5.0)
      (Game|OpenLevel(byName) "Main_Menu"))))

(event Custom|ReloadBowler
  (bind _returnvalue (Game|GetPlayerController 0))
  (bind _returnvalue_2 (Utilities|ThrowLocation))
  (bind _returnvalue_3 (Utilities|ThrowLocation))
  (bind _hitresult (Game|Player|GetHitResultUnderCursorbyChannel _returnvalue "TraceTypeQuery1" true))
  (bind _impactpoint (Collision|BreakHitResult _hitresult))
  (bind _returnvalue_4 (- _impactpoint _returnvalue_2))
  (bind (_x _y _z) (Math|Vector|BreakVector _returnvalue_4))
  (bind _returnvalue_5 (+ _z 5e+02))
  (bind _returnvalue_6 (Math|Vector|MakeVector _x _y _returnvalue_5))
  ;[1 1 1] Bowler and FireBowler Skill
  (Timeline|Timeline_0 PlayFromStart
    (:Finished
      (Utilities|FlowControl|DoOnce false) ; enters at Reset
    )))

(event Custom|StartBlockState
  ;[1 1 1] Start Block State
  (Variables|Default|SetBlocking true)
  (Pawn|Components|CharacterMovement|DisableMovement (Variables|Character|GetCharacterMovement))
  (Utilities|Time|SetTimerbyFunctionName 0 "RotationByCursorWithInter" 0.0001 true true))

(event Custom|EndBlockState
  ;[1 1 1] End Block State
  (Variables|Default|SetBlocking false)
  (Animation|StopAnimMontage 0)
  (Pawn|Components|CharacterMovement|SetMovementMode (Variables|Character|GetCharacterMovement) "MOVE_Walking" 0)
  (Class|KismetSystemLibrary|PauseTimer 0 "RotationByCursorWithInter"))

(event Custom|ReloadShieldDash
  ;[1 1 1] Shield Dash Skill
  (Timeline|Timeline PlayFromStart
    (:Finished
      (Utilities|FlowControl|DoOnce false) ; enters at Reset
    )))

(event Custom|StartRollState
  (bind _playercontroller (Variables|Default|GetPlayerController))
  ;[1 1 1] Start Roll State
  (Variables|Actor|SetbCanBeDamaged false)
  (Variables|/Game/IvanaKupala/Oka/Input/BP_TopDownController.BP_TopDownController_C|SetDisabled_Input _playercontroller true)
  (Animation|Montage|PlayMontage (Variables|Character|GetMesh) "/Game/IvanaKupala/Oka/Animations/Blocking/Oka_Roll_Montage.Oka_Roll_Montage"
    (:OnCompleted
      (Variables|Actor|SetbCanBeDamaged true)
      (Variables|/Game/IvanaKupala/Oka/Input/BP_TopDownController.BP_TopDownController_C|SetDisabled_Input _playercontroller false)
      (CallFunction|SendOkaStateEvent "(TagName=\"Oka.RollOver\")"))))

(event Custom|StartAttackState
  ;[1 1 1] Start Attack State
  (if (not (Variables|Default|GetAttacking))
    (Variables|Default|SetAttacking true)
    (bind (_x _y _z) (Rotation|RotationbyCursor :!label _label))
    (Transformation|SetActorRotation (Math|Rotator|MakeRotator _x _y _z))
    (Variables|/Game/IvanaKupala/Oka/Input/BP_TopDownController.BP_TopDownController_C|SetDisabled_Input (Variables|Default|GetPlayerController) true)
    (Animation|Montage|PlayMontage (Variables|Character|GetMesh) (Utilities|Select :Index (Variables|Default|GetCombo) :Option%200 "/Game/IvanaKupala/Oka/Animations/Attacks/Oka_Slash_Montage.Oka_Slash_Montage" :Option%201 "/Game/IvanaKupala/Oka/Animations/Attacks/Oka_Second_Slash_Montage.Oka_Second_Slash_Montage" :Option%202 "/Game/IvanaKupala/Oka/Animations/Attacks/Oka_Slash_Long_Montage.Oka_Slash_Long_Montage")
      (:then
        (Math|Integer|IncrementInt (Variables|Default|GetCombo)))
      (:OnCompleted
        (Variables|/Game/IvanaKupala/Oka/Input/BP_TopDownController.BP_TopDownController_C|SetDisabled_Input (Variables|Default|GetPlayerController) false :!label _label_2)
        (if (and (Game|Player|IsInputKeyDown (Variables|Default|GetPlayerController) "LeftMouseButton") (< (Variables|Default|GetCombo) 3))
          (goto _label)
          (else
            (Variables|Default|SetCombo 0)
            (Default|EndAttack (Variables|Default|GetWeapon))
            (if (Game|Player|IsInputKeyDown (Variables|Default|GetPlayerController) "LeftMouseButton")
              (CallFunction|SendOkaStateEvent "(TagName=\"AttackReady\")")
              (else
                (CallFunction|SendOkaStateEvent "(TagName=\"AttackOver\")"))))))
      (:OnInterrupted
        (Utilities|FlowControl|RetriggerableDelay 1.5)
        (Variables|Default|SetAttacking false)
        (goto _label_2)))))

(event Custom|StartAimingState
  ;[1 1 1] Start Aiming State
  (Variables|Default|SetAiming true)
  (Pawn|Components|CharacterMovement|DisableMovement (Variables|Character|GetCharacterMovement))
  (Utilities|Time|SetTimerbyFunctionName 0 "RotationByCursorWithInter" 0.0001 true true)
  (Throwing|CreatePredictionSpline)
  (Utilities|Time|SetTimerbyFunctionName 0 "DrowPredictionSpline" 0.0001 true true))

(event Custom|EndAimingState
  ;[1 1 1] End Aiming State
  (Variables|Default|SetAiming false)
  (Animation|StopAnimMontage 0)
  (Pawn|Components|CharacterMovement|SetMovementMode (Variables|Character|GetCharacterMovement) "MOVE_Walking" 0)
  (Class|KismetSystemLibrary|PauseTimer 0 "RotationByCursorWithInter")
  (Class|KismetSystemLibrary|PauseTimer 0 "DrowPredictionSpline")
  (Throwing|DestroyPredictionSpline))

(event Input|KeyboardEvents|DebugKey0
  (params (Key :type Key%20Structure :default "None") (ActionValue :type Input%20Action%20Value%20Structure))
  (:Pressed
    (Utilities|FlowControl|FlipFlop
      (:A
        (Variables|Skills|SetFireBowler false))
      (:B
        (Variables|Skills|SetFireBowler true)))))

(event Input|MouseEvents|LeftMouseButton
  (params (Key :type Key%20Structure :default "None"))
  (bind _returnvalue (Game|GetPlayerController 0))
  (bind _returnvalue_2 (Utilities|ThrowLocation))
  (bind _returnvalue_3 (Utilities|ThrowLocation))
  (bind _hitresult (Game|Player|GetHitResultUnderCursorbyChannel _returnvalue "TraceTypeQuery1" true))
  (bind _impactpoint (Collision|BreakHitResult _hitresult))
  (bind _returnvalue_4 (- _impactpoint _returnvalue_2))
  (bind (_x _y _z) (Math|Vector|BreakVector _returnvalue_4))
  (bind _returnvalue_5 (+ _z 5e+02))
  (bind _returnvalue_6 (Math|Vector|MakeVector _x _y _returnvalue_5))
  ;[1 1 1] Shield Dash Skill
  (:Pressed
    (if (Variables|Default|GetBlocking)
      (Utilities|FlowControl|DoOnce false
        (:Completed
          (Pawn|Components|CharacterMovement|SetMovementMode (Variables|Character|GetCharacterMovement) "MOVE_Walking" 0)
          (Class|DamageInterface|CanDealDmg(Message) (Variables|Default|GetShieldRef))
          (Animation|Montage|PlayMontage (Variables|Character|GetMesh) "/Game/IvanaKupala/Oka/Animations/Blocking/Oka_Roll_Montage.Oka_Roll_Montage"
            (:OnCompleted
              _)
            (:OnInterrupted
              _))
          (Class|DamageInterface|StopDealDmg(Message) (Variables|Default|GetShieldRef))
          (Pawn|Components|CharacterMovement|DisableMovement (Variables|Character|GetCharacterMovement))
          (Default|EndAttack (Variables|Default|GetShieldRef))
          (CallFunction|ReloadShieldDash)
          (CallFunction|EndBlockState)))
      (else
        ;[1 1 1] Bowler and FireBowler Skill
        (if (Variables|Default|GetAiming)
          (Utilities|FlowControl|DoOnce false
            (:Completed
              (Utilities|PredictionSplineValid?
                (:Is%20Valid
                  (Throwing|DestroyPredictionSpline)
                  (if (Variables|Skills|GetFireBowler)
                    (Game|SpawnActorfromClass "/Game/IvanaKupala/Oka/Skills/TakeAim/BP_FireCoal.BP_FireCoal_C" (Math|Transform|MakeTransform _returnvalue_3 "0, 0, 0" "1.000000,1.000000,1.000000") "Undefined" "MultiplyWithRoot" 0 _returnvalue_6 0)
                    (else
                      (Game|SpawnActorfromClass "/Game/IvanaKupala/Oka/Skills/TakeAim/BP_Coal.BP_Coal_C" (Math|Transform|MakeTransform _returnvalue_3 "0, 0, 0" "1.000000,1.000000,1.000000") "Undefined" "MultiplyWithRoot" 0 _returnvalue_6 0)))
                  (CallFunction|ReloadBowler)
                  (CallFunction|EndAimingState))))))))))

(fn ConstructionScript
  (Default|ConnectStateTree (Variables|Default|GetStateTreeQueue) (Variables|Default|GetOkaStateTree)))

(fn CheckActorLoc
  (params (ActorToCheck :type Actor%20Object%20Reference))
  (bind _capsulecomponent (Variables|Collision|GetCapsuleComponent))
  (return (< (Class|KismetMathLibrary|DegAcos (Math|Vector|DotProduct (Class|KismetMathLibrary|VectorNormal2D (- (Transformation|GetActorLocation ActorToCheck) (Transformation|GetWorldLocation _capsulecomponent)) 0.0001) (Math|Vector|GetForwardVector _capsulecomponent))) 6e+01)))

(fn IsMontagePlaying
  (params (Montage :type Anim%20Montage%20Object%20Reference))
  (return (Animation|Montage|MontageIsPlaying (Components|SkeletalMesh|GetAnimInstance (Variables|Character|GetMesh)) Montage)))

(fn SendOkaStateEvent
  (params (Tag :type Gameplay%20Tag%20Structure))
  (Gameplay|StateTree|SendStateTreeEvent (Variables|Default|GetOkaStateTree) (Utilities|Struct|MakeStateTreeEvent Tag) :!class /Script/GameplayStateTreeModule.StateTreeComponent)
  (return))

(fn RotationbyCursor
  (bind _returnvalue (Transformation|GetActorRotation))
  (return (.roll _returnvalue) (.pitch _returnvalue) (.yaw (Math|Rotator|FindLookatRotation (+ "" "") (- (.ImpactPoint (Collision|BreakHitResult (.HitResult (Game|Player|GetHitResultUnderCursorbyChannel (Game|GetPlayerController 0) "TraceTypeQuery1" true)))) (Transformation|GetActorLocation))))))

(fn RotationbyCursorwithInter
  (bind _returnvalue (Transformation|GetActorRotation))
  (Transformation|SetActorRotation (Math|Rotator|MakeRotator (.roll _returnvalue) (.pitch _returnvalue) (.yaw (Class|KismetMathLibrary|RInterptoConstant (Transformation|GetActorRotation) (Math|Rotator|FindLookatRotation (+ "" "") (- (.ImpactPoint (Collision|BreakHitResult (.HitResult (Game|Player|GetHitResultUnderCursorbyChannel (Game|GetPlayerController 0) "TraceTypeQuery1" true)))) (Transformation|GetActorLocation))) (Utilities|Time|GetWorldDeltaSeconds) 3.5e+02)))))

(fn DrowPredictionSpline
  (bind _returnvalue (Game|GetPlayerController 0))
  (bind _returnvalue_2 (Utilities|ThrowLocation))
  (bind _hitresult (Game|Player|GetHitResultUnderCursorbyChannel _returnvalue "TraceTypeQuery1" true))
  (bind _impactpoint (Collision|BreakHitResult _hitresult))
  (bind _returnvalue_3 (- _impactpoint _returnvalue_2))
  (bind (_x _y _z) (Math|Vector|BreakVector _returnvalue_3))
  (Utilities|PredictionSplineValid?
    (:Is%20Valid
      (Utilities|FlowControl|Sequence
        (:then_0
          (bind (_outhit _outpathpositions _outlasttracedestination _returnvalue_4) (Class|GameplayStatics|BlueprintPredictProjectilePathbyTraceChannel (Utilities|ThrowLocation) (Math|Vector|MakeVector _x _y (+ _z 5e+02)) true 15.0 "ECC_WorldDynamic" false (Utilities|Array|MakeArray self (Variables|Default|GetShieldRef)) "None"))
          (if _returnvalue_4
            (Rendering|SetActorHiddenInGame (Variables|Throwing|GetPredictionEndPoint) false)
            (Transformation|SetActorLocation (Variables|Throwing|GetPredictionEndPoint) (.ImpactPoint (Collision|BreakHitResult _outhit)) false true)
            (else
              (Rendering|SetActorHiddenInGame (Variables|Throwing|GetPredictionEndPoint) true)))
          (Spline|SetSplinePoints (Variables|Throwing|GetPredictionsSpline) _outpathpositions "World" true)
          (Throwing|DestroyPredictionMeshes))
        (:then_1
          (for _index (range 0 (Math|Float|Truncate (/ (Spline|GetSplineLength (Variables|Throwing|GetPredictionsSpline)) 1e+02)))
            (LocalVariables|SetIndex _index)
            (bind _returnvalue_5 (AddComponent|AddSplineMeshComponent true))
            (Utilities|Array|Add (Variables|Throwing|GetPredictionSplineMeshes) _returnvalue_5)
            (SplineMesh|SetStartandEnd _returnvalue_5 (Spline|GetLocationatDistanceAlongSpline (Variables|Throwing|GetPredictionsSpline) (* (LocalVariables|GetIndex) 1e+02) "World") (Math|Vector|ClampVectorSize (Spline|GetTangentatDistanceAlongSpline (Variables|Throwing|GetPredictionsSpline) (* (LocalVariables|GetIndex) 1e+02) "World") 0.0 1e+02) (Spline|GetLocationatDistanceAlongSpline (Variables|Throwing|GetPredictionsSpline) (* (+ (LocalVariables|GetIndex) 1) 1e+02) "World") (Math|Vector|ClampVectorSize (Spline|GetTangentatDistanceAlongSpline (Variables|Throwing|GetPredictionsSpline) (* (+ (LocalVariables|GetIndex) 1) 1e+02) "World") 0.0 1e+02) true :!class /Script/Engine.SplineMeshComponent)))))))

(fn DestroyPredictionMeshes
  (for _array_element (Variables|Throwing|GetPredictionSplineMeshes)
    (Components|DestroyComponent _array_element))
  (Utilities|Array|Clear (Variables|Throwing|GetPredictionSplineMeshes)))

(fn DestroyPredictionSpline
  (bind _predictionsspline (Variables|Throwing|GetPredictionsSpline)
    (:then
      (Components|DestroyComponent _predictionsspline)
      (Variables|Throwing|SetPredictionsSpline 0)
      (Throwing|DestroyPredictionMeshes)
      (Actor|DestroyActor (Variables|Throwing|GetPredictionEndPoint))
      (Variables|Throwing|SetPredictionEndPoint 0))
    (:else)))

(fn CreatePredictionSpline
  (bind _returnvalue (AddComponent|AddSplineComponent false))
  (Variables|Throwing|SetPredictionsSpline _returnvalue)
  (bind _returnvalue_2 (Game|SpawnActorfromClass "/Game/IvanaKupala/Oka/Skills/TakeAim/BP_PredictionEndPoint.BP_PredictionEndPoint_C" (Math|Transform|MakeTransform "0, 0, 0" "0, 0, 0" "1.000000,1.000000,1.000000") "Undefined" "MultiplyWithRoot" 0 0))
  (bind _output_get (Variables|Throwing|SetPredictionEndPoint _returnvalue_2))
  (Rendering|SetActorHiddenInGame _output_get false))