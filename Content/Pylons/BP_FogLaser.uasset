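; BP_FogLaser is a laser-hit receiver that removes its Cube component, apparently a fog barrier, when struck by a yellow laser.
; LaserBounce checks hit response and laser color, sets Activate and fires the fog-open dispatcher.
; The handler rechecks Activate after three seconds, then destroys the Cube and turns off the light on the tagged BP_LasersSpawn.
; The handler's dispatcher binding is unreachable in this graph.
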(event Custom|FogOpenDispacher_Event
  (if (Variables|Default|GetActivate)
    (Utilities|FlowControl|Delay 3.0)
    (if (Variables|Default|GetActivate)
      (Components|DestroyComponent (Variables|Default|GetCube))
      (bind _outactors (Actor|GetAllActorsOfClasswithTag "/Game/IvanaKupala/Interactives/Pylons/BP_LasersSpawn.BP_LasersSpawn_C" "1"))
      (Default|LightOffEvent (Utilities|Array|Get(acopy) _outactors))
      (else
        (Variables|Default|SetActivate true)))))

(event EventBeginPlay
  (|CallParentFunction) ; This node is disabled and will not be called.\nDrag off pins to build functionality.
)

(event Collision|EventActorBeginOverlap
  (params (OtherActor :type Actor%20Object%20Reference))
  (|CallParentFunction OtherActor) ; This node is disabled and will not be called.\nDrag off pins to build functionality.
)

(event EventTick
  (params (DeltaSeconds :type Float%20%28single-precision%29))
  (|CallParentFunction DeltaSeconds) ; This node is disabled and will not be called.\nDrag off pins to build functionality.
)

(fn ConstructionScript
  (|CallParentFunction))

(fn LaserBounce
  (params (P_LaserHit :type BP%20Laser%20Object%20Reference) (P_HitResponce :type Boolean) (P_HitInformation :type Hit%20Result%20Structure) (P_HitComponent :type Primitive%20Component%20Object%20Reference))
  (if (and P_HitResponce (== (Variables|/Game/IvanaKupala/Interactives/Pylons/BP_LasersParent.BP_LasersParent_C|GetLaserColor P_LaserHit) "(R=0.850980,G=0.756863,B=0.000000,A=1.000000)"))
    (Variables|Default|SetActivate true)
    (CallFunction|FogOpenDispacherEvent)
    (else
      (Variables|Default|SetActivate false)))
  (return 0))